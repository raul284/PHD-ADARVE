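; Talkable NPC that runs voiced, data table-driven conversations with the player through a world-space dialog widget turned toward them.
; Table rows are grouped by conversation number and rebuilt at each conversation start.
; Player and NPC lines advance on interaction or when audio finishes, while quest lines await one of two options, whose dialogs are spliced into the current conversation.
; Interactions outside quest prompts are logged through DBManager.
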(event Custom|SelectSecondOptionFromQuest
  ;[1 1 1] Dialogs
  (bind _dialog (CallFunction|GetDialog))
  (CallFunction|AddOptionDialogstoConversation (.dialogs (.questionsecondoption _dialog)))
  (Default|HideOptions (Variables|Default|GetWidget))
  (bind _continue (CallFunction|NextDialog))
  (if _continue
    (CallFunction|ProcessDialog)))

(event Custom|OnDialogAudioFinished
  ;[1 1 1] Dialogs
  (if (Variables|Dialog|GetTalking)
    (Utilities|FlowControl|Delay 0.2)
    (bind _continue (CallFunction|NextDialog))
    (if _continue
      (CallFunction|ProcessDialog)
      (else
        (CallFunction|StopConversation)))))

(event Custom|SelectFirstOptionFromQuest
  ;[1 1 1] Dialogs
  (bind _dialog (CallFunction|GetDialog))
  (CallFunction|AddOptionDialogstoConversation (.dialogs (.questionfirstoption _dialog)))
  (Default|HideOptions (Variables|Default|GetWidget))
  (bind _continue (CallFunction|NextDialog))
  (if _continue
    (CallFunction|ProcessDialog)))

(event Custom|ProcessDialog
  (bind _audio (Variables|Default|GetAudio))
  (bind _widget (Variables|Default|GetWidget))
  ;[1 1 1] Dialogs
  (if (Variables|Dialog|GetTalking)
    (Variables|Dialog|SetIsQuest? false)
    (bind _dialog (CallFunction|GetDialog))
    (switch Utilities|FlowControl|Switch|SwitchonE_DialogType (.type (.DialogData (Utilities|Struct|BreakF_Dialog _dialog)))
      (:NewEnumerator2
        (Development|PrintString "Un diálogo que no tiene dueño :(" true true "(R=1.000000,G=0.000000,B=0.000000,A=1.000000)"))
      (:NewEnumerator0
        (Default|CreatePlayerText (Variables|Default|GetWidget) (Utilities|Text|ToText(String) (Variables|/Game/Game/Blueprints/Characters/Players/BP_Player.BP_Player_C|GetName (Variables|Default|GetPlayer))) (.text (.DialogData (Utilities|Struct|BreakF_Dialog _dialog))))
        (Audio|Components|Audio|SetSound _audio (.voice (.DialogData (Utilities|Struct|BreakF_Dialog _dialog))) :!label _label)
        (Audio|Components|Audio|Play _audio 0.0)
        (EventDispatchers|AssignOnAudioFinished _audio (delegate Custom|OnDialogAudioFinished)))
      (:NewEnumerator1
        (Default|CreateNPCText (Variables|Default|GetWidget) (Utilities|Text|ToText(String) (Variables|Default|GetName)) (.text (.DialogData (Utilities|Struct|BreakF_Dialog _dialog))))
        (goto _label))
      (:NewEnumerator3
        (Variables|Dialog|SetIsQuest? true)
        (Default|CreateNPCText _widget (Utilities|Text|ToText(String) (Variables|Default|GetName)) (.text (.DialogData (Utilities|Struct|BreakF_Dialog _dialog))))
        (Default|SetOptionsText _widget (.Text (Utilities|Struct|BreakF_QuestOption (.QuestionFirstOption (Utilities|Struct|BreakF_Dialog _dialog)))) (.Text (Utilities|Struct|BreakF_QuestOption (.QuestionSecondOption (Utilities|Struct|BreakF_Dialog _dialog)))))
        (Default|ShowOptions _widget)))))

(event Custom|StartConversation
  ;[1 1 1] Dialogs
  (CallFunction|SetDialogsfromDataTable)
  (if (and (> (Utilities|Array|Length (Variables|Dialog|GetConversations)) 0) (Variables|Dialog|GetCanStartConversation))
    (Variables|Dialog|SetConversationStarted true)
    (Variables|Dialog|SetDialogIndex 0)
    (Variables|Dialog|SetTalking true)
    (Rendering|SetVisibility (Variables|Default|GetDialogWidget) true false)
    (Default|ShowDialogBox (Variables|Default|GetWidget))
    (CallFunction|ProcessDialog)))

(event Custom|NextConversation
  (bind _conversations (Variables|Dialog|GetConversations))
  (bind _returnvalue (Utilities|Array|Length _conversations))
  ;[1 1 1] Dialogs
  (if (> _returnvalue 0)
    (Variables|Dialog|SetConversationIndex (Math|Integer|Clamp(Integer) (+ (Variables|Dialog|GetConversationIndex) 1) 0 (- _returnvalue 1)))))

(event Custom|StopConversation
  ;[1 1 1] Dialogs
  (Variables|Dialog|SetTalking false)
  (Rendering|SetVisibility (Variables|Default|GetDialogWidget) false false)
  (Default|HideDialogBox (Variables|Default|GetWidget))
  (Audio|Components|Audio|Stop (Variables|Default|GetAudio))
  (Default|CleanDialogBox (Variables|Default|GetWidget)))

(event EventBeginPlay
  (|CallParentFunction)
  (CallFunction|SetDialogsfromDataTable)
  (Rendering|SetVisibility (Variables|Default|GetDialogWidget) false false)
  (bind _aswbp_dialog (Utilities|Casting|CastToWBP_Dialog (UserInterface|GetWidget (Variables|Default|GetDialogWidget))))
  (bind _output_get (Variables|Default|SetWidget _aswbp_dialog))
  (Default|SetOwner _output_get self))

(event EventInteractwith
  (params (Player :type BP%20Player%20Object%20Reference))
  ;[1 1 1] Interact
  (|CallParentFunction Player)
  (if (Variables|Dialog|GetTalking)
    (if (not (Variables|Dialog|GetIsQuest?))
      (bind _continue (CallFunction|NextDialog))
      (if _continue
        (CallFunction|ProcessDialog)
        (else
          (CallFunction|StopConversation)))
      (bind _dbmanager (Variables|Default|GetDBManager)
        (:then
          (Default|SendInteractEventtoDB _dbmanager (Utilities|Struct|MakeF_InteractEventsTableItem 0 (Variables|Default|GetActorId) (Variables|/Game/Game/Blueprints/Characters/Players/BP_Player.BP_Player_C|GetUserId (Variables|Default|GetPlayer)) "NewEnumerator0" "NewEnumerator20" (Math|DateTime|Now))))
        (:else)))
    (else
      (CallFunction|StartConversation)
      (bind _dbmanager_2 (Variables|Default|GetDBManager)
        (:then
          (Default|SendInteractEventtoDB _dbmanager_2 (Utilities|Struct|MakeF_InteractEventsTableItem 0 (Variables|Default|GetActorId) (Variables|/Game/Game/Blueprints/Characters/Players/BP_Player.BP_Player_C|GetUserId (Variables|Default|GetPlayer)) "NewEnumerator0" "NewEnumerator10" (Math|DateTime|Now))))
        (:else)))))

(event EventCancelInteract
  (params (Player :type BP%20Player%20Object%20Reference))
  ;[1 1 1] Interact
  (|CallParentFunction Player))

(event EventTick
  (params (DeltaSeconds :type Float%20%28single-precision%29))
  (bind _dialogwidget (Variables|Default|GetDialogWidget))
  (bind _player (Variables|Default|GetPlayer))
  (bind _returnvalue (Transformation|GetWorldLocation _dialogwidget))
  (bind _mesh (Variables|/Script/Engine.Character|GetMesh _player))
  (bind _returnvalue_2 (Transformation|GetWorldLocation _mesh))
  (bind _returnvalue_3 (Math|Rotator|FindLookatRotation _returnvalue _returnvalue_2))
  (|CallParentFunction DeltaSeconds)
  (Variables|Default|GetPlayer
    (:then
      (Transformation|SetWorldRotation _dialogwidget (Math|Rotator|MakeRotator (.roll _returnvalue_3) (.pitch (Transformation|GetWorldRotation _dialogwidget)) (.yaw _returnvalue_3)) false false))
    (:else)))

(fn ConstructionScript)

(fn NextDialog
  (bind _conversations (Variables|Dialog|GetConversations))
  (bind _conversationindex (Variables|Dialog|GetConversationIndex))
  (bind _output (Utilities|Array|Get(acopy) _conversations _conversationindex))
  (bind _dialogs (Utilities|Struct|BreakF_DialogsArray _output))
  (bind _returnvalue (Utilities|Array|Length _dialogs))
  (if (and (> _returnvalue 0) (< (+ (Variables|Dialog|GetDialogIndex) 1) _returnvalue))
    (Math|Integer|IncrementInt (Variables|Dialog|GetDialogIndex)
      (:%20%20
        (return true)))
    (else
      (return false))))

(fn SetDialogsfromDataTable
  (Utilities|Array|Clear (Variables|Dialog|GetConversations))
  (bind _dialog_data_table (Variables|Dialog|GetDialog%20Data%20Table)
    (:then
      (bind _returnvalue (Class|DataTableFunctionLibrary|GetDataTableColumnasString _dialog_data_table "Conversation Number"))
      (bind _number_of_conversations (CallFunction|GetNumberOfConversations _returnvalue))
      (Utilities|FlowControl|ForLoopwithBreak 0 (- _number_of_conversations 1)
        (:LoopBody
          (Utilities|Array|Add (Variables|Dialog|GetConversations) (Utilities|Struct|MakeF_DialogsArray)))
        (:Completed
          (bind _outrownames (DataTable|GetDataTableRowNames _dialog_data_table))
          (for _array_element _outrownames
            (bind _returnvalue_2 (Utilities|GetDataTableRow _dialog_data_table _array_element)
              (:then
                (Utilities|Array|Add (Utilities|Struct|BreakF_DialogsArray (Utilities|Array|Get(acopy) (Variables|Dialog|GetConversations) (.ConversationNumber (Utilities|Struct|BreakF_Dialog _returnvalue_2)))) (Utilities|Struct|MakeF_Dialog (.ConversationNumber (Utilities|Struct|BreakF_Dialog _returnvalue_2)) (.DialogData (Utilities|Struct|BreakF_Dialog _returnvalue_2)) (.QuestionFirstOption (Utilities|Struct|BreakF_Dialog _returnvalue_2)) (.QuestionSecondOption (Utilities|Struct|BreakF_Dialog _returnvalue_2))))))))))
    (:else)))

(fn GetNumberOfConversations
  (params (Dialogs :type Array%20of%20Strings))
  (for _array_element Dialogs
    (Utilities|Set|Add (LocalVariables|GetSet) _array_element))
  (return (Utilities|Set|Length (LocalVariables|GetSet))))

(fn GetDialog
  (return (Utilities|Array|Get(acopy) (Utilities|Struct|BreakF_DialogsArray (Utilities|Array|Get(acopy) (Variables|Dialog|GetConversations) (Variables|Dialog|GetConversationIndex))) (Variables|Dialog|GetDialogIndex))))

(fn AddOptionDialogstoConversation
  (params (New%20Dialogs :type Array%20of%20F%20Dialog%20Line%20Structures))
  (for (_array_element _array_index) New%20Dialogs
    (Utilities|Array|Insert (Utilities|Struct|BreakF_DialogsArray (Utilities|Array|Get(acopy) (Variables|Dialog|GetConversations) (Variables|Dialog|GetConversationIndex))) (Utilities|Struct|MakeF_Dialog (Variables|Dialog|GetConversationIndex) _array_element "(Text_18_6FC0436A42E8B2867021A5A58EEF0CC1=\"\",Dialogs_13_652B905E4A69557145CC91BF8F6D21E9=)" "(Text_18_6FC0436A42E8B2867021A5A58EEF0CC1=\"\",Dialogs_13_652B905E4A69557145CC91BF8F6D21E9=)") (+ (Variables|Dialog|GetDialogIndex) 1 _array_index))))