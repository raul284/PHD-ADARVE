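; Gameplay manager for Scenario 3 that extends a parent manager to drive a step-based VR tutorial with the Tuddy buddy.
; On player setup it locks the inventory, starts the introduction and binds delegates from tutorial, description panel, walkie-talkies, bollard place points and RBQ van.
; Handlers complete steps and trigger dialogs, syncing report state across walkie-talkies.
; It is unfinished: many handlers use S2 steps, several are stubs, and inventory unlock never runs.
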(event EventBeginPlay
  (|CallParentFunction)
  (CallFunction|BindItemActions)
  (CallFunction|BindNPCActions))

(event EventAddItemtoGameManagerImportantList
  (params (ItemType :type E_ItemType%20Enum :default "NewEnumerator2") (Actor :type Actor%20Object%20Reference))
  (switch Utilities|FlowControl|Switch|SwitchonE_ItemType ItemType
    (:NewEnumerator5
      (bind _asbp_walkie_talkie (Utilities|Casting|CastToBP_WalkieTalkie Actor))
      (Default|SetInitialConditions _asbp_walkie_talkie (Variables|Default|GetInitialReportCompleted) (Variables|Default|GetFinalReportCompleted))
      (CallFunction|BindWalkieTalkieEvents _asbp_walkie_talkie)
      (Utilities|Array|Add (Variables|Default|GetWalkieTalkieList) _asbp_walkie_talkie))))

(event EventSetPlayerData
  (|CallParentFunction)
  (CallFunction|BindPlayerActions)
  (Utilities|FlowControl|Sequence
    (:then_0
      (bind _asbp_player_vr (Utilities|Casting|CastToBP_Player_VR (Variables|Default|GetPlayer)))
      (bind _output_get (Variables|Default|SetTutorialBuddy (Variables|/Game/Game/Blueprints/Characters/Players/BP_Player_VR.BP_Player_VR_C|GetTutorialBuddyActor _asbp_player_vr)))
      (bind _tutorialmanager (Variables|Default|GetTutorialManager)
        (:then
          (Default|SetCurrentTutorialBuddy _tutorialmanager _output_get)
          (CallFunction|BindTuddyActions))
        (:else
          (Default|Log (Variables|Default|GetGameInstance) "NewEnumerator2" "Falta el TutorialManager" false))))
    (:then_1
      (bind _asbp_player_vr_2 (Utilities|Casting|CastToBP_Player_VR (Variables|Default|GetPlayer)))
      (Variables|/Game/Game/Blueprints/Characters/Players/BP_Player_VR.BP_Player_VR_C|SetCanOpenInventory _asbp_player_vr_2 false))
    (:then_2
      (CallFunction|StartScenario)
      (CallFunction|CompleteStep "NewEnumerator9"))))

(event EventStartScenario
  (|CallParentFunction)
  (Utilities|FlowControl|Delay 3.0)
  (CallFunction|SetCurrentGameplayStep "NewEnumerator59")
  (Default|StartExtraLinesDialog (Variables|Default|GetTutorialManager) "NewEnumerator13"))

(event Custom|BindInventoryActions
  (bind _asbp_player_vr (Utilities|Casting|CastToBP_Player_VR (Variables|Default|GetPlayer)))
  (EventDispatchers|AssignEDInventoryOpenned (Variables|/Game/Game/Blueprints/Characters/Players/BP_Player_VR.BP_Player_VR_C|GetInventoryActor _asbp_player_vr) (delegate Custom|OnInventoryOpen))
  (EventDispatchers|AssignEDInventoryClosed (Variables|/Game/Game/Blueprints/Characters/Players/BP_Player_VR.BP_Player_VR_C|GetInventoryActor _asbp_player_vr) (delegate Custom|OnInventoryClose)))

(event Custom|OnInventoryOpen
  (bind _yes (CallFunction|IsCurrentStep "NewEnumerator59"))
  (if _yes
    (Development|PrintString "Hello")))

(event Custom|OnInventoryClose)

(event EventBindPlayerActions
  (|CallParentFunction))

(event Custom|OnDescriptionCompleted
  (bind _yes (CallFunction|IsCurrentStep "NewEnumerator59"))
  (if _yes
    (CallFunction|CompleteStep "NewEnumerator59")
    (CallFunction|SetCurrentGameplayStep "NewEnumerator59")
    (Utilities|FlowControl|Delay 2.0)
    (Default|StartExtraLinesDialog (Variables|Default|GetTutorialManager) "NewEnumerator14")))

(event Custom|BindWalkieTalkieEvents
  (params (WalkieTalkie :type BP%20Walkie%20Talkie%20Object%20Reference))
  (EventDispatchers|BindEventtoEDInteractionStarted WalkieTalkie (delegate Custom|OnWalkieGrabbed))
  (EventDispatchers|BindEventtoEDInitialReportCompleted WalkieTalkie (delegate Custom|OnWalkieInitialReportCompleted))
  (EventDispatchers|BindEventtoEDFinalReportCompleted WalkieTalkie (delegate Custom|OnWalkieFinalReportCompleted)))

(event Custom|BindSAGB100Actions
  (params (SABG100 :type BP%20Dosimeter%20SABG100%20Object%20Reference))
  (EventDispatchers|AssignEDItemRadiationMeasured SABG100 (delegate Custom|OnSABG100ItemRadiationMeasured))
  (EventDispatchers|AssignEDNPCRadiationMeasured SABG100 (delegate Custom|ONSABG100NPCRadiationMeasured)))

(event Custom|BindEPDActions
  (params (EPD :type BP%20Dosimeter%20EPD%20Object%20Reference)))

(event Custom|OnSABG100ItemRadiationMeasured
  (params (Actor :type BP%20Interact%20Item%20Parent%20Object%20Reference))
  (CallFunction|CompleteStep "NewEnumerator5"))

(event Custom|ONSABG100NPCRadiationMeasured
  (params (Actor :type BP%20NPC%20Object%20Reference))
  (Utilities|Casting|CastToBP_NPC_S2_Driver Actor)
  (CallFunction|CompleteStep "NewEnumerator4"))

(event Custom|OnRBQItemSpawned
  (params (Actor :type BP%20Item%20Initial%20State%20Object%20Reference))
  (switch Utilities|FlowControl|Switch|SwitchonE_ItemType (Variables|/Game/Game/Blueprints/Actors/Items/BP_ItemInitialState.BP_ItemInitialState_C|GetItemType Actor)))

(event Custom|OnWalkieInitialReportCompleted
  (bind _yes (CallFunction|IsCurrentStep "NewEnumerator49"))
  (Variables|Default|SetInitialReportCompleted _yes)
  (for _array_element (Variables|Default|GetWalkieTalkieList)
    (Default|SetInitialConditions _array_element (Variables|Default|GetInitialReportCompleted) (Variables|Default|GetFinalReportCompleted)))
  (CallFunction|CompleteStep "NewEnumerator49")
  (Utilities|FlowControl|Delay 1.0)
  (CallFunction|SetCurrentGameplayStep "NewEnumerator55")
  (Default|StartExtraLinesDialog (Variables|Default|GetTutorialManager) "NewEnumerator9"))

(event Custom|OnWalkieFinalReportCompleted
  (Variables|Default|SetFinalReportCompleted true)
  (for _array_element (Variables|Default|GetWalkieTalkieList)
    (Default|SetInitialConditions _array_element (Variables|Default|GetInitialReportCompleted) (Variables|Default|GetFinalReportCompleted))
    (CallFunction|CompleteStep "NewEnumerator6")
    (Utilities|FlowControl|Delay 1.0)
    (CallFunction|SetCurrentGameplayStep "NewEnumerator54")
    (Default|StartExtraLinesDialog (Variables|Default|GetTutorialManager) "NewEnumerator11")))

(event Custom|BindRBQVanEvents
  (bind _rbqvan (Variables|Default|GetRBQVan)
    (:then
      (EventDispatchers|BindEventtoEDItemSpawned _rbqvan (delegate Custom|OnRBQItemSpawned)))
    (:else
      (Default|Log (Variables|Default|GetGameInstance) "NewEnumerator2" "Falta RBQ Van" false))))

(event Custom|BindDescriptionPanelEvents
  (bind _descriptionpanel (Variables|Default|GetDescriptionPanel)
    (:then
      (EventDispatchers|BindEventtoEDDescriptionCompleted _descriptionpanel (delegate Custom|OnDescriptionCompleted)))
    (:else
      (Default|Log (Variables|Default|GetGameInstance) "NewEnumerator2" "Falta el DescriptionPanel" false))))

(event Custom|OnWalkieGrabbed
  (bind _yes (CallFunction|IsCurrentStep "NewEnumerator49"))
  (if _yes
    (Default|HideAutomaticHintPanel (Variables|Default|GetTutorialManager))
    (Default|HideCurrentTuddy (Variables|Default|GetTutorialManager))))

(event Custom|OnOneSecurityBollardHasBeenPlaced
  (params (Item :type BP%20Pickable%20Item%20Object%20Reference) (PlacePoint :type BP%20Place%20Point%20Object%20Reference))
  (CallFunction|CompleteStep "NewEnumerator3"))

(event EventBindItemActions
  (|CallParentFunction)
  (CallFunction|BindDescriptionPanelEvents)
  (CallFunction|BindRBQVanEvents)
  (CallFunction|BindPlacePointsActions))

(event EventBindPlacePointsActions
  (|CallParentFunction)
  (bind _securitybollardplacepointmanager (Variables|Default|GetSecurityBollardPlacePointManager)
    (:then
      (EventDispatchers|AssignEDOneItemHasBeenPlaced _securitybollardplacepointmanager (delegate Custom|OnOneSecurityBollardHasBeenPlaced)))
    (:else
      (Default|Log (Variables|Default|GetGameInstance) "NewEnumerator2" "Falta el PlacePointManager de los \"postes de balizamiento\"" false))))

(event EventBindNPCActions
  (|CallParentFunction))

(event Custom|OnInventoryDescriptionExtraLines
  (bind _yes (CallFunction|IsCurrentStep "NewEnumerator60"))
  (if _yes
    (Default|AutomaticCall (Variables|Default|GetTutorialManager) "NewEnumerator12")
    (bind _asbp_player_vr (Utilities|Casting|CastToBP_Player_VR (Variables|Default|GetPlayer)))
    (Variables|/Game/Game/Blueprints/Characters/Players/BP_Player_VR.BP_Player_VR_C|SetCanOpenInventory _asbp_player_vr true)))

(event Custom|OnTuddyIntroductionCompleted
  (Default|StartDescription (Variables|Default|GetDescriptionPanel)))

(event Custom|BindTutorialManagerActions
  (EventDispatchers|BindEventtoEDTutorialDemanded (Variables|Default|GetTutorialManager) (delegate Custom|OnTutorialDemanded)))

(event Custom|OnTutorialDemanded)

(event Custom|OnTuddyDialogCompleted
  (params (CurrentTuddyDialogType :type E_TuddyDialogLinesType%20Enum :default "NewEnumerator0"))
  (switch Utilities|FlowControl|Switch|SwitchonE_GameplayStepTypes (Variables|Default|GetCurrentStepType)))

(event EventBindTuddyActions
  (|CallParentFunction)
  (EventDispatchers|BindEventtoEDDialogCompleted (Variables|/Game/Game/Blueprints/Tutorial/BP_TutorialBuddy.BP_TutorialBuddy_C|GetAC_TuddyDialogManager (Variables|/Game/Game/Blueprints/Tutorial/BP_TutorialManager.BP_TutorialManager_C|GetCurrentTutorialBuddy (Variables|Default|GetTutorialManager))) (delegate Custom|OnTuddyDialogCompleted))
  (CallFunction|BindTutorialManagerActions))

(fn ConstructionScript
  (|CallParentFunction))