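; AC_Database is an actor component that logs simulation radiation and RBQ events to the game instance's DatabaseManager.
; On BeginPlay it caches the game instance and owner, then re-broadcasts the manager's database closing and closed events through its own dispatchers.
; Send events package user ID and scenario type with recorded dose, position and time arrays from a player or EPD dosimeter owner, or with RBQ actor data.
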(event Custom|BindDatabaseEvents
  (bind _database_manager (Variables|/Game/Game/Blueprints/RR_GameInstance.RR_GameInstance_C|GetDatabase%20Manager (Variables|Default|GetGame%20Instance))
    (:then
      (EventDispatchers|AssignEDDatabaseNeedtobeClosed _database_manager (delegate Custom|OnDatabaseNeedToBeClosed))
      (EventDispatchers|AssignEDDatabaseClosed _database_manager (delegate Custom|OnDatabaseClosed)))
    (:else)))

(event Custom|OnDatabaseNeedToBeClosed
  (Default|CallEDDatabaseNeedtobeClosed))

(event Custom|OnDatabaseClosed
  (Default|CallEDDatabaseClosed))

(event EventBeginPlay
  (Utilities|FlowControl|Sequence
    (:then_0
      (bind _asrr_game_instance (Utilities|Casting|CastToRR_GameInstance (Game|GetGameInstance)))
      (Variables|Default|SetGame%20Instance _asrr_game_instance)
      (Variables|Default|SetOwner (Components|GetOwner)))
    (:then_1
      (CallFunction|BindDatabaseEvents))))

(event Custom|SendEPDRadiationEventToDB
  (bind _data (Default|GetDataBaseMainInfoEvent (Variables|Default|GetGame%20Instance)))
  (bind _asbp_dosimeter_epd (Utilities|Casting|CastToBP_Dosimeter_EPD (Variables|Default|GetOwner)))
  (bind _database_manager (Variables|/Game/Game/Blueprints/RR_GameInstance.RR_GameInstance_C|GetDatabase%20Manager (Variables|Default|GetGame%20Instance))
    (:then
      (Default|SendEPDRadiationEventtoDB _database_manager (Utilities|Struct|MakeF_EPDRadiationEvent 0 (.user_id (Utilities|Struct|BreakF_MainInfoEvent _data)) (.scenario_type (Utilities|Struct|BreakF_MainInfoEvent _data)) (Variables|/Game/Game/Blueprints/Actors/Dosimeters/BP_Dosimeter_EPD.BP_Dosimeter_EPD_C|GetEPDId _asbp_dosimeter_epd) (Variables|/Game/Game/Blueprints/Actors/Dosimeters/BP_Dosimeter_EPD.BP_Dosimeter_EPD_C|GetCurrentEventDoseRateArray _asbp_dosimeter_epd) (Variables|/Game/Game/Blueprints/Actors/Dosimeters/BP_Dosimeter_EPD.BP_Dosimeter_EPD_C|GetCurrentEventDoseAbsortionArray _asbp_dosimeter_epd) (Variables|/Game/Game/Blueprints/Actors/Dosimeters/BP_Dosimeter_EPD.BP_Dosimeter_EPD_C|GetCurrentEventPositionArray _asbp_dosimeter_epd) (Variables|/Game/Game/Blueprints/Actors/Dosimeters/BP_Dosimeter_EPD.BP_Dosimeter_EPD_C|GetCurrentEventDatetimeArray _asbp_dosimeter_epd))))
    (:else)))

(event Custom|SendRBQEventToDB
  (params (actor_id :type Array%20of%20Integers) (num_of_actors :type Array%20of%20Integers))
  (bind _data (Default|GetDataBaseMainInfoEvent (Variables|Default|GetGame%20Instance)))
  (Default|SendRBQEventtoDB (Variables|/Game/Game/Blueprints/RR_GameInstance.RR_GameInstance_C|GetDatabase%20Manager (Variables|Default|GetGame%20Instance)) (Utilities|Struct|MakeF_RBQEvent 0 (.user_id (Utilities|Struct|BreakF_MainInfoEvent _data)) (.scenario_type (Utilities|Struct|BreakF_MainInfoEvent _data)) actor_id num_of_actors (Math|DateTime|Now))))

(event Custom|SendUserRadiationEventToDB
  (bind _returnvalue (Actor|GetActorOfClass "/Game/Game/Blueprints/Actors/Radiation/BP_RadiationEmissionPoint.BP_RadiationEmissionPoint_C"))
  (Utilities|IsValid _returnvalue
    (:Is%20Valid
      (bind _data (Default|GetDataBaseMainInfoEvent (Variables|Default|GetGame%20Instance)))
      (bind _asbp_player (Utilities|Casting|CastToBP_Player (Variables|Default|GetOwner)))
      (bind _database_manager (Variables|/Game/Game/Blueprints/RR_GameInstance.RR_GameInstance_C|GetDatabase%20Manager (Variables|Default|GetGame%20Instance))
        (:then
          (Default|SendUserRadiationEventtoDB _database_manager (Utilities|Struct|MakeF_UserRadiationEvent 0 (.user_id (Utilities|Struct|BreakF_MainInfoEvent _data)) (.scenario_type (Utilities|Struct|BreakF_MainInfoEvent _data)) (Variables|/Game/Game/Blueprints/Characters/Players/BP_Player.BP_Player_C|GetCurrentEventRadiationDoseRateArray _asbp_player) (Variables|/Game/Game/Blueprints/Characters/Players/BP_Player.BP_Player_C|GetCurrentEventDoseRadiationAbsortionArray _asbp_player) (Variables|/Game/Game/Blueprints/Characters/Players/BP_Player.BP_Player_C|GetCurrentEventRadiationPositionArray _asbp_player) (Variables|/Game/Game/Blueprints/Characters/Players/BP_Player.BP_Player_C|GetCurrentEventRadiationDatetimeArray _asbp_player))))
        (:else)))))