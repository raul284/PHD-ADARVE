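; Database manager actor that routes experiment telemetry (sessions, users, teams, experiments, interact, gameplay and move events) to database backends.
; On BeginPlay, the authority spawns BP_Database_Server and relays its closed event through its own DatabaseClosed dispatcher.
; Send events forward insert queries to each valid backend, while user ID lookup and closing target only the server.
; The local-file backend's spawn is disconnected here.
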(event Custom|Send%20Experiment%20to%20DB
  (params (Data :type F%20Experiment%20Table%20Item%20Structure))
  (Utilities|FlowControl|Sequence
    (:then_0
      (bind _serverdb (Variables|Default|GetServerDB)
        (:then
          (Default|CreateExperimentInsertQuery _serverdb Data))
        (:else)))
    (:then_1
      (bind _localfiledb (Variables|Default|GetLocalFileDB)
        (:then
          (Default|CreateExperimentInsertQuery _localfiledb Data))
        (:else)))))

(event Custom|Send%20Session%20to%20DB
  (params (Data :type F%20Session%20Table%20Item%20Structure))
  (Utilities|FlowControl|Sequence
    (:then_0
      (bind _serverdb (Variables|Default|GetServerDB)
        (:then
          (Default|CreateSessionInsertQuery _serverdb Data))
        (:else)))
    (:then_1
      (bind _localfiledb (Variables|Default|GetLocalFileDB)
        (:then
          (Default|CreateSessionInsertQuery _localfiledb Data))
        (:else)))))

(event Custom|Get%20User%20Id
  (params (Player%20Name :type String))
  (Utilities|FlowControl|Sequence
    (:then_0
      (bind _serverdb (Variables|Default|GetServerDB)
        (:then
          (Class|BIDatabase|GetUserId(Message) _serverdb Player%20Name))
        (:else)))))

(event Custom|Send%20Interact%20Event%20to%20DB
  (params (Data :type F%20Interact%20Events%20Table%20Item%20Structure))
  (Utilities|FlowControl|Sequence
    (:then_0
      (bind _serverdb (Variables|Default|GetServerDB)
        (:then
          (Default|CreateInteractEventInsertQuery _serverdb Data))
        (:else)))
    (:then_1
      (bind _localfiledb (Variables|Default|GetLocalFileDB)
        (:then
          (Default|CreateInteractEventInsertQuery _localfiledb Data))
        (:else)))))

(event Custom|Send%20Move%20Event%20to%20DB
  (params (Data :type F%20Move%20Events%20Table%20Item%20Structure))
  (Utilities|FlowControl|Sequence
    (:then_0
      (bind _serverdb (Variables|Default|GetServerDB)
        (:then
          (Default|CreateMoveEventQuery _serverdb Data))
        (:else)))
    (:then_1
      (bind _localfiledb (Variables|Default|GetLocalFileDB)
        (:then
          (Default|CreateMoveEventQuery _localfiledb Data))
        (:else)))))

(event Custom|Send%20Gameplay%20Event%20to%20DB
  (params (Data :type F%20Gameplay%20Events%20Table%20Item%20Structure))
  (Utilities|FlowControl|Sequence
    (:then_0
      (bind _serverdb (Variables|Default|GetServerDB)
        (:then
          (Default|CreateGameplayEventInsertQuery _serverdb Data))
        (:else)))
    (:then_1
      (bind _localfiledb (Variables|Default|GetLocalFileDB)
        (:then
          (Default|CreateGameplayEventInsertQuery _localfiledb Data))
        (:else)))))

(event Custom|CloseDatabase
  (bind _serverdb (Variables|Default|GetServerDB)
    (:then
      (Default|CloseDatabase _serverdb))
    (:else)))

(event Custom|Send%20User%20to%20DB
  (params (Data :type F%20User%20Table%20Item%20Structure))
  (Utilities|FlowControl|Sequence
    (:then_0
      (bind _serverdb (Variables|Default|GetServerDB)
        (:then
          (Default|CreateUserInsertQuery _serverdb Data))
        (:else)))
    (:then_1
      (bind _localfiledb (Variables|Default|GetLocalFileDB)
        (:then
          (Default|CreateUserInsertQuery _localfiledb Data))
        (:else)))))

(event Custom|ServerDatabaseClosed
  (Variables|Default|SetServerClosed true)
  (Default|CallEDDatabaseClosed))

(event Custom|Send%20Team%20to%20DB
  (params (Data :type F%20Team%20Table%20Item%20Structure))
  (Utilities|FlowControl|Sequence
    (:then_0
      (bind _serverdb (Variables|Default|GetServerDB)
        (:then
          (Default|CreateTeamInsertQuery _serverdb Data))
        (:else)))
    (:then_1
      (bind _localfiledb (Variables|Default|GetLocalFileDB)
        (:then
          (Default|CreateTeamInsertQuery _localfiledb Data))
        (:else)))))

(event EventBeginPlay
  (Networking|SwitchHasAuthority
    (:Authority
      (bind _returnvalue (Game|SpawnActorfromClass "/Game/Game/Blueprints/Database/BP_Database_Server.BP_Database_Server_C" (Math|Transform|MakeTransform "0, 0, 0") "Undefined" 0 0))
      (bind _output_get (Variables|Default|SetServerDB _returnvalue))
      (EventDispatchers|BindEventtoEDServerDatabaseClosed _output_get (delegate Custom|ServerDatabaseClosed)))))

(fn ConstructionScript)