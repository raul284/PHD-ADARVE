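; Manager for placeable traffic cone items that completes a gameplay step once all cones are placed.
; It extends a parent placement manager, calling the parent's AllItemsPlaced logic, then checking AreAllItemPlaced before notifying GameplayManager.
; Its ActivateAllPoints override is empty, with the parent call left disconnected, so the inherited activation logic does not run through that event.
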(event EventBeginPlay
  (|CallParentFunction))

(event EventActivateAllPoints
  (params (Activate :type Boolean)))

(event EventAllItemsPlaced
  (|CallParentFunction)
  (if (Variables|Default|GetAreAllItemPlaced)
    (Default|CompleteStep (Variables|Default|GetGameplayManager) "NewEnumerator3")))

(fn ConstructionScript
  (|CallParentFunction))