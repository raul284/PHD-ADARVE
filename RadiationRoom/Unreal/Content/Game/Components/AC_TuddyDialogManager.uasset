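; Actor component that runs the speech-bubble dialog of the tutorial buddy (Tuddy).
; Init caches the owning BP_TutorialBuddy, its bubble widget and its typewriter component.
; Dialogs start from passed-in lines or a data table row ID, and each line advances after a short delay once typing completes.
; Event dispatchers report start, stop and completion, the last carrying dialog type, extra-line type and ID.
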(event Custom|OnTypewriterCompleted
  (if (Variables|Default|GetIsTalking?)
    (Utilities|FlowControl|Delay 1.5)
    (CallFunction|NextDialog)))

(event Custom|StartNewExtraLineDialog
  (params (ExtraLineType :type E_TuddyExtraLineTypes%20Enum :default "NewEnumerator1") (TuddyDialogType :type E_TuddyDialogLinesType%20Enum :default "NewEnumerator0") (DialogLines :type Array%20of%20Texts))
  (Variables|Default|SetCurrentExtraLineType ExtraLineType)
  (CallFunction|StartNewDialog TuddyDialogType DialogLines))

(event Custom|ProcessDialog
  (Default|SetDialogText (Variables|Default|GetWidget) (Utilities|Array|Get(acopy) (Variables|Default|GetCurrentDialogLines) (Variables|Default|GetCurrentDialogIndex)) (Variables|Default|GetTypewriterComponent)))

(event Custom|NextDialog
  (bind _there_are_more_dialogs (CallFunction|MoreDialogLines?))
  (if _there_are_more_dialogs
    (Variables|Default|SetCurrentDialogIndex (+ (Variables|Default|GetCurrentDialogIndex) 1))
    (CallFunction|ProcessDialog)
    (else
      (CallFunction|EndDialog))))

(event Custom|StopDialog
  (Default|HideDialogBubble (Variables|Default|GetOwner))
  (Variables|Default|SetIsTalking? false)
  (Default|CallEDDialogStopped))

(event Custom|EndDialog
  (CallFunction|ResetDialogValues)
  (Default|HideDialogBubble (Variables|Default|GetOwner))
  (Variables|Default|SetIsTalking? false)
  (Default|CallEDDialogCompleted (Variables|Default|GetCurrentTuddyDialogType) (Variables|Default|GetCurrentExtraLineType) (Variables|Default|GetCurrentDialogID))
  (Variables|Default|SetCurrentExtraLineType "NewEnumerator1")
  (Variables|Default|SetCurrentDialogID "None"))

(event Custom|ResetDialogValues
  (Utilities|Array|Clear (Variables|Default|GetCurrentDialogLines))
  (Variables|Default|SetCurrentDialogIndex 0))

(event Custom|Init
  (Utilities|FlowControl|Sequence
    (:then_0
      (bind _asbp_tutorial_buddy (Utilities|Casting|CastToBP_TutorialBuddy (Components|GetOwner)))
      (Variables|Default|SetOwner _asbp_tutorial_buddy))
    (:then_1
      (bind _aswbp_tutorial_buddy_dialog_pannel (Utilities|Casting|CastToWBP_TutorialBuddyDialogPannel (UserInterface|GetWidget (Variables|/Game/Game/Blueprints/Tutorial/BP_TutorialBuddy.BP_TutorialBuddy_C|GetDialogBubbleWidgetComponent (Variables|Default|GetOwner)))))
      (Variables|Default|SetWidget _aswbp_tutorial_buddy_dialog_pannel))
    (:then_2
      (bind _output_get (Variables|Default|SetTypewriterComponent (Variables|/Game/Game/Blueprints/Tutorial/BP_TutorialBuddy.BP_TutorialBuddy_C|GetTypewriterText (Variables|Default|GetOwner))))
      (EventDispatchers|BindEventtoOnCompleted _output_get (delegate Custom|OnTypewriterCompleted)))))

(event Custom|StartNewDialog
  (params (TuddyDialogType :type E_TuddyDialogLinesType%20Enum :default "NewEnumerator0") (DialogLines :type Array%20of%20Texts))
  (CallFunction|ResetDialogValues)
  (Variables|Default|SetCurrentTuddyDialogType TuddyDialogType)
  (Variables|Default|SetCurrentDialogLines DialogLines)
  (Variables|Default|SetIsTalking? true)
  (Default|CallEDDialogStarted)
  (Default|ShowDialogBubble (Variables|Default|GetOwner))
  (CallFunction|ProcessDialog))

(event Custom|StartNewDialogByID
  (params (Dialog%20ID :type Name))
  (bind _returnvalue (Utilities|GetDataTableRow (Variables|Default|GetExtraLinesDialogDataTable) Dialog%20ID)
    (:then
      (Variables|Default|SetCurrentDialogLines (.ListOfLines (Utilities|Struct|BreakF_TuddyExtraLines _returnvalue)))
      (Variables|Default|SetCurrentDialogID Dialog%20ID)
      (Variables|Default|SetIsTalking? true)
      (Default|CallEDDialogStarted)
      (Default|ShowDialogBubble (Variables|Default|GetOwner))
      (CallFunction|ProcessDialog))))

(event EventBeginPlay)

(fn MoreDialogLines?
  (return (< (Variables|Default|GetCurrentDialogIndex) (- (Utilities|Array|Length (Variables|Default|GetCurrentDialogLines)) 1))))