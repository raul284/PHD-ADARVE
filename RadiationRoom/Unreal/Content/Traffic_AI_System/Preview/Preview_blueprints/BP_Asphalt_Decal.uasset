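; BP_Asphalt_Decal is an asphalt decal actor from the Traffic AI System preview content that snaps itself to the surface at its location.
; Its construction script runs a vertical WorldStatic line trace through the decal, ignoring all BP_Road_preview actors.
; On a hit, it moves the Decal component to the impact point; there is no active runtime logic.
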(event EventBeginPlay)

(event EventTick
  (params (DeltaSeconds :type Float%20%28single-precision%29)))

(fn ConstructionScript
  (bind _decal (Variables|Decal|GetDecal))
  (bind _returnvalue (Transformation|GetWorldLocation _decal))
  (bind _outactors (Actor|GetAllActorsOfClass "/Game/Traffic_AI_System/Preview/Preview_blueprints/BP_Road_preview.BP_Road_preview_C"))
  (bind (_outhit _returnvalue_2) (Collision|LineTraceForObjects (+ _returnvalue "0, 0,300.000000") (+ _returnvalue "0, 0,-300.000000") (Utilities|Array|MakeArray "ObjectTypeQuery1") false _outactors "None"))
  (if _returnvalue_2
    (Transformation|SetWorldLocation (Variables|Decal|GetDecal) (.ImpactPoint (Collision|BreakHitResult _outhit)) false false)))