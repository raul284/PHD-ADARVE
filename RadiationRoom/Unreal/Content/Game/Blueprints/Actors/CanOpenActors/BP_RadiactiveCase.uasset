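; BP_RadiactiveCase is a VR case actor whose lid opens as the player drags its grabbed knob.
; It binds to the grab-status event of a BP_HandlePoint child actor and, while held, updates the lid each Tick.
; SetOpenAngle pitches TopCasePivot from the look-at angle between motion controller and pivot, minus a hard-coded offset.
; The AngleOffset input is ignored and the angle clamp is unconnected, so rotation is unclamped.
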(event Custom|OnKnobStatusChanged
  (params (Grabbed :type Boolean))
  (bind _output_get (Variables|Default|SetKnob%20Grabbed Grabbed))
  (if _output_get
    _))

(event EventBeginPlay
  (bind _asbp_handle_point (Utilities|Casting|CastToBP_HandlePoint (Variables|/Script/Engine.ChildActorComponent|GetChildActor (Variables|Default|GetKnob1))))
  (bind _output_get (Variables|Default|SetKnob _asbp_handle_point))
  (EventDispatchers|BindEventtoEDonKnobGrabStatusChanged _output_get (delegate Custom|OnKnobStatusChanged)))

(event EventTick
  (params (DeltaSeconds :type Float%20%28single-precision%29))
  (if (Variables|Default|GetKnob%20Grabbed)
    (bind _current_motion_controller (Variables|/Game/Game/Blueprints/Actors/Items/BP_PickableItem.BP_PickableItem_C|GetCurrent%20Motion%20Controller (Variables|Default|GetKnob))
      (:then
        (CallFunction|SetOpenAngle _current_motion_controller 85.0))
      (:else))))

(fn ConstructionScript)

(fn SetOpenAngle
  (params (MotionController :type Motion%20Controller%20Component%20Object%20Reference) (AngleOffset :type Float%20%28double-precision%29))
  (Transformation|SetRelativeRotation (Variables|Default|GetTopCasePivot) (Math|Rotator|MakeRotator 0.0 (- (.pitch (Math|Rotator|FindLookatRotation (Transformation|GetWorldLocation MotionController) (Transformation|GetWorldLocation (Variables|Default|GetTopCasePivot)))) 1.2e+02) 0.0) false false))