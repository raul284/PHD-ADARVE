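; Gameplay manager for scenario S1, a VR tutorial covering teleporting, item detection and grabbing, NPC conversation and tidying up.
; Extends parent bindings to player, tutorial buddy ("Tuddy"), item, place-point and NPC events, advancing quests behind current-quest checks.
; Dialog completions unlock items and doors by step type, while helper functions test phase completion across item and place-point arrays.
; Items spawn through delayed recursion, and entering the big room swaps the standalone buddy for the player's own.
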(event Custom|SetCurrentTuddyOnTutorialManager
  (params (Tuddy :type BP%20Tutorial%20Buddy%20Object%20Reference))
  (Default|SetCurrentTutorialBuddy (Variables|Default|GetTutorialManager) Tuddy)
  (CallFunction|BindTuddyActions))

(event EventBeginPlay
  (|CallParentFunction)
  (Utilities|FlowControl|Sequence
    (:then_0
      (for _array_element (Variables|Default|GetFirstRoomItems)
        (Rendering|SetActorHiddenInGame _array_element true)))
    (:then_1
      (CallFunction|SetCurrentTuddyonTutorialManager (Variables|Tuddy|GetIndependentTutorialBuddy))
      (Default|HideCurrentTuddy (Variables|Default|GetTutorialManager)))
    (:then_2
      (CallFunction|BindItemActions)
      (CallFunction|BindPlacePointsActions)
      (CallFunction|BindTuddyActions)
      (CallFunction|BindNPCActions))
    (:then_3
      (Default|SetActive (Variables|DestinationPoints|GetTableDestinationPoint) false))
    (:then_4
      (CallFunction|StartScenario)
      (Utilities|FlowControl|Delay 0.2)
      (CallFunction|CompleteQuest "None"))))

(event EventTick
  (params (DeltaSeconds :type Float%20%28single-precision%29)))

(event EventSetPlayerData
  (CallFunction|BindPlayerActions))

(event EventStartScenario
  (|CallParentFunction)
  (Utilities|FlowControl|Delay 3.0))

(event Custom|OnTuddyIntroductionDialogCompleted
  (if (CallFunction|IsCurrentQuest "None")
    (CallFunction|CompleteQuest "None")))

(event Custom|OnTuddyIsOnHand
  (if (CallFunction|IsCurrentQuest "None")
    (CallFunction|CompleteQuest "None")))

(event Custom|OnFinalConversationCompleted
  (if (CallFunction|IsCurrentQuest "None")
    (CallFunction|CompleteQuest "None")))

(event Custom|OnTuddyDialogCompleted
  (params (CurrentTuddyDialogType :type E_TuddyDialogLinesType%20Enum :default "NewEnumerator0") (CurrentExtraLineType :type E_TuddyExtraLineTypes%20Enum :default "NewEnumerator1") (DialogID :type Name))
  (switch Utilities|FlowControl|Switch|SwitchonE_GameplayStepTypes (Variables|Default|GetCurrentStepType)
    (:NewEnumerator39
      (CallFunction|OnTuddyIntroductionDialogCompleted))
    (:NewEnumerator40
      (for _array_element (Variables|Default|GetFirstRoomItems)
        (Variables|/Game/Game/Blueprints/Actors/Items/BP_TutorialPickableItem.BP_TutorialPickableItem_C|SetCanBeDetected _array_element true)))
    (:NewEnumerator41
      (for _array_element_2 (Variables|Default|GetFirstRoomItems)
        (Variables|/Game/Game/Blueprints/Actors/Items/BP_TutorialPickableItem.BP_TutorialPickableItem_C|SetCanBeGrabbed _array_element_2 true)))
    (:NewEnumerator48
      (Default|AutomaticOpenandLockDoor (Variables|Door|GetBigRoomDoor)))
    (:NewEnumerator43
      (CallFunction|OnTuddyIsonHand))
    (:NewEnumerator47
      (CallFunction|OnFinalConversationCompleted))))

(event EventBindTuddyActions
  (|CallParentFunction)
  (EventDispatchers|BindEventtoEDDialogCompleted (Variables|/Game/Game/Blueprints/Tutorial/BP_TutorialBuddy.BP_TutorialBuddy_C|GetAC_TuddyDialogManager (Variables|/Game/Game/Blueprints/Tutorial/BP_TutorialManager.BP_TutorialManager_C|GetCurrentTutorialBuddy (Variables|Default|GetTutorialManager))) (delegate Custom|OnTuddyDialogCompleted)))

(event Custom|UserEnterBigRoom
  (params (OverlappedActor :type Actor%20Object%20Reference) (OtherActor :type Actor%20Object%20Reference))
  (if (CallFunction|IsCurrentQuest "None")
    (if (== OtherActor (CallFunction|GetMyPlayer))
      (Actor|DestroyActor (Variables|Tuddy|GetIndependentTutorialBuddy))
      (bind _asbp_player_vr (Utilities|Casting|CastToBP_Player_VR (CallFunction|GetMyPlayer)))
      (bind _output_get (Variables|Tuddy|SetWrispTutorialBuddy (Variables|/Game/Game/Blueprints/Characters/Players/BP_Player_VR.BP_Player_VR_C|GetTutorialBuddyActor _asbp_player_vr)))
      (CallFunction|SetCurrentTuddyonTutorialManager _output_get)
      (CallFunction|CompleteQuest "None"))))

(event Custom|OnPlayerEnterOnTableDestinationPoint
  (if (and (CallFunction|IsCurrentQuest "None") (>= (Variables|Default|GetTimesTeleported) 5))
    (Default|SetActive (Variables|DestinationPoints|GetTableDestinationPoint) false)))

(event Custom|UserEnterExitRoom
  (params (OverlappedActor :type Actor%20Object%20Reference) (OtherActor :type Actor%20Object%20Reference))
  (if (CallFunction|IsCurrentQuest "None")
    (if (== OtherActor (CallFunction|GetMyPlayer))
      (CallFunction|CompleteQuest "None")
      (CallFunction|EndGameplay))))

(event Custom|OnPlayerTeleported
  (if (CallFunction|IsCurrentQuest "None")
    (bind _output_get (Variables|Default|SetTimesTeleported (+ (Variables|Default|GetTimesTeleported) 1)))
    (if (== _output_get 5)
      (Default|Activate (Variables|Default|GetConfetti%20Niagara%20System))
      (Default|HideAutomaticHintPanel (Variables|Default|GetTutorialManager))
      (CallFunction|CompleteQuest "None")
      (Utilities|FlowControl|Delay 1.0)
      (CallFunction|SpawnFirstRoomItems))))

(event EventBindPlayerActions
  (|CallParentFunction)
  (EventDispatchers|BindEventtoEDTeleported (CallFunction|GetMyPlayer) (delegate Custom|OnPlayerTeleported))
  (EventDispatchers|BindEventtoEDPlayerEnteronDestinationPoint (Variables|DestinationPoints|GetTableDestinationPoint) (delegate Custom|OnPlayerEnterOnTableDestinationPoint))
  (Collision|BindEventtoOnActorBeginOverlap (Variables|Triggers|GetBigRoomTrigger) (delegate Custom|UserEnterBigRoom))
  (Collision|BindEventtoOnActorBeginOverlap (Variables|Triggers|GetExitRoomTrigger) (delegate Custom|UserEnterExitRoom)))

(event Custom|SpawnFirstRoomItems
  (params (Actor%20Index :type Integer))
  (if (< Actor%20Index (Utilities|Array|Length (Variables|Default|GetFirstRoomItems)))
    (Default|Spawn (Utilities|Array|Get(acopy) (Variables|Default|GetFirstRoomItems) Actor%20Index))
    (Utilities|FlowControl|Delay 0.7)
    (CallFunction|SpawnFirstRoomItems (+ Actor%20Index 1))
    (else
      (Default|CallEDFirstRoomItemsSpawned))))

(event Custom|OnTutorialItemDetected
  (params (Actor :type BP%20Interact%20Item%20Parent%20Object%20Reference))
  (if (CallFunction|IsCurrentQuest "None")
    (bind _completed (CallFunction|IsTutorialItemDetectionPhaseCompleted?))
    (if _completed
      (Default|HideAutomaticHintPanel (Variables|Default|GetTutorialManager))
      (CallFunction|CompleteQuest "None"))))

(event Custom|OnOneItemPlaced
  (params (Item :type BP%20Pickable%20Item%20Object%20Reference) (PlacePoint :type BP%20Place%20Point%20Object%20Reference))
  (if (CallFunction|IsCurrentQuest "None")
    (Default|HideAutomaticHintPanel (Variables|Default|GetTutorialManager))
    (Default|HideCurrentTuddy (Variables|Default|GetTutorialManager))))

(event Custom|OnTutorialItemGrabbed
  (params (Actor :type BP%20Interact%20Item%20Parent%20Object%20Reference))
  (if (CallFunction|IsCurrentQuest "None")
    (bind _completed (CallFunction|IsTutorialItemGrabPhaseCompleted?))
    (if _completed
      (Default|HideAutomaticHintPanel (Variables|Default|GetTutorialManager))
      (CallFunction|CompleteQuest "None"))))

(event Custom|OnPlacePointManagerCompleted
  (if (CallFunction|IsCurrentQuest "None")
    (bind _completed (CallFunction|IsTidyUpPhaseCompleted?))
    (if _completed
      (CallFunction|CompleteQuest "None")
      (Default|NextConversation (Variables|Default|GetNPC)))))

(event Custom|OnFirstRoomItemsSpawned
  (Utilities|FlowControl|Delay 1.0))

(event EventBindItemActions
  (|CallParentFunction)
  (EventDispatchers|BindEventtoEDFirstRoomItemsSpawned (delegate Custom|OnFirstRoomItemsSpawned))
  (for _array_element (Variables|Default|GetFirstRoomItems)
    (EventDispatchers|BindEventtoEDDetectionStarted _array_element (delegate Custom|OnTutorialItemDetected))
    (EventDispatchers|AssignEDInteractionStarted _array_element (delegate Custom|OnTutorialItemGrabbed))))

(event EventBindPlacePointsActions
  (|CallParentFunction)
  (for _array_element (Variables|Default|GetPlacePointManagers)
    (EventDispatchers|BindEventtoEDOneItemHasBeenPlaced _array_element (delegate Custom|OnOneItemPlaced))
    (EventDispatchers|BindEventtoEDAllPlacePointswithItems _array_element (delegate Custom|OnPlacePointManagerCompleted))))

(event Custom|OnNPCConversationFinished
  (params (ConversationNumber :type Integer))
  (switch Utilities|FlowControl|Switch|SwitchonE_GameplayStepTypes (Variables|Default|GetCurrentStepType)
    (:NewEnumerator44
      (CallFunction|OnNPCIntroductionCompleted))
    (:NewEnumerator46
      (CallFunction|OnInformtoNPCCompleted))))

(event Custom|OnNPCIntroductionCompleted
  (if (CallFunction|IsCurrentQuest "None")
    (CallFunction|CompleteQuest "None")))

(event Custom|OnInformToNPCCompleted
  (if (CallFunction|IsCurrentQuest "None")
    (CallFunction|CompleteQuest "None")))

(event Custom|OnNPCConversationStarted
  (switch Utilities|FlowControl|Switch|SwitchonE_GameplayStepTypes (Variables|Default|GetCurrentStepType)
    (:NewEnumerator44
      (Default|HideAutomaticHintPanel (Variables|Default|GetTutorialManager))
      (Default|HideCurrentTuddy (Variables|Default|GetTutorialManager)))))

(event EventBindNPCActions
  (|CallParentFunction)
  (bind _npc (Variables|Default|GetNPC)
    (:then
      (EventDispatchers|BindEventtoEDConversationStarted _npc (delegate Custom|OnNPCConversationStarted))
      (EventDispatchers|BindEventtoEDConversationFinished _npc (delegate Custom|OnNPCConversationFinished)))
    (:else
      (Default|Log (CallFunction|GetMyGameInstance) "NewEnumerator2" "Falta NPC" false))))

(fn ConstructionScript)

(fn IsTutorialItemDetectionPhaseCompleted?
  (for _array_element (Variables|Default|GetFirstRoomItems)
    (if (not (Variables|/Game/Game/Blueprints/Actors/Items/BP_TutorialPickableItem.BP_TutorialPickableItem_C|GetHasBeenDetected _array_element))
      (return false)))
  (return true))

(fn IsTutorialItemGrabPhaseCompleted?
  (for _array_element (Variables|Default|GetFirstRoomItems)
    (if (not (Variables|/Game/Game/Blueprints/Actors/Items/BP_TutorialPickableItem.BP_TutorialPickableItem_C|GetLiar _array_element))
      (if (not (Variables|/Game/Game/Blueprints/Actors/Items/BP_TutorialPickableItem.BP_TutorialPickableItem_C|GetHasBeenGrabbed _array_element))
        (return false))))
  (return true))

(fn IsTidyUpPhaseCompleted?
  (for _array_element (Variables|Default|GetPlacePointManagers)
    (if (not (Variables|/Game/Game/Blueprints/Actors/Items/PlacePoints/BP_PlacePointManager.BP_PlacePointManager_C|GetAllPointsUsed _array_element))
      (return false)))
  (return true))