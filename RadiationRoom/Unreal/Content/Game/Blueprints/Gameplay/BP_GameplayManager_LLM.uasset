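; Gameplay manager for an LLM scenario that opens with a Tutorial Buddy dialog and reacts to NPC conversations.
; It extends a parent manager, starting the scenario on BeginPlay, then showing the buddy and launching its intro dialog by ID after short delays.
; Overridable bind events hook the dialog-completed and conversation-finished dispatchers.
; Completed dialogs print a message and hide the buddy, while finished NPC conversations only print a Spanish success message.
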(event Custom|OnNPCConversationFinished
  (params (ConversationNumber :type Integer))
  (Development|PrintString (Utilities|String|ToString(Text) (Utilities|Text|FormatText "La conversación nº {n} con {npc} ha terminado con éxito." ConversationNumber (Variables|/Game/Game/Blueprints/Characters/AI/BP_NPC.BP_NPC_C|GetName (Variables|Default|GetNPC)))) true true "(R=0.000000,G=0.660000,B=1.000000,A=1.000000)" 1e+01))

(event Custom|OnTutorialBuddyDialogCompleted
  (params (CurrentTuddyDialogType :type E_TuddyDialogLinesType%20Enum :default "NewEnumerator0") (CurrentExtraLineType :type E_TuddyExtraLineTypes%20Enum :default "NewEnumerator1") (DialogID :type Name))
  (Development|PrintString "El diálogo del Tutorial Buddy ha terminado con éxito.")
  (Utilities|FlowControl|Delay 1.0)
  (Default|Hide (Variables|Default|GetTutorial%20Buddy)))

(event EventBeginPlay
  (|CallParentFunction)
  (CallFunction|StartScenario))

(event EventStartScenario
  (bind _tutorial_buddy (Variables|Default|GetTutorial%20Buddy))
  (|CallParentFunction)
  (Utilities|FlowControl|Delay 1.0)
  (Default|Show _tutorial_buddy)
  (Utilities|FlowControl|Delay 0.5)
  (Default|StartNewDialogbyID (Variables|/Game/Game/Blueprints/Tutorial/BP_TutorialBuddy.BP_TutorialBuddy_C|GetAC_TuddyDialogManager _tutorial_buddy) "LLM1001"))

(event EventBindNPCActions
  (EventDispatchers|BindEventtoEDConversationFinished (Variables|Default|GetNPC) (delegate Custom|OnNPCConversationFinished)))

(event EventBindTuddyActions
  (EventDispatchers|BindEventtoEDDialogCompleted (Variables|/Game/Game/Blueprints/Tutorial/BP_TutorialBuddy.BP_TutorialBuddy_C|GetAC_TuddyDialogManager (Variables|Default|GetTutorial%20Buddy)) (delegate Custom|OnTutorialBuddyDialogCompleted)))

(fn ConstructionScript
  (|CallParentFunction))