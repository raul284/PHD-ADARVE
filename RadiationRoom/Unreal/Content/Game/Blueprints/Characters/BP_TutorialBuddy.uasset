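; Tutorial buddy actor that presents help through world widget panels and a dialog bubble, and destroys itself when the player's overlap ends.
; On BeginPlay it wires up its three widgets, registers with BP_TutorialManager and starts a self-restarting timeline that bobs the body.
; AutomaticCall steps through the item's dialog lines on timed delays, then shifts the body and shows the single-item panel.
; UserCall briefly shows the bubble, then opens the help panel.
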(event Custom|UserCall
  (Utilities|FlowControl|Delay 0.5)
  (Rendering|SetVisibility (Variables|Default|GetDialogWidget) true false)
  (Utilities|FlowControl|Delay 2.0)
  (Rendering|SetVisibility (Variables|Default|GetDialogWidget) false false)
  (Rendering|SetVisibility (Variables|Default|GetHelpPannelWidget) true false))

(event Custom|CloseHelpPanel
  (Rendering|SetVisibility (Variables|Default|GetHelpPannelWidget) false false)
  (Rendering|SetVisibility (Variables|Default|GetSingleItemHelpPannelWidget) false false))

(event Custom|AutomaticCall
  (params (Tutorial%20Item%20Data :type F%20Tutorial%20Item%20Structure))
  (bind _tuddylines (Utilities|Struct|BreakF_TutorialItem Tutorial%20Item%20Data))
  (Default|SetTutorialData (Variables|Default|GetSingleTutorialWidget) Tutorial%20Item%20Data)
  (Rendering|SetVisibility (Variables|Default|GetDialogWidget) true false)
  (Variables|Default|SetCurrentDialogIndex 0)
  (if (Utilities|Array|IsNotEmpty _tuddylines) :!label _label
    (if (> (Utilities|Array|Length _tuddylines) (Variables|Default|GetCurrentDialogIndex))
      (Default|SetDialogText (Variables|Default|GetDialogBubbleWidget) (Utilities|Array|Get(acopy) _tuddylines (Variables|Default|GetCurrentDialogIndex)))
      (Utilities|FlowControl|Delay 2.5)
      (bind _result (Math|Integer|IncrementInt (Variables|Default|GetCurrentDialogIndex))
        (:%20%20
          (Variables|Default|SetCurrentDialogIndex _result)
          (goto _label)))
      (else
        _))
    (else
      (Utilities|FlowControl|Delay 2.0)))
  (Transformation|SetRelativeLocation (Variables|Default|GetBody) "0.000000,-130.000000,15.000000" false false)
  (Rendering|SetVisibility (Variables|Default|GetDialogWidget) false false)
  (Rendering|SetVisibility (Variables|Default|GetSingleItemHelpPannelWidget) true false))

(event Custom|CreateHelpPanelButtons
  (params (Tutorial%20Item%20List :type Array%20of%20F%20Tutorial%20Item%20Structures))
  (Default|CreateButtonList (Variables|Default|GetHelpPanelWidget) Tutorial%20Item%20List))

(event Custom|WaveMovement
  (bind _alpha (Timeline|Timeline PlayFromStart)
    (:Update
      (Transformation|AddLocalOffset (Variables|Default|GetBody) (Math|Vector|MakeVector 0.0 0.0 (* _alpha 0.5)) false false))
    (:Finished
      (CallFunction|WaveMovement))))

(event EventBeginPlay
  (Utilities|FlowControl|Sequence
    (:then_0
      (bind _aswbp_help_pannel (Utilities|Casting|CastToWBP_HelpPannel (UserInterface|GetWidget (Variables|Default|GetHelpPannelWidget))))
      (bind _output_get (Variables|Default|SetHelpPanelWidget _aswbp_help_pannel))
      (Variables|/Game/Game/Blueprints/UI/Tutorial/WBP_HelpPannel.WBP_HelpPannel_C|SetOwner _output_get self)
      (bind _aswbp_single_tutorial_item (Utilities|Casting|CastToWBP_SingleTutorialItem (UserInterface|GetWidget (Variables|Default|GetSingleItemHelpPannelWidget))))
      (bind _output_get_2 (Variables|Default|SetSingleTutorialWidget _aswbp_single_tutorial_item))
      (Variables|/Game/Game/Blueprints/UI/Tutorial/WBP_SingleTutorialItem.WBP_SingleTutorialItem_C|SetOwner _output_get_2 self)
      (bind _aswbp_tutorial_buddy_dialog_pannel (Utilities|Casting|CastToWBP_TutorialBuddyDialogPannel (UserInterface|GetWidget (Variables|Default|GetDialogWidget))))
      (Variables|Default|SetDialogBubbleWidget _aswbp_tutorial_buddy_dialog_pannel))
    (:then_1
      (CallFunction|WaveMovement))
    (:then_2
      (bind _returnvalue (Actor|GetActorOfClass "/Game/Game/Blueprints/Tutorial/BP_TutorialManager.BP_TutorialManager_C"))
      (bind _output_get_3 (Variables|Default|SetTutorialManager _returnvalue))
      (Default|SetCurrentTutorialBuddy _output_get_3 self))))

(event EventTick
  (params (DeltaSeconds :type Float%20%28single-precision%29)))

(event Collision|EventActorEndOverlap
  (params (OtherActor :type Actor%20Object%20Reference))
  (if (== OtherActor (Variables|Default|GetPlayer))
    (Actor|DestroyActor)))

(fn ConstructionScript)

(fn GetWorldRotationbyComponent
  (params (SceneComponent :type Scene%20Component%20Object%20Reference))
  (bind _returnvalue (Transformation|GetWorldLocation SceneComponent))
  (bind _player (Variables|Default|GetPlayer))
  (bind _returnvalue_2 (Transformation|GetActorLocation _player))
  (bind _returnvalue_3 (Math|Rotator|FindLookatRotation _returnvalue _returnvalue_2))
  (bind (_roll _pitch _yaw) (Math|Rotator|BreakRotator _returnvalue_3))
  (return (Math|Rotator|MakeRotator _roll 1e+01 _yaw)))