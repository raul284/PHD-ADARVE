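; BP_GameplayManager_MaterialTheft is the gameplay manager for the Material Theft scenario, setting its opening objective and ambient audio.
; Shortly after BeginPlay it starts walkie static, traffic, siren and horn sounds, with horns replayed recursively at random intervals.
; When the firefighter mate's first conversation ends during that objective, it plays a truck door sound, stops walkie and siren, lowers street noise and completes the objective.
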(event Custom|StartGameplay
  (bind _returnvalue (Audio|SpawnSound2D "/Game/Game/Assets/Sounds/walkie_static.walkie_static" 0.1 1.0 0.0 0 false false))
  (Variables|Sounds|SetSound%20Walkie _returnvalue)
  (bind _returnvalue_2 (Audio|SpawnSound2D "/Game/Game/Assets/Sounds/effects/traffic.traffic" 0.08 1.0 0.0 0 false false))
  (Variables|Sounds|SetSound%20Traffic _returnvalue_2)
  (bind _returnvalue_3 (Audio|SpawnSound2D "/Game/Game/Assets/Sounds/effects/fire_truck_siren.fire_truck_siren" 0.05 1.0 0.0 0 false false))
  (Variables|Sounds|SetSound%20Firetruck%20Siren _returnvalue_3)
  (bind _returnvalue_4 (Audio|SpawnSound2D "/Game/Game/Assets/Sounds/effects/car_hornes.car_hornes" 0.1 1.0 0.0 0 false false))
  (Variables|Sounds|SetSound%20Car%20Hornes _returnvalue_4)
  (CallFunction|PlayCarHornSound)
  (Variables|Default|SetPlay%20Car%20Hornes true))

(event Custom|PlayCarHornSound
  (if (Variables|Default|GetPlay%20Car%20Hornes)
    (Audio|Components|Audio|Play (Variables|Sounds|GetSound%20Car%20Hornes) 0.0)
    (Utilities|FlowControl|Delay (Math|Random|RandomFloatinRange 4.0 1e+01))
    (CallFunction|PlayCarHornSound)))

(event EventBeginPlay
  (|CallParentFunction)
  (Utilities|FlowControl|Delay 0.2)
  (Default|CallObjectiveChanged "NewEnumerator9")
  (CallFunction|StartGameplay))

(event Collision|EventActorBeginOverlap
  (params (OtherActor :type Actor%20Object%20Reference)))

(event EventTick
  (params (DeltaSeconds :type Float%20%28single-precision%29)))

(event EventNPCConversationFinished
  (params (NPC%20 :type BP%20NPC%20Talkable%20Object%20Reference) (ConversationIndex :type Integer))
  (|CallParentFunction NPC%20 ConversationIndex)
  (Utilities|Casting|CastToBP_NPC_FirefighterMate NPC%20)
  (if (and (== ConversationIndex 0) (Utilities|Enum|Equal(Enum) (Variables|Default|GetCurrentObjectiveType) "NewEnumerator9"))
    (bind _returnvalue (Audio|SpawnSound2D "/Game/Game/Assets/Sounds/effects/fire_truck_openclosedoor.fire_truck_openclosedoor" 0.5 1.0 0.0 0))
    (Variables|Sounds|SetSound%20Firetruck%20Door _returnvalue)
    (Audio|Components|Audio|Stop (Variables|Sounds|GetSound%20Walkie))
    (Audio|Components|Audio|Stop (Variables|Sounds|GetSound%20Firetruck%20Siren))
    (Audio|Components|Audio|SetVolumeMultiplier (Variables|Sounds|GetSound%20Traffic) 0.2 :!class /Script/Engine.AudioComponent)
    (Audio|Components|Audio|SetVolumeMultiplier (Variables|Sounds|GetSound%20Car%20Hornes) 0.3 :!class /Script/Engine.AudioComponent)
    (CallFunction|CompleteObjective (Variables|Default|GetCurrentObjectiveType))))

(fn ConstructionScript
  (|CallParentFunction))