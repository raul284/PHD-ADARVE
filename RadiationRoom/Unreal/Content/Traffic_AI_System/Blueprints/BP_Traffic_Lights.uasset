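; Traffic light actor for the Traffic AI System, running timed or manually stepped intersection signals, or serving as a hidden priority-road sign.
; A parentless light gathers child lights and cycles all through shared rounds with yellow transitions, firing OnLightChanged.
; Construction syncs round arrays and builds dynamic materials for colors and arrows, with pedestrian lights flickering green during yellow.
; Priority Road mode temporarily turns non-priority lights red via a retriggerable delay.
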(event Custom|Next%20traffic%20loop
  ;[0.08653 0.329 1] Traffic light loop (Traffic Lights mode)
  (for _array_element (Variables|System|GetConnected%20lights)
    (CallFunction|SetLights _array_element (select (Utilities|Array|Get(acopy) (Variables|BP_Traffic_Lights_C|GetRounds _array_element) (Variables|System|GetCurrent%20round)) "NewEnumerator2" "NewEnumerator0"))
    (CallFunction|OnLightChanged _array_element (select (Utilities|Array|Get(acopy) (Variables|BP_Traffic_Lights_C|GetRounds _array_element) (Variables|System|GetCurrent%20round)) "NewEnumerator2" "NewEnumerator0")))
  (if (not (Variables|Settings|GetManual%20lights))
    (Utilities|FlowControl|Delay (Utilities|Array|Get(acopy) (Variables|Settings|GetRound%20length) (Variables|System|GetCurrent%20round)))
    (for _array_element_2 (Variables|System|GetConnected%20lights)
      (if (not (Math|Boolean|Equal(Boolean) (Utilities|Array|Get(acopy) (Variables|BP_Traffic_Lights_C|GetRounds _array_element_2) (select (== (Variables|System|GetCurrent%20round) (Utilities|Array|LastIndex (Variables|Settings|GetRounds))) 0 (+ (Variables|System|GetCurrent%20round) 1))) (Utilities|Array|Get(acopy) (Variables|BP_Traffic_Lights_C|GetRounds _array_element_2) (Variables|System|GetCurrent%20round))))
        (CallFunction|SetLights _array_element_2 (select (Utilities|Array|Get(acopy) (Variables|BP_Traffic_Lights_C|GetRounds _array_element_2) (Variables|System|GetCurrent%20round)) "NewEnumerator1" "NewEnumerator3"))
        (CallFunction|OnLightChanged _array_element_2 (select (Utilities|Array|Get(acopy) (Variables|BP_Traffic_Lights_C|GetRounds _array_element_2) (Variables|System|GetCurrent%20round)) "NewEnumerator1" "NewEnumerator3"))))
    (if (not (Variables|Settings|GetManual%20lights))
      (Utilities|FlowControl|Delay (Variables|Settings|GetYellow%20light%20time))
      (Variables|System|SetCurrent%20round (select (== (Variables|System|GetCurrent%20round) (Utilities|Array|LastIndex (Variables|Settings|GetRounds))) 0 (+ (Variables|System|GetCurrent%20round) 1)))
      (if (not (Variables|System|GetPaused?))
        (CallFunction|NextTrafficLoop)))))

(event Custom|Disable%20flickering
  ;[0.1656 1 0.1149] Disable flickering for green pedestrian light
  (Utilities|FlowControl|Delay (Variables|Settings|GetYellow%20light%20time))
  (Rendering|Components|Light|SetLightFunctionMaterial (Variables|Default|GetSpotLight) "/Game/Traffic_AI_System/Misc/Materials/M_Traffic_light_Light_function.M_Traffic_light_Light_function"))

(event Custom|Attach%20to%20target
  (bind _attachment_target (Variables|Default|GetAttachment%20Target))
  ;[0.3122 1 0.371] You can attach yout light to any actor. The traffic light will stick to a socket called "T_Slot". If your mesh will not have it, it will be attached to its pivot point.
  (Utilities|IsValid _attachment_target
    (:Is%20Valid
      (Transformation|AttachActorToActor self _attachment_target "T_Slot" "SnapToTarget" "SnapToTarget" "KeepWorld" true))
    (:Is%20Not%20Valid
      (Development|PrintString "Traffic AI System: Attachment target not selected" true true "(R=1.000000,G=0.000000,B=0.000000,A=1.000000)" 7.0))))

(event Custom|Switch%20traffic%20lights%20%28Priority%20road%20mode%20only%29
  ;[1 0.8555 0.2249] Switch lights (Priority road mode)
  (for _array_element (select (Utilities|IsValid (Variables|Settings|GetParent%20light)) (Variables|BP_Traffic_Lights_C|GetConnected%20lights (Variables|Settings|GetParent%20light)) (Variables|System|GetConnected%20lights))
    (switch Utilities|FlowControl|Switch|SwitchonEnum_Traffic_light_type (Variables|BP_Traffic_Lights_C|GetLight%20mode _array_element)
      (:NewEnumerator0
        (Development|PrintString (Utilities|String|Append "Traffic AI System Error: You cannot have Traffic Lights and Signs modes both on the same intersection. (" (Utilities|GetDisplayName self) ")") true true "(R=1.000000,G=0.025290,B=0.000000,A=1.000000)" 1e+01))
      (:NewEnumerator1
        (CallFunction|SetLights _array_element (select (Variables|BP_Traffic_Lights_C|GetPriority%20road? _array_element) "NewEnumerator2" "NewEnumerator0")))))
  (Utilities|FlowControl|RetriggerableDelay 2.0)
  (for _array_element_2 (select (Utilities|IsValid (Variables|Settings|GetParent%20light)) (Variables|BP_Traffic_Lights_C|GetConnected%20lights (Variables|Settings|GetParent%20light)) (Variables|System|GetConnected%20lights))
    (CallFunction|SetLights _array_element_2 "NewEnumerator2")))

(event Custom|OnLight%20Changed
  (params (New%20light :type Enum_Current_traffic_light%20Enum :default "NewEnumerator0"))
  ;[1 1 1] This event will fire every time light is changed (1.2 update)
)

(event Custom|Switch%20manual%20light
  ;[0.08653 0.329 1] Traffic light loop (Traffic Lights mode)
  ;;[1 1 1] Manual light switching (1.2 update)
  (if (Variables|Settings|GetManual%20lights)
    (switch int (Variables|System|GetManual%20lights%20order)
      (:0
        (Variables|System|SetManual%20lights%20order 1)
        (for _array_element (Variables|System|GetConnected%20lights)
          (CallFunction|SetLights _array_element (select (Utilities|Array|Get(acopy) (Variables|BP_Traffic_Lights_C|GetRounds _array_element) (Variables|System|GetCurrent%20round)) "NewEnumerator2" "NewEnumerator0"))
          (CallFunction|OnLightChanged _array_element (select (Utilities|Array|Get(acopy) (Variables|BP_Traffic_Lights_C|GetRounds _array_element) (Variables|System|GetCurrent%20round)) "NewEnumerator2" "NewEnumerator0")))
        (if (not (Variables|Settings|GetManual%20lights))
          (Utilities|FlowControl|Delay (Utilities|Array|Get(acopy) (Variables|Settings|GetRound%20length) (Variables|System|GetCurrent%20round)))
          (for _array_element_2 (Variables|System|GetConnected%20lights) :!label _label
            (if (not (Math|Boolean|Equal(Boolean) (Utilities|Array|Get(acopy) (Variables|BP_Traffic_Lights_C|GetRounds _array_element_2) (select (== (Variables|System|GetCurrent%20round) (Utilities|Array|LastIndex (Variables|Settings|GetRounds))) 0 (+ (Variables|System|GetCurrent%20round) 1))) (Utilities|Array|Get(acopy) (Variables|BP_Traffic_Lights_C|GetRounds _array_element_2) (Variables|System|GetCurrent%20round))))
              (CallFunction|SetLights _array_element_2 (select (Utilities|Array|Get(acopy) (Variables|BP_Traffic_Lights_C|GetRounds _array_element_2) (Variables|System|GetCurrent%20round)) "NewEnumerator1" "NewEnumerator3"))
              (CallFunction|OnLightChanged _array_element_2 (select (Utilities|Array|Get(acopy) (Variables|BP_Traffic_Lights_C|GetRounds _array_element_2) (Variables|System|GetCurrent%20round)) "NewEnumerator1" "NewEnumerator3"))))
          (if (not (Variables|Settings|GetManual%20lights))
            (Utilities|FlowControl|Delay (Variables|Settings|GetYellow%20light%20time))
            (Variables|System|SetCurrent%20round (select (== (Variables|System|GetCurrent%20round) (Utilities|Array|LastIndex (Variables|Settings|GetRounds))) 0 (+ (Variables|System|GetCurrent%20round) 1)) :!label _label_2)
            (if (not (Variables|System|GetPaused?))
              (CallFunction|NextTrafficLoop)))))
      (:1
        (Variables|System|SetManual%20lights%20order 2)
        (goto _label))
      (:2
        (Variables|System|SetManual%20lights%20order 1)
        (goto _label_2)))))

(event EventBeginPlay
  ;[0.08653 0.329 1] Traffic light loop (Traffic Lights mode)
  (CallFunction|FindChildLights) ; 1.2.2 Update
  (Rendering|Components|Light|SetIntensity (Variables|Default|GetSpotLight) (Variables|Settings|GetSpot%20light%20intensity))
  ;;[1 0.8555 0.2249] If mode set to "signs", do not start the loop
  (switch Utilities|FlowControl|Switch|SwitchonEnum_Traffic_light_type (Variables|Settings|GetLight%20mode)
    (:NewEnumerator0
      (Utilities|IsValid (Variables|Settings|GetParent%20light) ; Check if has parent light
        (:Is%20Not%20Valid
          (if (Variables|Settings|GetManual%20lights)
            (CallFunction|SwitchManualLight)
            (else
              (for _array_element (Variables|System|GetConnected%20lights)
                (CallFunction|SetLights _array_element (select (Utilities|Array|Get(acopy) (Variables|BP_Traffic_Lights_C|GetRounds _array_element) (Variables|System|GetCurrent%20round)) "NewEnumerator2" "NewEnumerator0"))
                (CallFunction|OnLightChanged _array_element (select (Utilities|Array|Get(acopy) (Variables|BP_Traffic_Lights_C|GetRounds _array_element) (Variables|System|GetCurrent%20round)) "NewEnumerator2" "NewEnumerator0")))
              (if (not (Variables|Settings|GetManual%20lights))
                (Utilities|FlowControl|Delay (Utilities|Array|Get(acopy) (Variables|Settings|GetRound%20length) (Variables|System|GetCurrent%20round)))
                (for _array_element_2 (Variables|System|GetConnected%20lights)
                  (if (not (Math|Boolean|Equal(Boolean) (Utilities|Array|Get(acopy) (Variables|BP_Traffic_Lights_C|GetRounds _array_element_2) (select (== (Variables|System|GetCurrent%20round) (Utilities|Array|LastIndex (Variables|Settings|GetRounds))) 0 (+ (Variables|System|GetCurrent%20round) 1))) (Utilities|Array|Get(acopy) (Variables|BP_Traffic_Lights_C|GetRounds _array_element_2) (Variables|System|GetCurrent%20round))))
                    (CallFunction|SetLights _array_element_2 (select (Utilities|Array|Get(acopy) (Variables|BP_Traffic_Lights_C|GetRounds _array_element_2) (Variables|System|GetCurrent%20round)) "NewEnumerator1" "NewEnumerator3"))
                    (CallFunction|OnLightChanged _array_element_2 (select (Utilities|Array|Get(acopy) (Variables|BP_Traffic_Lights_C|GetRounds _array_element_2) (Variables|System|GetCurrent%20round)) "NewEnumerator1" "NewEnumerator3"))))
                (if (not (Variables|Settings|GetManual%20lights))
                  (Utilities|FlowControl|Delay (Variables|Settings|GetYellow%20light%20time))
                  (Variables|System|SetCurrent%20round (select (== (Variables|System|GetCurrent%20round) (Utilities|Array|LastIndex (Variables|Settings|GetRounds))) 0 (+ (Variables|System|GetCurrent%20round) 1)))
                  (if (not (Variables|System|GetPaused?))
                    (CallFunction|NextTrafficLoop)))))))))
    (:NewEnumerator1
      ;;[1 0.8555 0.2249] If in "Priority Road" mode, set all lights to green at Begin Play
      (CallFunction|SetLights "NewEnumerator2"))))

(fn ConstructionScript
  (bind _staticmeshcomponent (Variables|Debug|GetStaticMeshComponent))
  (bind _priority_road_ (Variables|Settings|GetPriority%20road?))
  (bind _parent_light (Variables|Settings|GetParent%20light))
  (bind _rounds (Variables|Settings|GetRounds))
  (bind _rounds_2 (Variables|Settings|GetRounds))
  (bind _round_length (Variables|Settings|GetRound%20length))
  (bind _rounds_3 (Variables|Settings|GetRounds))
  (bind _round_length_2 (Variables|Settings|GetRound%20length))
  (bind _returnvalue (Utilities|Array|Length _rounds_2))
  (bind _returnvalue_2 (Utilities|Array|Length _round_length_2))
  (bind _returnvalue_3 (Utilities|Array|Length _rounds_3))
  (bind _returnvalue_4 (select _priority_road_ "(R=0.000000,G=1.000000,B=0.717875,A=1.000000)" "(R=1.000000,G=0.321203,B=0.000000,A=1.000000)"))
  (bind _rounds_4 (Variables|BP_Traffic_Lights_C|GetRounds _parent_light))
  (bind _returnvalue_5 (Utilities|Array|Length _rounds_4))
  (bind _returnvalue_6 (- _returnvalue_3 _returnvalue_2))
  (bind _returnvalue_7 (> _returnvalue_5 _returnvalue))
  (bind _returnvalue_8 (> _returnvalue_6 0))
  (Variables|Settings|SetUpdate%20Light false)
  (Utilities|FlowControl|Sequence
    (:then_0
      ;[1 0.4478 0.9467] Create material instances for lights
      (for _array_element (Class|MeshComponent|GetMaterialSlotNames (Variables|Debug|GetStaticMeshComponent))
        (if (Math|Boolean|ORBoolean (Utilities|Name|Equal(Name) _array_element "Green") (Utilities|Name|Equal(Name) _array_element "Yellow") (Utilities|Name|Equal(Name) _array_element "Red")) ; 1.2 Update. Fix for custom light meshes
          (Rendering|Material|SetMaterial _staticmeshcomponent (Rendering|Material|GetMaterialIndex (Variables|Debug|GetStaticMeshComponent) (select (Utilities|Name|Equal(Name) _array_element "Red") "Red" (select (Utilities|Name|Equal(Name) _array_element "Yellow") "Yellow" "Green"))) (select (Utilities|Enum|Equal(Enum) (Variables|Visual|GetArrow%20type) "NewEnumerator0") "/Game/Traffic_AI_System/Misc/Materials/MI_Traffic_light.MI_Traffic_light" "/Game/Traffic_AI_System/Misc/Materials/MI_Traffic_light_arrow.MI_Traffic_light_arrow"))
          (bind _returnvalue_9 (Rendering|Material|CreateDynamicMaterialInstance _staticmeshcomponent (Rendering|Material|GetMaterialIndex (Variables|Debug|GetStaticMeshComponent) (select (Utilities|Name|Equal(Name) _array_element "Red") "Red" (select (Utilities|Name|Equal(Name) _array_element "Yellow") "Yellow" "Green"))) (Rendering|Material|GetMaterial (Variables|Debug|GetStaticMeshComponent) (Rendering|Material|GetMaterialIndex (Variables|Debug|GetStaticMeshComponent) (select (Utilities|Name|Equal(Name) _array_element "Red") "Red" (select (Utilities|Name|Equal(Name) _array_element "Yellow") "Yellow" "Green")))) "None" :!class /Script/Engine.PrimitiveComponent))
          (switch name _array_element
            (:Red
              (Variables|System|SetRed _returnvalue_9))
            (:Yellow
              (Variables|System|SetYellow _returnvalue_9))
            (:Green
              (Variables|System|SetGreen _returnvalue_9))))))
    (:then_1
      ;[0.3665 0.5249 1] Set arrows
      (if (not (Utilities|Enum|Equal(Enum) (Variables|Visual|GetArrow%20type) "NewEnumerator0"))
        (for _array_element_2 (Utilities|Array|MakeArray (Variables|System|GetGreen) (Variables|System|GetYellow) (Variables|System|GetRed))
          (Variables|System|SetCurrent%20Light%20Visual (select (== _array_element_2 (Variables|System|GetGreen)) "NewEnumerator2" (select (== (Variables|System|GetYellow) _array_element_2) "NewEnumerator1" "NewEnumerator0")))
          (Rendering|Material|SetVectorParameterValue _array_element_2 "Arrow Type" "(R=0.000000,G=0.000000,B=0.000000,A=0.000000)" :!class /Script/Engine.MaterialInstanceDynamic)
          (switch Utilities|FlowControl|Switch|SwitchonEnum_Traffic_arrow_type (Variables|Visual|GetArrow%20type)
            (:NewEnumerator1
              (CallFunction|SetArrow _array_element_2 "(R=1.000000,G=0.000000,B=0.000000,A=0.000000)" "NewEnumerator0" false))
            (:NewEnumerator2
              (CallFunction|SetArrow _array_element_2 "(R=1.000000,G=0.000000,B=0.000000,A=0.000000)" "NewEnumerator1" false))
            (:NewEnumerator3
              (CallFunction|SetArrow _array_element_2 "(R=1.000000,G=0.000000,B=0.000000,A=0.000000)" "NewEnumerator2" false))
            (:NewEnumerator4
              (CallFunction|SetArrow _array_element_2 "(R=0.000000,G=1.000000,B=0.000000,A=0.000000)" "NewEnumerator0" true))
            (:NewEnumerator5
              (CallFunction|SetArrow _array_element_2 "(R=0.000000,G=1.000000,B=0.000000,A=0.000000)" "NewEnumerator0" false))
            (:NewEnumerator6
              (CallFunction|SetArrow _array_element_2 (select (== _array_element_2 (Variables|System|GetGreen)) "(R=0.000000,G=0.000000,B=0.000000,A=1.000000)" "(R=0.000000,G=0.000000,B=1.000000,A=0.000000)") "NewEnumerator0" true))))))
    (:then_2
      ;[0.5185 0.5895 1] Set light colors
      (switch Utilities|FlowControl|Switch|SwitchonEnum_Traffic_light_type (Variables|Settings|GetLight%20mode)
        (:NewEnumerator0
          (Rendering|Material|SetVectorParameterValue (Variables|System|GetGreen) "Color" (Variables|Visual|GetGreen%20Color) :!class /Script/Engine.MaterialInstanceDynamic)
          (Rendering|Material|SetVectorParameterValue (Variables|System|GetYellow) "Color" (Variables|Visual|GetYellow%20Color) :!class /Script/Engine.MaterialInstanceDynamic)
          (Rendering|Material|SetVectorParameterValue (Variables|System|GetRed) "Color" (Variables|Visual|GetRed%20Color) :!class /Script/Engine.MaterialInstanceDynamic)
          (Rendering|Components|Light|SetLightColor (Variables|Default|GetSpotLight) (Variables|Visual|GetYellow%20Color) true))
        (:NewEnumerator1
          ;;[1 0.8555 0.2249] If light mode is set to "Signs", blue light means that the road has priority
          (Rendering|Material|SetVectorParameterValue (Variables|System|GetGreen) "Color" _returnvalue_4 :!class /Script/Engine.MaterialInstanceDynamic)
          (Rendering|Components|Light|SetLightColor (Variables|Default|GetSpotLight) _returnvalue_4 true)
          ;;[1 0.8555 0.2249] Set Traffic light mesh and Spot light to be hidden in game and disable collisions
          (Development|SetHiddeninGame (Variables|Debug|GetStaticMeshComponent) true true)
          (Collision|SetActorEnableCollision self false))))
    (:then_3
      ;[0.5212 1 0.4969] Set light intensity
      (for _array_element_3 (Utilities|Array|MakeArray (Variables|System|GetGreen) (Variables|System|GetYellow) (Variables|System|GetRed))
        (Rendering|Material|SetScalarParameterValue _array_element_3 "Intensity" (Variables|Visual|GetLight%20Intensity) :!class /Script/Engine.MaterialInstanceDynamic)))
    (:then_4
      ;[1 0.8555 0.2249] If light is parent, set green light, if not - set red
      (switch Utilities|FlowControl|Switch|SwitchonEnum_Traffic_light_type (Variables|Settings|GetLight%20mode)
        (:NewEnumerator0
          (Utilities|IsValid (Variables|Settings|GetParent%20light)
            (:Is%20Valid
              (CallFunction|SetLights "NewEnumerator0"))
            (:Is%20Not%20Valid
              (CallFunction|SetLights "NewEnumerator2")
              (AddComponent|AddTextRenderComponent false (Math|Transform|MakeTransform "0, 0,50.000000" "0,90.000000, 0" "1,1,1") :!label _label))))
        (:NewEnumerator1
          (Utilities|IsValid (Variables|Settings|GetParent%20light)
            (:Is%20Not%20Valid
              (goto _label))))))
    (:then_5
      ;[0.08653 0.329 1] Check if this light is Parent light
      (Utilities|Array|Clear (Variables|System|GetConnected%20lights))
      (Utilities|IsValid (Variables|Settings|GetParent%20light)
        (:Is%20Valid
          ;[1 0.61 0.8317] Fill rounds if have Parent
          (if _returnvalue_7
            (while _returnvalue_7
              (Utilities|Array|Add _rounds false))
            (else
              (while (> _returnvalue _returnvalue_5)
                (Utilities|Array|RemoveIndex _rounds (Utilities|Array|LastIndex _rounds))))))
        (:Is%20Not%20Valid
          (Utilities|FlowControl|Sequence
            (:then_0
              ;[1 0.5766 0.5168] If number of rounds is less than two, display error message, and make sure it has at least two rounds
              (while (< (Utilities|Array|Length (Variables|Settings|GetRounds)) 2)
                (bind _isa (Utilities|FlowControl|FlipFlop)
                  (:A
                    _)
                  (:B
                    _))
                (Utilities|Array|Add (Variables|Settings|GetRounds) _isa)
                (Development|PrintString "Traffic AI System: Traffic light needs to have at least two rounds" true true "(R=1.000000,G=0.000000,B=0.000000,A=1.000000)" 7.0)))
            (:then_1
              ;[0.4463 1 0.9602] Fill Light rounds arrays for Parent and all connected lights
              (CallFunction|FindChildLights) ; Collapsed into a function in 1.2.2 version
            )
            (:then_2
              ;[0.3091 1 0.3049] Populate Round length array
              (if _returnvalue_8
                (while _returnvalue_8
                  (Utilities|Array|Add (Variables|Settings|GetRound%20length) (Variables|System|GetDefault%20round%20time)))
                (else
                  (while (< _returnvalue_6 0)
                    (Utilities|Array|RemoveIndex _round_length (Utilities|Array|LastIndex _round_length))))))
            (:then_3
              ;[1 0.22 0.07011] At the end add SELF to "Connected lights" array
              (Utilities|Array|AddUnique (Variables|System|GetConnected%20lights) self))))))))

(fn SetLights
  (params (Light :type Enum_Current_traffic_light%20Enum :default "NewEnumerator0"))
  (Variables|System|SetCurrent%20Light%20Visual Light)
  (Variables|System|SetCurrent%20Light (Utilities|Select :Index Light :NewEnumerator0 "NewEnumerator0" :NewEnumerator3 "NewEnumerator0" :NewEnumerator1 "NewEnumerator0" :NewEnumerator2 "NewEnumerator2"))
  (switch Utilities|FlowControl|Switch|SwitchonEnum_Current_traffic_light (Variables|System|GetCurrent%20Light%20Visual)
    (:NewEnumerator0
      ;[1 0.838 0.3518] Set traffic light color
      (CallFunction|SetOneLight "NewEnumerator0" true false :!label _label)
      (CallFunction|SetOneLight "NewEnumerator1" false false)
      (CallFunction|SetOneLight "NewEnumerator2" false false)
      ;[0.4554 1 0.4034] Set Spot Light color
      (Rendering|Components|Light|SetLightColor (Variables|Default|GetSpotLight) (Variables|Visual|GetRed%20Color) true))
    (:NewEnumerator3
      (if (Variables|System|GetLight%20for%20pedestrians?)
        (goto _label)
        (else
          (CallFunction|SetOneLight "NewEnumerator0" true false)
          (CallFunction|SetOneLight "NewEnumerator1" true false)
          (CallFunction|SetOneLight "NewEnumerator2" false false)
          (Rendering|Components|Light|SetLightColor (Variables|Default|GetSpotLight) (Math|Color|Lerp(LinearColor) (Variables|Visual|GetRed%20Color) (Variables|Visual|GetYellow%20Color) 0.5) true))))
    (:NewEnumerator1
      (if (Variables|System|GetLight%20for%20pedestrians?)
        ;[0.1886 0.4336 1] Flickering green light for pedestrians instead of red
        (CallFunction|SetOneLight "NewEnumerator0" false false)
        (CallFunction|SetOneLight "NewEnumerator1" false false)
        (CallFunction|SetOneLight "NewEnumerator2" true true)
        (Rendering|Components|Light|SetLightColor (Variables|Default|GetSpotLight) (Variables|Visual|GetGreen%20Color) true)
        (Rendering|Components|Light|SetLightFunctionMaterial (Variables|Default|GetSpotLight) "/Game/Traffic_AI_System/Misc/Materials/MI_Traffic_light_Light_function_flickering.MI_Traffic_light_Light_function_flickering")
        (CallFunction|DisableFlickering)
        (else
          (CallFunction|SetOneLight "NewEnumerator0" false false)
          (CallFunction|SetOneLight "NewEnumerator1" true false)
          (CallFunction|SetOneLight "NewEnumerator2" false false)
          (Rendering|Components|Light|SetLightColor (Variables|Default|GetSpotLight) (Variables|Visual|GetYellow%20Color) true))))
    (:NewEnumerator2
      (CallFunction|SetOneLight "NewEnumerator0" false false)
      (CallFunction|SetOneLight "NewEnumerator1" false false)
      (CallFunction|SetOneLight "NewEnumerator2" true false)
      (Rendering|Components|Light|SetLightColor (Variables|Default|GetSpotLight) (Variables|Visual|GetGreen%20Color) true)))
  (return))

(fn SetOneLight
  (params (Light :type Enum_Current_traffic_light%20Enum :default "NewEnumerator0") (On? :type Boolean) (Flicker :type Boolean))
  (bind _green (Variables|System|GetGreen))
  (bind _red (Variables|System|GetRed))
  (bind _yellow (Variables|System|GetYellow))
  (bind _returnvalue (Utilities|Select :Index Light :NewEnumerator0 _red :NewEnumerator3 0 :NewEnumerator1 _yellow :NewEnumerator2 _green))
  (Rendering|Material|SetScalarParameterValue _returnvalue "Light on" (Math|Conversions|ToFloat(Boolean) On?) :!class /Script/Engine.MaterialInstanceDynamic)
  (Rendering|Material|SetScalarParameterValue _returnvalue "Light Flicker" (Math|Conversions|ToFloat(Boolean) Flicker) :!class /Script/Engine.MaterialInstanceDynamic)
  (return))

(fn SetArrow
  (params (Material :type Material%20Instance%20Dynamic%20Object%20Reference) (Value :type Linear%20Color%20Structure :default "(R=1.000000,G=0.000000,B=0.000000,A=0.000000)") (Direction :type Enum_TurnType%20Enum :default "NewEnumerator0") (Mirror? :type Boolean))
  (Rendering|Material|SetVectorParameterValue Material "Arrow Type" Value :!class /Script/Engine.MaterialInstanceDynamic)
  (Rendering|Material|SetScalarParameterValue Material "Mirror Arrow" (select Mirror? 1.0 -1.0) :!class /Script/Engine.MaterialInstanceDynamic)
  (Rendering|Material|SetScalarParameterValue Material "Rotation" (Utilities|Select :Index Direction :NewEnumerator0 0.0 :NewEnumerator1 0.5 :NewEnumerator2 1.5) :!class /Script/Engine.MaterialInstanceDynamic)
  (Rendering|Material|SetScalarParameterValue Material "Invert arrow?" (Math|Conversions|ToFloat(Boolean) (Utilities|Select :Index (Variables|System|GetCurrent%20Light%20Visual) :NewEnumerator0 (Variables|Visual|GetRed%20Inverted%20arrow) :NewEnumerator3 false :NewEnumerator1 (Variables|Visual|GetYellow%20Inverted%20arrow) :NewEnumerator2 (Variables|Visual|GetGreen%20Inverted%20arrow))) :!class /Script/Engine.MaterialInstanceDynamic)
  (return))

(fn PauseTrafficLights
  (params (Pause :type Boolean))
  (switch Utilities|FlowControl|Switch|SwitchonEnum_Traffic_light_type (Variables|Settings|GetLight%20mode)
    (:NewEnumerator0
      (if (Variables|Settings|GetManual%20lights)
        _
        (else
          (if Pause
            (Variables|System|SetPaused? true)
            (else
              (Variables|System|SetPaused? false)
              (CallFunction|NextTrafficLoop)))
          (return))))
    (:NewEnumerator1
      _))
  (return))

(fn FindChildLights
  (bind _rounds (Variables|Settings|GetRounds))
  (bind _returnvalue (Utilities|Array|Length _rounds))
  (bind _outactors (Actor|GetAllActorsOfClass "BP_Traffic_Lights_C"))
  (for _array_element _outactors
    (if (== (Variables|BP_Traffic_Lights_C|GetParent%20light _array_element) self)
      ;[1 0.8555 0.2249] Round Length is cleared for connected lights, because those values are taken from the parent
      (Utilities|Array|Clear (Variables|BP_Traffic_Lights_C|GetRound%20length _array_element))
      (Utilities|Array|AddUnique (Variables|System|GetConnected%20lights) _array_element)
      (if (> (Utilities|Array|Length (Variables|BP_Traffic_Lights_C|GetRounds _array_element)) _returnvalue)
        (Utilities|FlowControl|DoN (- (Utilities|Array|Length (Variables|BP_Traffic_Lights_C|GetRounds _array_element)) _returnvalue)
          (:Exit
            (Utilities|Array|RemoveIndex (Variables|BP_Traffic_Lights_C|GetRounds _array_element) (Utilities|Array|LastIndex (Variables|BP_Traffic_Lights_C|GetRounds _array_element)))))
        (else
          (Utilities|FlowControl|DoN (- _returnvalue (Utilities|Array|Length (Variables|BP_Traffic_Lights_C|GetRounds _array_element)))
            (:Exit
              (Utilities|Array|Add (Variables|BP_Traffic_Lights_C|GetRounds _array_element) false)))))))
  (return))