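; Radiation emission point actor that represents an isotope source and can contaminate actors that touch it.
; On BeginPlay it fills IsotopeData, including radiation, from the IsotopesDataTable row matching its isotope.
; When IsEncapsuled is true, mesh hits set IsContamined on the other actor's AC_Radiation component.
; CalculateRadiationWithDistance has an inverse-square form, but its zero numerator leaves it without a real radiation value.
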(event OnComponentHit(StaticMesh)
  (params (HitComponent :type Primitive%20Component%20Object%20Reference) (OtherActor :type Actor%20Object%20Reference) (OtherComp :type Primitive%20Component%20Object%20Reference) (NormalImpulse :type Vector :default "0, 0, 0") (Hit :type Hit%20Result%20Structure%20%28by%20ref%29))
  (bind _returnvalue (Actor|GetComponentbyClass OtherActor "/Game/Game/Blueprints/Components/AC_Radiation.AC_Radiation_C"))
  (if (Variables|RadiationData|GetIsEncapsuled?)
    (Utilities|IsValid _returnvalue
      (:Is%20Valid
        (Variables|/Game/Game/Blueprints/Components/AC_Radiation.AC_Radiation_C|SetIsContamined? _returnvalue true)))))

(event Custom|SetIsotopeData
  (bind _isotopesdatatable (Variables|RadiationData|GetIsotopesDataTable))
  (bind _outrownames (DataTable|GetDataTableRowNames _isotopesdatatable))
  (bind _array_element (Utilities|Array|ForEachLoopwithBreak _outrownames :!label _label)
    (:LoopBody
      (bind _returnvalue (Utilities|GetDataTableRow _isotopesdatatable _array_element)
        (:then
          (if (Utilities|Enum|Equal(Enum) (.Isotope (Utilities|Struct|BreakF_IsotopesData _returnvalue)) (.Isotope (Utilities|Struct|BreakF_IsotopesData (Variables|RadiationData|GetIsotopeData))))
            (Variables|RadiationData|SetIsotopeData (Utilities|Struct|MakeF_IsotopesData (.Isotope (Utilities|Struct|BreakF_IsotopesData _returnvalue)) (.Radiation (Utilities|Struct|BreakF_IsotopesData _returnvalue))))
            (goto _label Break)))))))

(event EventBeginPlay
  (|CallParentFunction)
  (CallFunction|SetIsotopeData))

(fn ConstructionScript)

(fn CalculateRadiationwithDistance
  (params (OtherActor :type Actor%20Object%20Reference))
  (return (/ 0.0 (Class|KismetMathLibrary|VectorDistanceSquared (Transformation|GetActorLocation OtherActor) (Transformation|GetActorLocation)))))