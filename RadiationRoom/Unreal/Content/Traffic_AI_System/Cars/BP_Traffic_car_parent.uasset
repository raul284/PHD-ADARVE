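; Parent vehicle pawn for the traffic AI system's cars, drivable by either the player or the AI.
; Keys drive movement, lights, indicators and doors, and Enter returns control to the preview pawn and AI, parking the car.
; AI feeds VehicleMovement through SetInputs, while test events switch BPTrafficCarComponent between navigation, roaming, speeding and predefined paths.
; Tick updates engine audio and destroys the car after it stays nearly stopped too long.
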(event Custom|Navigate%20to%20actor
  (bind _target_actor (Variables|Default|GetTarget%20Actor))
  ;[1 0.5094 0.4195] If you want to test navigating to an actor, select Target Actor, click on a vehicle while PIE, and click "Navigate to actor" button. (1.1 Update)
  (Utilities|IsValid (Game|GetPlayerController 0) ; Check if in editor
    (:Is%20Valid
      (Utilities|IsValid _target_actor
        (:Is%20Valid
          (Default|SetAIModetoNavigatetoPoint (Variables|Default|GetBP_Traffic_Car_Component) _target_actor "0, 0, 0" 0 false (Variables|Default|GetReach%20Target%20Type) 75.0 false false))))))

(event Custom|Set%20mode%20to%20"AI%20Drive"
  ;[1 0.9743 0.3585] Sets AI mode to "AI Drive" (1.1 Update)
  (Utilities|IsValid (Game|GetPlayerController 0) ; Check if in editor
    (:Is%20Valid
      (Default|SetAIModetoRoam (Variables|Default|GetBP_Traffic_Car_Component) 0 true))))

(event Custom|Toggle%20speeding
  (bind _bp_traffic_car_component (Variables|Default|GetBP_Traffic_Car_Component))
  ;[1 1 1] Speeding test
  (Utilities|FlowControl|FlipFlop
    (:A
      (Default|SetSpeeding _bp_traffic_car_component true false))
    (:B
      (Default|SetSpeeding _bp_traffic_car_component false false))))

(event Custom|Open%20doors
  (params (Close :type Boolean))
  (bind _returnvalue (not Close))
  (bind _bp_car_body_apperance_component (Variables|Default|GetBP_Car_body_apperance_Component))
  ;[1 1 1] Car doors
  (Default|OpenDoor _bp_car_body_apperance_component "NewEnumerator0" _returnvalue)
  (Default|OpenDoor _bp_car_body_apperance_component "NewEnumerator1" _returnvalue)
  (Default|OpenDoor _bp_car_body_apperance_component "NewEnumerator2" _returnvalue)
  (Default|OpenDoor _bp_car_body_apperance_component "NewEnumerator3" _returnvalue))

(event Custom|Use%20predefined%20path
  ;[1 1 1] Predefined path preview (1.2 Update)
  (if (Variables|Default|GetUse%20predefined%20path?)
    (Default|SetAIModetoPredefinedPath (Variables|Default|GetBP_Traffic_Car_Component) true (Variables|Default|GetPredefined%20path%20example) false)))

(event EventTick
  (params (DeltaSeconds :type Float%20%28single-precision%29))
  ;[0.3756 0.7102 1] Set engine sound parameters
  (Utilities|FlowControl|Sequence
    (:then_0
      (Audio|Parameter|SetFloatParameter (Variables|Default|GetEngine_Cue) "RPM" (Class|WheeledVehicleMovementComponent|GetEngineRotationSpeed (Variables|Default|GetVehicleMovement)) :!class /Script/Engine.AudioComponent)
      (Audio|Parameter|SetFloatParameter (Variables|Default|GetEngine_Cue) "Volume" (Utilities|Select :Index (Variables|/Game/Traffic_AI_System/Components/BP_Traffic_Car_Component.BP_Traffic_Car_Component_C|GetCar%20mode (Variables|Default|GetBP_Traffic_Car_Component)) :NewEnumerator0 1.0 :NewEnumerator1 0.0 :NewEnumerator2 1.0) :!class /Script/Engine.AudioComponent))
    (:then_1
      (if (<= (Variables|/Game/Traffic_AI_System/Components/BP_Traffic_Car_Component.BP_Traffic_Car_Component_C|GetForward%20Speed (Variables|Default|GetBP_Traffic_Car_Component)) 2.0)
        (bind _output_get (Variables|Default|SetTimeStopped (+ (Variables|Default|GetTimeStopped) DeltaSeconds)))
        (if (>= _output_get (Variables|Default|GetMaxTimeStopped))
          (Actor|DestroyActor))
        (else
          (Variables|Default|SetTimeStopped 0.0))))))

(event EventBeginPlay
  ;[1 1 1] Predefined path preview (1.2 Update)
  (Utilities|FlowControl|Delay 5.0)
  (CallFunction|UsePredefinedPath) ; For preview level
)

(event EventSetInputs
  (params (Throttle :type Float%20%28single-precision%29) (Brakes :type Float%20%28single-precision%29) (Steering :type Float%20%28single-precision%29) (Handbrake :type Boolean) (Reverse? :type Boolean))
  (bind _vehiclemovement (Variables|Default|GetVehicleMovement))
  ;[0.2577 1 0.2174] Set inputs for AI (This part is essential for AI cars to work!)
  (Class|WheeledVehicleMovementComponent|SetThrottleInput _vehiclemovement Throttle)
  (Class|WheeledVehicleMovementComponent|SetBrakeInput _vehiclemovement Brakes)
  (Class|WheeledVehicleMovementComponent|SetSteeringInput _vehiclemovement Steering)
  (Class|WheeledVehicleMovementComponent|SetHandbrakeInput _vehiclemovement Handbrake)
  ;[1 0.269 0.6684] Set gear to reverse
  (if Reverse?
    (Utilities|FlowControl|Sequence
      (:then_0
        (Utilities|FlowControl|DoOnce false :!label _label
          (:Completed
            (Class|WheeledVehicleMovementComponent|SetUseAutoGears _vehiclemovement false)
            (Class|WheeledVehicleMovementComponent|SetTargetGear _vehiclemovement -1 true))))
      (:then_1
        (goto _label_2 Reset)))
    (else
      (Utilities|FlowControl|Sequence
        (:then_0
          (Utilities|FlowControl|DoOnce false :!label _label_2
            (:Completed
              (Class|WheeledVehicleMovementComponent|SetTargetGear _vehiclemovement 1 true)
              (Class|WheeledVehicleMovementComponent|SetUseAutoGears _vehiclemovement true))))
        (:then_1
          (goto _label Reset))))))

(event Input|MouseEvents|MouseX
  (params (AxisValue :type Float%20%28single-precision%29))
  ;[1 0.7207 0.4828 1 33] Other inputs
  ;;[0.3718 1 0.4796] Camera rotation
  (for _array_element (Actor|GetComponentsByClass "/Script/Engine.SpringArmComponent")
    (Transformation|AddRelativeRotation _array_element (Math|Rotator|MakeRotator 0.0 0.0 AxisValue) false false)))

(event Input|MouseEvents|MouseY
  (params (AxisValue :type Float%20%28single-precision%29))
  ;[1 0.7207 0.4828 1 33] Other inputs
  ;;[0.3718 1 0.4796] Camera rotation
  (for _array_element (Actor|GetComponentsByClass "/Script/Engine.SpringArmComponent")
    (if (not (> (Math|Float|Absolute(Float) (+ (.pitch (Variables|/Script/Engine.SceneComponent|GetRelativeRotation _array_element)) AxisValue)) 89.0))
      (Transformation|AddRelativeRotation _array_element (Math|Rotator|MakeRotator 0.0 AxisValue 0.0) false false))))

(event Input|KeyboardEvents|Up
  (params (Key :type Key%20Structure :default "None"))
  (bind _vehiclemovement (Variables|Default|GetVehicleMovement))
  ;[1 0.3591 0.2993 1 33] Steering Inputs
  ;;[1 0.3729 0.343] Accelerate
  (:Pressed
    (Class|WheeledVehicleMovementComponent|SetThrottleInput _vehiclemovement 1.0))
  (:Released
    (Class|WheeledVehicleMovementComponent|SetThrottleInput _vehiclemovement 0.0)))

(event Input|KeyboardEvents|Right
  (params (Key :type Key%20Structure :default "None"))
  (bind _vehiclemovement (Variables|Default|GetVehicleMovement))
  ;[1 0.3591 0.2993 1 33] Steering Inputs
  ;;[0.5312 1 0.5849] Steering
  (:Pressed
    (Variables|Default|SetRight%20Input 1.0)
    (Class|WheeledVehicleMovementComponent|SetSteeringInput _vehiclemovement (Variables|Default|GetRight%20Input)))
  (:Released
    (Variables|Default|SetRight%20Input 0.0)
    (Class|WheeledVehicleMovementComponent|SetSteeringInput _vehiclemovement (Variables|Default|GetLeft%20Input))))

(event Input|KeyboardEvents|Enter
  (params (Key :type Key%20Structure :default "None"))
  ;[1 0.7207 0.4828 1 33] Other inputs
  ;;[0.05208 0.05208 0.05208] Leave the vehicle
  (:Pressed
    (bind _outactors (Actor|GetAllActorsOfClass "/Game/Traffic_AI_System/Preview/Preview_blueprints/BP_Preview_pawn.BP_Preview_pawn_C"))
    (Pawn|Possess (Game|GetPlayerController 0) (Utilities|Array|Get(acopy) _outactors))
    (Transformation|SetActorLocation (Utilities|Array|Get(acopy) _outactors) (+ (Transformation|GetActorLocation self) "0, 0,200.000000") false true)
    (Pawn|Possess (Variables|/Game/Traffic_AI_System/Preview/Preview_blueprints/BP_Preview_pawn.BP_Preview_pawn_C|GetUnpossesed%20AI (Utilities|Array|Get(acopy) _outactors)) self)
    (Default|SetCarModeEvent (Variables|Default|GetBP_Traffic_Car_Component) "NewEnumerator1")))

(event Input|KeyboardEvents|O
  (params (Key :type Key%20Structure :default "None"))
  ;[1 1 1] Car doors
  (:Pressed
    (CallFunction|OpenDoors false)))

(event Input|KeyboardEvents|P
  (params (Key :type Key%20Structure :default "None"))
  ;[1 1 1] Car doors
  (:Pressed
    (CallFunction|OpenDoors true)))

(event Input|KeyboardEvents|Left
  (params (Key :type Key%20Structure :default "None"))
  (bind _vehiclemovement (Variables|Default|GetVehicleMovement))
  ;[1 0.3591 0.2993 1 33] Steering Inputs
  ;;[0.5312 1 0.5849] Steering
  (:Pressed
    (Variables|Default|SetLeft%20Input -1.0)
    (Class|WheeledVehicleMovementComponent|SetSteeringInput _vehiclemovement (Variables|Default|GetLeft%20Input)))
  (:Released
    (Variables|Default|SetLeft%20Input 0.0)
    (Class|WheeledVehicleMovementComponent|SetSteeringInput _vehiclemovement (Variables|Default|GetRight%20Input))))

(event Input|KeyboardEvents|Down
  (params (Key :type Key%20Structure :default "None"))
  (bind _bp_car_body_apperance_component (Variables|Default|GetBP_Car_body_apperance_Component))
  (bind _vehiclemovement (Variables|Default|GetVehicleMovement))
  ;[1 0.3591 0.2993 1 33] Steering Inputs
  ;;[0.403 0.5311 1] Brake
  (:Pressed
    (Class|WheeledVehicleMovementComponent|SetBrakeInput _vehiclemovement 1.0)
    (Default|BrakeLight _bp_car_body_apperance_component true))
  (:Released
    (Class|WheeledVehicleMovementComponent|SetBrakeInput _vehiclemovement 0.0)
    (Default|BrakeLight _bp_car_body_apperance_component false)))

(event Input|KeyboardEvents|R
  (params (Key :type Key%20Structure :default "None"))
  (bind _vehiclemovement (Variables|Default|GetVehicleMovement))
  ;[1 0.3591 0.2993 1 33] Steering Inputs
  ;;[1 1 1] Reverse
  (:Pressed
    (Class|WheeledVehicleMovementComponent|SetUseAutoGears _vehiclemovement false)
    (Class|WheeledVehicleMovementComponent|SetTargetGear (Variables|Default|GetVehicleMovement) -1 true)
    (Default|EnableReverseLight (Variables|Default|GetBP_Car_body_apperance_Component) true))
  (:Released
    (Class|WheeledVehicleMovementComponent|SetTargetGear _vehiclemovement 0 true)
    (Class|WheeledVehicleMovementComponent|SetUseAutoGears _vehiclemovement true)
    (Default|EnableReverseLight (Variables|Default|GetBP_Car_body_apperance_Component) false)))

(event Input|KeyboardEvents|SpaceBar
  (params (Key :type Key%20Structure :default "None"))
  (bind _vehiclemovement (Variables|Default|GetVehicleMovement))
  ;[1 0.3591 0.2993 1 33] Steering Inputs
  ;;[1 0.269 0.6684] Handbrake
  (:Pressed
    (Class|WheeledVehicleMovementComponent|SetHandbrakeInput _vehiclemovement true))
  (:Released
    (Class|WheeledVehicleMovementComponent|SetHandbrakeInput _vehiclemovement false)))

(event Input|KeyboardEvents|L
  (params (Key :type Key%20Structure :default "None"))
  ;[1 0.7207 0.4828 1 33] Other inputs
  ;;[1 0.8571 0.3441] Headlights
  (:Pressed
    (bind _isa (Utilities|FlowControl|FlipFlop)
      (:A
        _)
      (:B
        _))
    (Default|EnableHeadlights (Variables|Default|GetBP_Car_body_apperance_Component) _isa)))

(event Input|KeyboardEvents|H
  (params (Key :type Key%20Structure :default "None"))
  (bind _bp_car_body_apperance_component (Variables|Default|GetBP_Car_body_apperance_Component))
  ;[1 0.7207 0.4828 1 33] Other inputs
  ;;[1 1 1] Hazard lights (1.1 Update)
  (:Pressed
    (Default|EnableIndicator _bp_car_body_apperance_component (Variables|/Game/Traffic_AI_System/Components/BP_Car_body_appearance_Component.BP_Car_body_appearance_Component_C|GetIndicator%20state _bp_car_body_apperance_component) (not (Variables|/Game/Traffic_AI_System/Components/BP_Car_body_appearance_Component.BP_Car_body_appearance_Component_C|GetHazard? _bp_car_body_apperance_component)) false)))

(event Input|KeyboardEvents|E
  (params (Key :type Key%20Structure :default "None"))
  (bind _bp_traffic_obstacle_component (Variables|Default|GetBP_Traffic_obstacle_Component))
  (bind _bp_car_body_apperance_component (Variables|Default|GetBP_Car_body_apperance_Component))
  ;[1 0.7207 0.4828 1 33] Other inputs
  ;;[1 0.4851 0.2522] Turn Signal
  (:Pressed
    (switch Utilities|FlowControl|Switch|SwitchonEnum_TurnType (Variables|/Game/Traffic_AI_System/Components/BP_Car_body_appearance_Component.BP_Car_body_appearance_Component_C|GetIndicator%20state (Variables|Default|GetBP_Car_body_apperance_Component))
      (:NewEnumerator0
        (Default|EnableIndicator _bp_car_body_apperance_component "NewEnumerator1" false false :!label _label)
        (Variables|/Game/Traffic_AI_System/Components/BP_Traffic_obstacle_Component.BP_Traffic_obstacle_Component_C|SetFuture%20road%20turn%20type _bp_traffic_obstacle_component "NewEnumerator1"))
      (:NewEnumerator1
        (Default|EnableIndicator _bp_car_body_apperance_component "NewEnumerator0" false false)
        (Variables|/Game/Traffic_AI_System/Components/BP_Traffic_obstacle_Component.BP_Traffic_obstacle_Component_C|SetFuture%20road%20turn%20type _bp_traffic_obstacle_component "NewEnumerator0"))
      (:NewEnumerator2
        (goto _label)))))

(event Input|KeyboardEvents|Q
  (params (Key :type Key%20Structure :default "None"))
  (bind _bp_car_body_apperance_component (Variables|Default|GetBP_Car_body_apperance_Component))
  ;[1 0.7207 0.4828 1 33] Other inputs
  ;;[1 0.4851 0.2522] Turn Signal
  (:Pressed
    (switch Utilities|FlowControl|Switch|SwitchonEnum_TurnType (Variables|/Game/Traffic_AI_System/Components/BP_Car_body_appearance_Component.BP_Car_body_appearance_Component_C|GetIndicator%20state (Variables|Default|GetBP_Car_body_apperance_Component))
      (:NewEnumerator0
        (Default|EnableIndicator _bp_car_body_apperance_component "NewEnumerator2" false false :!label _label)
        (Variables|/Game/Traffic_AI_System/Components/BP_Traffic_obstacle_Component.BP_Traffic_obstacle_Component_C|SetFuture%20road%20turn%20type (Variables|Default|GetBP_Traffic_obstacle_Component) "NewEnumerator2"))
      (:NewEnumerator1
        (goto _label))
      (:NewEnumerator2
        (Default|EnableIndicator _bp_car_body_apperance_component "NewEnumerator0" false false)
        (Variables|/Game/Traffic_AI_System/Components/BP_Traffic_obstacle_Component.BP_Traffic_obstacle_Component_C|SetFuture%20road%20turn%20type (Variables|Default|GetBP_Traffic_obstacle_Component) "NewEnumerator0")))))

(fn ConstructionScript)