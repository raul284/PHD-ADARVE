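; Gameplay manager for the S1 VR tutorial scenario, guiding the player from introduction through teleporting, item detection and grabbing, NPC conversations and tidying up to the exit.
; It extends a parent manager, binding player, tutorial buddy, item, place-point and NPC events.
; Handlers check the current step, complete it and trigger the next prompt, dialog or door.
; On entering the big room, the player's own buddy replaces the standalone one.
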(event Custom|SetCurrentTuddyOnTutorialManager
  (params (Tuddy :type BP%20Tutorial%20Buddy%20Object%20Reference))
  (Default|SetCurrentTutorialBuddy (Variables|Default|GetTutorialManager) Tuddy)
  (CallFunction|BindTuddyActions))

(event EventBeginPlay
  (|CallParentFunction)
  (Utilities|FlowControl|Sequence
    (:then_0
      (for _array_element (Variables|Default|GetFirstRoomItems)
        (Rendering|SetActorHiddenInGame _array_element true)))
    (:then_1
      (CallFunction|SetCurrentTuddyonTutorialManager (Variables|Tuddy|GetIndependentTutorialBuddy))
      (Default|HideCurrentTuddy (Variables|Default|GetTutorialManager)))
    (:then_2
      (CallFunction|BindItemActions)
      (CallFunction|BindPlacePointsActions)
      (CallFunction|BindTuddyActions)
      (CallFunction|BindNPCActions))
    (:then_3
      (Default|SetActive (Variables|DestinationPoints|GetTableDestinationPoint) false))
    (:then_4
      (CallFunction|StartScenario)
      (CallFunction|CompleteStep "NewEnumerator9"))))

(event EventTick
  (params (DeltaSeconds :type Float%20%28single-precision%29)))

(event EventSetPlayerData
  (|CallParentFunction)
  (CallFunction|BindPlayerActions))

(event EventStartScenario
  (|CallParentFunction)
  (Utilities|FlowControl|Delay 3.0)
  (CallFunction|SetCurrentGameplayStep "NewEnumerator39")
  (Default|StartExtraLinesDialog (Variables|Default|GetTutorialManager) "NewEnumerator0"))

(event Custom|OnTuddyIntroductionDialogCompleted
  (bind _yes (CallFunction|IsCurrentStep "NewEnumerator39"))
  (if _yes
    (CallFunction|CompleteStep "NewEnumerator39")
    (CallFunction|SetCurrentGameplayStep "NewEnumerator42")
    (Default|AutomaticCall (Variables|Default|GetTutorialManager) "NewEnumerator2")))

(event Custom|OnTuddyIsOnHand
  (bind _yes (CallFunction|IsCurrentStep "NewEnumerator43"))
  (if _yes
    (CallFunction|CompleteStep "NewEnumerator43")
    (CallFunction|SetCurrentGameplayStep "NewEnumerator44")
    (Default|AutomaticCall (Variables|Default|GetTutorialManager) "NewEnumerator7")))

(event Custom|OnFinalConversationCompleted
  (bind _yes (CallFunction|IsCurrentStep "NewEnumerator47"))
  (if _yes
    (CallFunction|CompleteStep "NewEnumerator47")
    (CallFunction|SetCurrentGameplayStep "NewEnumerator7")
    (Utilities|FlowControl|Delay 0.5)
    (Default|HideCurrentTuddy (Variables|Default|GetTutorialManager))
    (Default|AutomaticOpenandLockDoor (Variables|Door|GetExitDoor))))

(event Custom|OnTuddyDialogCompleted
  (params (CurrentTuddyDialogType :type E_TuddyDialogLinesType%20Enum :default "NewEnumerator0") (CurrentExtraLineType :type E_TuddyExtraLineTypes%20Enum :default "NewEnumerator1"))
  (switch Utilities|FlowControl|Switch|SwitchonE_GameplayStepTypes (Variables|Default|GetCurrentStepType)
    (:NewEnumerator39
      (CallFunction|OnTuddyIntroductionDialogCompleted))
    (:NewEnumerator40
      (for _array_element (Variables|Default|GetFirstRoomItems)
        (Variables|/Game/Game/Blueprints/Actors/Items/BP_TutorialPickableItem.BP_TutorialPickableItem_C|SetCanBeDetected _array_element true)))
    (:NewEnumerator41
      (for _array_element_2 (Variables|Default|GetFirstRoomItems)
        (Variables|/Game/Game/Blueprints/Actors/Items/BP_TutorialPickableItem.BP_TutorialPickableItem_C|SetCanBeGrabbed _array_element_2 true)))
    (:NewEnumerator48
      (Default|AutomaticOpenandLockDoor (Variables|Door|GetBigRoomDoor)))
    (:NewEnumerator43
      (CallFunction|OnTuddyIsonHand))
    (:NewEnumerator47
      (CallFunction|OnFinalConversationCompleted))))

(event EventBindTuddyActions
  (|CallParentFunction)
  (EventDispatchers|BindEventtoEDDialogCompleted (Variables|/Game/Game/Blueprints/Tutorial/BP_TutorialBuddy.BP_TutorialBuddy_C|GetAC_TuddyDialogManager (Variables|/Game/Game/Blueprints/Tutorial/BP_TutorialManager.BP_TutorialManager_C|GetCurrentTutorialBuddy (Variables|Default|GetTutorialManager))) (delegate Custom|OnTuddyDialogCompleted)))

(event Custom|UserEnterBigRoom
  (params (OverlappedActor :type Actor%20Object%20Reference) (OtherActor :type Actor%20Object%20Reference))
  (bind _yes (CallFunction|IsCurrentStep "NewEnumerator48"))
  (if _yes
    (if (== OtherActor (Variables|Default|GetPlayer))
      (Actor|DestroyActor (Variables|Tuddy|GetIndependentTutorialBuddy))
      (bind _asbp_player_vr (Utilities|Casting|CastToBP_Player_VR (Variables|Default|GetPlayer)))
      (bind _output_get (Variables|Tuddy|SetWrispTutorialBuddy (Variables|/Game/Game/Blueprints/Characters/Players/BP_Player_VR.BP_Player_VR_C|GetTutorialBuddyActor _asbp_player_vr)))
      (CallFunction|SetCurrentTuddyonTutorialManager _output_get)
      (CallFunction|CompleteStep "NewEnumerator48")
      (CallFunction|SetCurrentGameplayStep "NewEnumerator43")
      (Default|StartExtraLinesDialog (Variables|Default|GetTutorialManager) "NewEnumerator3"))))

(event Custom|OnPlayerEnterOnTableDestinationPoint
  (bind _yes (CallFunction|IsCurrentStep "NewEnumerator42"))
  (if (and _yes (>= (Variables|Default|GetTimesTeleported) 5))
    (Default|SetActive (Variables|DestinationPoints|GetTableDestinationPoint) false)))

(event Custom|UserEnterExitRoom
  (params (OverlappedActor :type Actor%20Object%20Reference) (OtherActor :type Actor%20Object%20Reference))
  (bind _yes (CallFunction|IsCurrentStep "NewEnumerator7"))
  (if _yes
    (if (== OtherActor (Variables|Default|GetPlayer))
      (CallFunction|CompleteStep "NewEnumerator7")
      (Default|CloseDatabase (Variables|Default|GetGameInstance)))))

(event Custom|OnPlayerTeleported
  (bind _yes (CallFunction|IsCurrentStep "NewEnumerator42"))
  (if _yes
    (bind _output_get (Variables|Default|SetTimesTeleported (+ (Variables|Default|GetTimesTeleported) 1)))
    (if (== _output_get 5)
      (Default|Activate (Variables|Default|GetConfetti%20Niagara%20System))
      (Default|HideAutomaticHintPanel (Variables|Default|GetTutorialManager))
      (CallFunction|CompleteStep "NewEnumerator42")
      (Utilities|FlowControl|Delay 1.0)
      (CallFunction|SpawnFirstRoomItems))))

(event EventBindPlayerActions
  (|CallParentFunction)
  (EventDispatchers|BindEventtoEDTeleported (Variables|Default|GetPlayer) (delegate Custom|OnPlayerTeleported))
  (EventDispatchers|BindEventtoEDPlayerEnteronDestinationPoint (Variables|DestinationPoints|GetTableDestinationPoint) (delegate Custom|OnPlayerEnterOnTableDestinationPoint))
  (Collision|BindEventtoOnActorBeginOverlap (Variables|Triggers|GetBigRoomTrigger) (delegate Custom|UserEnterBigRoom))
  (Collision|BindEventtoOnActorBeginOverlap (Variables|Triggers|GetExitRoomTrigger) (delegate Custom|UserEnterExitRoom)))

(event Custom|SpawnFirstRoomItems
  (params (Actor%20Index :type Integer))
  (if (< Actor%20Index (Utilities|Array|Length (Variables|Default|GetFirstRoomItems)))
    (Default|Spawn (Utilities|Array|Get(acopy) (Variables|Default|GetFirstRoomItems) Actor%20Index))
    (Utilities|FlowControl|Delay 0.7)
    (CallFunction|SpawnFirstRoomItems (+ Actor%20Index 1))
    (else
      (Default|CallEDFirstRoomItemsSpawned))))

(event Custom|OnTutorialItemDetected
  (bind _yes (CallFunction|IsCurrentStep "NewEnumerator40"))
  (if _yes
    (bind _completed (CallFunction|IsTutorialItemDetectionPhaseCompleted?))
    (if _completed
      (Default|HideAutomaticHintPanel (Variables|Default|GetTutorialManager))
      (Default|Activate (Variables|Default|GetConfetti%20Niagara%20System))
      (Utilities|FlowControl|Delay 2.0)
      (CallFunction|CompleteStep "NewEnumerator40")
      (CallFunction|SetCurrentGameplayStep "NewEnumerator41")
      (Default|AutomaticCall (Variables|Default|GetTutorialManager) "NewEnumerator5"))))

(event Custom|OnOneItemPlaced
  (params (Item :type BP%20Pickable%20Item%20Object%20Reference) (PlacePoint :type BP%20Place%20Point%20Object%20Reference))
  (bind _yes (CallFunction|IsCurrentStep "NewEnumerator45"))
  (if _yes
    (Default|HideAutomaticHintPanel (Variables|Default|GetTutorialManager))
    (Default|HideCurrentTuddy (Variables|Default|GetTutorialManager))))

(event Custom|OnTutorialItemGrabbed
  (bind _yes (CallFunction|IsCurrentStep "NewEnumerator41"))
  (if _yes
    (bind _completed (CallFunction|IsTutorialItemGrabPhaseCompleted?))
    (if _completed
      (Default|HideAutomaticHintPanel (Variables|Default|GetTutorialManager))
      (Default|Activate (Variables|Default|GetConfetti%20Niagara%20System))
      (Utilities|FlowControl|Delay 0.5)
      (CallFunction|CompleteStep "NewEnumerator41")
      (CallFunction|SetCurrentGameplayStep "NewEnumerator48")
      (Utilities|FlowControl|Delay 1.0)
      (Default|StartExtraLinesDialog (Variables|Default|GetTutorialManager) "NewEnumerator2"))))

(event Custom|OnPlacePointManagerCompleted
  (bind _yes (CallFunction|IsCurrentStep "NewEnumerator45"))
  (if _yes
    (bind _completed (CallFunction|IsTidyUpPhaseCompleted?))
    (if _completed
      (CallFunction|CompleteStep "NewEnumerator45")
      (Default|NextConversation (Variables|Default|GetNPC))
      (CallFunction|SetCurrentGameplayStep "NewEnumerator46"))))

(event Custom|OnFirstRoomItemsSpawned
  (Utilities|FlowControl|Delay 1.0)
  (CallFunction|SetCurrentGameplayStep "NewEnumerator40")
  (Default|AutomaticCall (Variables|Default|GetTutorialManager) "NewEnumerator4"))

(event EventBindItemActions
  (|CallParentFunction)
  (EventDispatchers|BindEventtoEDFirstRoomItemsSpawned (delegate Custom|OnFirstRoomItemsSpawned))
  (for _array_element (Variables|Default|GetFirstRoomItems)
    (EventDispatchers|BindEventtoEDDetectionStarted _array_element (delegate Custom|OnTutorialItemDetected))
    (EventDispatchers|AssignEDInteractionStarted _array_element (delegate Custom|OnTutorialItemGrabbed))))

(event EventBindPlacePointsActions
  (|CallParentFunction)
  (for _array_element (Variables|Default|GetPlacePointManagers)
    (EventDispatchers|BindEventtoEDOneItemHasBeenPlaced _array_element (delegate Custom|OnOneItemPlaced))
    (EventDispatchers|BindEventtoEDAllPlacePointswithItems _array_element (delegate Custom|OnPlacePointManagerCompleted))))

(event Custom|OnNPCConversationFinished
  (params (ConversationNumber :type Integer))
  (switch Utilities|FlowControl|Switch|SwitchonE_GameplayStepTypes (Variables|Default|GetCurrentStepType)
    (:NewEnumerator44
      (CallFunction|OnNPCIntroductionCompleted))
    (:NewEnumerator46
      (CallFunction|OnInformtoNPCCompleted))))

(event Custom|OnNPCIntroductionCompleted
  (bind _yes (CallFunction|IsCurrentStep "NewEnumerator44"))
  (if _yes
    (CallFunction|CompleteStep "NewEnumerator44")
    (CallFunction|SetCurrentGameplayStep "NewEnumerator45")
    (Default|NextConversation (Variables|Default|GetNPC))
    (Utilities|FlowControl|Delay 1.0)
    (Default|ShowCurrentTuddy (Variables|Default|GetTutorialManager))
    (Utilities|FlowControl|Delay 1.0)
    (Default|AutomaticCall (Variables|Default|GetTutorialManager) "NewEnumerator15")
    (for _array_element (Variables|Default|GetPlacePointManagers)
      (Variables|/Game/Game/Blueprints/Actors/Items/PlacePoints/BP_PlacePointManager.BP_PlacePointManager_C|SetCanActivatePoints _array_element true)
      (Default|ShowInfoWidget _array_element))))

(event Custom|OnInformToNPCCompleted
  (bind _yes (CallFunction|IsCurrentStep "NewEnumerator46"))
  (if _yes
    (CallFunction|CompleteStep "NewEnumerator46")
    (CallFunction|SetCurrentGameplayStep "NewEnumerator47")
    (Utilities|FlowControl|Delay 1.0)
    (Default|StartExtraLinesDialog (Variables|Default|GetTutorialManager) "NewEnumerator4")))

(event Custom|OnNPCConversationStarted
  (switch Utilities|FlowControl|Switch|SwitchonE_GameplayStepTypes (Variables|Default|GetCurrentStepType)
    (:NewEnumerator44
      (Default|HideAutomaticHintPanel (Variables|Default|GetTutorialManager))
      (Default|HideCurrentTuddy (Variables|Default|GetTutorialManager)))))

(event EventBindNPCActions
  (|CallParentFunction)
  (bind _npc (Variables|Default|GetNPC)
    (:then
      (EventDispatchers|BindEventtoEDConversationStarted _npc (delegate Custom|OnNPCConversationStarted))
      (EventDispatchers|BindEventtoEDConversationFinished _npc (delegate Custom|OnNPCConversationFinished)))
    (:else
      (Default|Log (Variables|Default|GetGameInstance) "NewEnumerator2" "Falta NPC" false))))

(fn ConstructionScript)

(fn IsTutorialItemDetectionPhaseCompleted?
  (for _array_element (Variables|Default|GetFirstRoomItems)
    (if (not (Variables|/Game/Game/Blueprints/Actors/Items/BP_TutorialPickableItem.BP_TutorialPickableItem_C|GetHasBeenDetected _array_element))
      (return false)))
  (return true))

(fn IsTutorialItemGrabPhaseCompleted?
  (for _array_element (Variables|Default|GetFirstRoomItems)
    (if (not (Variables|/Game/Game/Blueprints/Actors/Items/BP_TutorialPickableItem.BP_TutorialPickableItem_C|GetLiar _array_element))
      (if (not (Variables|/Game/Game/Blueprints/Actors/Items/BP_TutorialPickableItem.BP_TutorialPickableItem_C|GetHasBeenGrabbed _array_element))
        (return false))))
  (return true))

(fn IsTidyUpPhaseCompleted?
  (for _array_element (Variables|Default|GetPlacePointManagers)
    (if (not (Variables|/Game/Game/Blueprints/Actors/Items/PlacePoints/BP_PlacePointManager.BP_PlacePointManager_C|GetAllPointsUsed _array_element))
      (return false)))
  (return true))