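; Dialog manager component for BP_WalkieTalkie that plays voiced conversations between player and NPC when interacted with.
; It groups DataTable rows into conversations by conversation number, rebuilding them on BeginPlay and each conversation start.
; Lines play through the owner's audio and auto-advance when sound finishes; interacting again skips ahead, and interactions are logged to the player's DBManager.
; Quest-option helpers exist, but dialog processing never calls them.
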(event Custom|ProcessDialog
  ;[1 1 1] Process Dialog
  (if (Variables|Default|GetIsTalking?)
    (Variables|Default|SetIsQuest? false)
    (bind _dialog (CallFunction|GetCurrentDialog))
    (switch Utilities|FlowControl|Switch|SwitchonE_DialogType (.type (.DialogData (Utilities|Struct|BreakF_Dialog _dialog)))
      (:NewEnumerator2
        (Development|PrintString "Un diálogo que no tiene dueño :(" true true "(R=1.000000,G=0.000000,B=0.000000,A=1.000000)"))
      (:NewEnumerator0
        (CallFunction|CreatePlayerDialog))
      (:NewEnumerator1
        (CallFunction|CreateNPCDialog)))))

(event Custom|Interact%20With
  (if (not (Variables|Default|GetIsTalking?))
    (CallFunction|StartConversation)
    (CallFunction|SendDialogEventtoDB "NewEnumerator10")
    (elif (not (Variables|Default|GetIsQuest?))
      (bind _continue (CallFunction|NextDialog))
      (if _continue
        (CallFunction|ContinueDialog)
        (else
          (CallFunction|StopConversation)))
      (CallFunction|SendDialogEventtoDB "NewEnumerator20"))))

(event Custom|StartConversation
  ;[1 1 1] Conversation
  (CallFunction|SetDialogsfromDataTable)
  (bind _isempty (CallFunction|IsConversationEmpty))
  (if (and (not _isempty) (Variables|Default|GetCanStartConversation?))
    (Variables|Default|SetIsTalking? true)
    (Variables|Default|SetDialogIndex 0)
    (CallFunction|ProcessDialog)))

(event Custom|ContinueDialog
  ;[1 1 1] Process Dialog
  (CallFunction|ProcessDialog))

(event Custom|SendDialogEventToDB
  (params (Event%20Type :type E_InteractEventType%20Enum :default "NewEnumerator4"))
  (bind _owner (Variables|Default|GetOwner))
  (bind _player (Variables|/Game/Game/Blueprints/Actors/Items/BP_InteractItemParent.BP_InteractItemParent_C|GetPlayer _owner))
  ;[1 1 1] Database
  (bind _dbmanager (Variables|/Game/Game/Blueprints/Characters/Players/BP_Player.BP_Player_C|GetDBManager _player)
    (:then
      (Default|SendInteractEventtoDB _dbmanager (Utilities|Struct|MakeF_InteractEventsTableItem 0 (Variables|/Game/Game/Blueprints/Actors/Items/BP_InteractItemParent.BP_InteractItemParent_C|GetActorId (Variables|Default|GetOwner)) (Variables|/Game/Game/Blueprints/Characters/Players/BP_Player.BP_Player_C|GetUserId _player) "NewEnumerator0" Event%20Type (Math|DateTime|Now))))
    (:else)))

(event Custom|PlayDialogSound
  (bind _owner (Variables|Default|GetOwner))
  (bind _audio (Variables|/Game/Game/Blueprints/Actors/BP_WalkieTalkie.BP_WalkieTalkie_C|GetAudio _owner))
  ;[1 1 1] Sound
  (bind _dialog (CallFunction|GetCurrentDialog))
  (Audio|Components|Audio|SetSound _audio (.Voice (Utilities|Struct|BreakF_DialogLine (.dialogdata _dialog))))
  (Audio|Components|Audio|Play _audio 0.0)
  (EventDispatchers|BindEventtoOnAudioFinished _audio (delegate Custom|OnDialogSoundFinished)))

(event Custom|OnDialogSoundFinished
  ;[1 1 1] Sound
  (if (and (Variables|Default|GetIsTalking?) (not (Variables|Default|GetIsQuest?)))
    (Utilities|FlowControl|Delay 0.2)
    (bind _continue (CallFunction|NextDialog))
    (if _continue
      (CallFunction|ProcessDialog)
      (else
        (CallFunction|StopConversation)))))

(event Custom|StopConversation
  ;[1 1 1] Conversation
  (Variables|Default|SetIsTalking? false)
  (Default|CallConversationFinished (Variables|Default|GetConversationIndex)))

(event EventBeginPlay
  (Utilities|FlowControl|Sequence
    (:then_0
      (bind _asbp_walkie_talkie (Utilities|Casting|CastToBP_WalkieTalkie (Components|GetOwner)))
      (Variables|Default|SetOwner _asbp_walkie_talkie))
    (:then_2
      (CallFunction|SetDialogsfromDataTable))))

(event EventTick
  (params (DeltaSeconds :type Float%20%28single-precision%29)))

(fn NextDialog
  (bind _conversations (Variables|Default|GetConversations))
  (bind _conversationindex (Variables|Default|GetConversationIndex))
  (bind _output (Utilities|Array|Get(acopy) _conversations _conversationindex))
  (bind _dialogs (Utilities|Struct|BreakF_DialogsArray _output))
  (bind _returnvalue (Utilities|Array|Length _dialogs))
  (if (and (> _returnvalue 0) (< (+ (Variables|Default|GetDialogIndex) 1) _returnvalue))
    (Math|Integer|IncrementInt (Variables|Default|GetDialogIndex)
      (:%20%20
        (return true)))
    (else
      (return false))))

(fn NextConversation
  (bind _isempty (CallFunction|IsConversationEmpty))
  (if (and (not _isempty) (< (Variables|Default|GetConversationIndex) (- (Utilities|Array|Length (Variables|Default|GetConversations)) 1)))
    (Variables|Default|SetConversationIndex (+ (Variables|Default|GetConversationIndex) 1))))

(fn SetDialogsfromDataTable
  (Utilities|Array|Clear (Variables|Default|GetConversations))
  (bind _dialog_data_table (Variables|Default|GetDialog%20Data%20Table)
    (:then
      (bind _returnvalue (Class|DataTableFunctionLibrary|GetDataTableColumnasString _dialog_data_table "Conversation Number"))
      (bind _number_of_conversations (CallFunction|GetNumberOfConversations _returnvalue))
      (Utilities|FlowControl|ForLoopwithBreak 0 (- _number_of_conversations 1)
        (:LoopBody
          (Utilities|Array|Add (Variables|Default|GetConversations) (Utilities|Struct|MakeF_DialogsArray)))
        (:Completed
          (bind _outrownames (DataTable|GetDataTableRowNames _dialog_data_table))
          (for _array_element _outrownames
            (bind _returnvalue_2 (Utilities|GetDataTableRow _dialog_data_table _array_element)
              (:then
                (Utilities|Array|Add (Utilities|Struct|BreakF_DialogsArray (Utilities|Array|Get(acopy) (Variables|Default|GetConversations) (.ConversationNumber (Utilities|Struct|BreakF_Dialog _returnvalue_2)))) (Utilities|Struct|MakeF_Dialog (.ConversationNumber (Utilities|Struct|BreakF_Dialog _returnvalue_2)) 0.0 (.DialogData (Utilities|Struct|BreakF_Dialog _returnvalue_2)) (.QuestionFirstOption (Utilities|Struct|BreakF_Dialog _returnvalue_2)) (.QuestionSecondOption (Utilities|Struct|BreakF_Dialog _returnvalue_2))))))))))
    (:else)))

(fn GetNumberOfConversations
  (params (List%20of%20Dialogs :type Array%20of%20Strings))
  (for _array_element List%20of%20Dialogs
    (Utilities|Set|Add (LocalVariables|GetAuxSet) _array_element))
  (return (Utilities|Set|Length (LocalVariables|GetAuxSet))))

(fn GetCurrentDialog
  (return (Utilities|Array|Get(acopy) (Utilities|Struct|BreakF_DialogsArray (Utilities|Array|Get(acopy) (Variables|Default|GetConversations) (Variables|Default|GetConversationIndex))) (Variables|Default|GetDialogIndex))))

(fn AddOptionDialogstoConversation
  (params (New%20Dialogs :type Array%20of%20F%20Dialog%20Line%20Structures))
  (for (_array_element _array_index) New%20Dialogs
    (Utilities|Array|Insert (Utilities|Struct|BreakF_DialogsArray (Utilities|Array|Get(acopy) (Variables|Default|GetConversations) (Variables|Default|GetConversationIndex))) (Utilities|Struct|MakeF_Dialog (Variables|Default|GetConversationIndex) 0.0 _array_element) (+ (Variables|Default|GetDialogIndex) 1 _array_index))))

(fn IsConversationEmpty
  (return (== (Utilities|Array|Length (Variables|Default|GetConversations)) 0)))

(fn CreatePlayerDialog
  (CallFunction|PlayDialogSound))

(fn CreateNPCDialog
  (CallFunction|PlayDialogSound))

(fn CreateNPCQuest
  (bind _widget (Variables|Default|GetWidget))
  (Variables|Default|SetIsQuest? true)
  (CallFunction|CreateNPCDialog)
  (bind _dialog (CallFunction|GetCurrentDialog))
  (Default|SetOptionsText _widget (.Text (Utilities|Struct|BreakF_QuestOption (.QuestionFirstOption (Utilities|Struct|BreakF_Dialog _dialog)))) (.Text (Utilities|Struct|BreakF_QuestOption (.QuestionSecondOption (Utilities|Struct|BreakF_Dialog _dialog)))))
  (Default|ShowOptions _widget))