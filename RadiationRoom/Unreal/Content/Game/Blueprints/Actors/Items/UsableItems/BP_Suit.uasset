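; BP_Suit is a usable item that the player holds to put on a security suit over time.
; Interacting reveals a wear-progress widget if the player is unsuited; its Wear button starts audio and a Tick-driven timer that updates progress.
; Cancelling resets the timer; completion fires the Dressed dispatcher, flags the player as suited and destroys the actor after a delay.
; It also registers itself in the gameplay manager's important-item list.
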(event Custom|On_WearButtonClicked
  (Variables|Default|SetGettingDressed true)
  (Audio|Components|Audio|Play (Variables|Default|GetAudio) 0.0))

(event Custom|GetDress
  (params (DeltaTime :type Float%20%28double-precision%29))
  (if (and (Variables|Default|GetGettingDressed) (not (Variables|Default|GetDressed)))
    (Variables|Default|SetCurrentTimer (+ (Variables|Default|GetCurrentTimer) DeltaTime))
    (Default|SetProgress (Variables|Default|GetWidgetActor) (|({935F46A7-4DA4-627D-E003-AAB31168D55F}/{E30B1488-4717-F42E-FA68-63BC8AC6DC69})))
    (if (>= (Variables|Default|GetCurrentTimer) (Variables|Default|GetMaxTimer))
      (CallFunction|GetDressedProgressCompleted))))

(event Custom|GetDressedProgressCompleted
  (Variables|Default|SetDressed true)
  (Variables|Default|SetGettingDressed false)
  (Default|CallEDDressed)
  (Variables|/Game/Game/Blueprints/Characters/Players/BP_Player.BP_Player_C|SetIsWearingASecuritySuit (Variables|Default|GetPlayer) true)
  (Utilities|FlowControl|Delay 1.0)
  (Actor|DestroyActor))

(event EventBeginPlay
  (bind _gameplaymanager (CallFunction|GetMyGameplayManager))
  (|CallParentFunction)
  (Utilities|FlowControl|Sequence
    (:then_0
      (bind _aswbp_wear_suit_progress (Utilities|Casting|CastToWBP_WearSuitProgress (UserInterface|GetWidget (Variables|Default|GetWidgetComponent))))
      (Variables|Default|SetWidgetActor _aswbp_wear_suit_progress)
      (Development|SetHiddeninGame (Variables|Default|GetWidgetComponent) true false)
      (EventDispatchers|AssignEDWear (Variables|Default|GetWidgetActor) (delegate Custom|On_WearButtonClicked)))
    (:then_1
      (Utilities|IsValid _gameplaymanager
        (:Is%20Valid
          (Default|AddItemtoGameManagerImportantList _gameplaymanager (Variables|Default|GetItemType) self))))))

(event EventTick
  (params (DeltaSeconds :type Float%20%28single-precision%29))
  (|CallParentFunction DeltaSeconds)
  (CallFunction|GetDress DeltaSeconds))

(event EventInteractwith
  (params (Player :type BP%20Player%20Object%20Reference) (Hand :type EControllerHand%20Enum :default "Left"))
  (|CallParentFunction Player "Left")
  (if (not (Variables|/Game/Game/Blueprints/Characters/Players/BP_Player.BP_Player_C|GetIsWearingASecuritySuit Player))
    (Default|OnSuitGrabbed (Variables|Default|GetWidgetActor))
    (Development|SetHiddeninGame (Variables|Default|GetWidgetComponent) false false)))

(event EventCancelInteract
  (params (Player :type BP%20Player%20Object%20Reference) (Hand :type EControllerHand%20Enum :default "Left"))
  (|CallParentFunction Player "Left")
  (Variables|Default|SetGettingDressed false)
  (Variables|Default|SetCurrentTimer 0.0)
  (Development|SetHiddeninGame (Variables|Default|GetWidgetComponent) true false)
  (Audio|Components|Audio|Stop (Variables|Default|GetAudio)))

(fn ConstructionScript
  (|CallParentFunction))