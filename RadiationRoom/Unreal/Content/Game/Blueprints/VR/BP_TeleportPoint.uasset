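; VR teleport point Blueprint with a text label that turns to face the local player; its graphs hold no teleport logic.
; Every tick, it casts the pawn of the local player controller to BP_Player and computes a look-at rotation from the TextRender to that pawn's mesh.
; It applies only yaw and roll from that rotation, keeping the text's current pitch so the label does not tilt up or down.
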(event Custom|LookAtPlayer
  (bind _returnvalue (Game|GetPlayerController 0))
  (bind _textrender (Variables|Default|GetTextRender))
  (if (Pawn|IsLocalController _returnvalue)
    (bind _asbp_player_parent (Utilities|Casting|CastToBP_Player (Pawn|GetControlledPawn _returnvalue)))
    (Transformation|SetWorldRotation (Variables|Default|GetTextRender) (Math|Rotator|MakeRotator (.roll (Math|Rotator|FindLookatRotation (Transformation|GetWorldLocation _textrender) (Transformation|GetWorldLocation (Variables|/Script/Engine.Character|GetMesh _asbp_player_parent)))) (.pitch (Transformation|GetWorldRotation _textrender)) (.yaw (Math|Rotator|FindLookatRotation (Transformation|GetWorldLocation _textrender) (Transformation|GetWorldLocation (Variables|/Script/Engine.Character|GetMesh _asbp_player_parent))))) false false)))

(event EventTick
  (params (DeltaSeconds :type Float%20%28single-precision%29))
  (CallFunction|LookatPlayer))

(fn ConstructionScript)