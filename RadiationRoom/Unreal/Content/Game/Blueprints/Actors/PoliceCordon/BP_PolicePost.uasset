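; Police cordon post actor with a cable rope that stretches from its pole to another post or any attached actor.
; The rope starts hidden and appears on start attachment, while attach and detach events set the end actor and state flags.
; Every tick it recomputes the cable end offset and length, targeting the other post's rope component or the actor's root.
; Start detachment is an empty stub.
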(event Custom|RopeEndMoving
  (bind _endactor (Variables|Default|GetEndActor))
  (bind _cable (Variables|Default|GetCable))
  (bind _cable_2 (Variables|Default|GetCable))
  (Utilities|IsValid _endactor
    (:Is%20Valid
      (Variables|/Script/CableComponent.CableComponent|SetbAttachEnd (Variables|Default|GetCable) true)
      (bind _asbp_police_post (Utilities|Casting|CastToBP_PolicePost _endactor)
        (:then
          (bind _endpoint (CallFunction|GetDistance (Variables|BP_PolicePost_C|GetRopeInPole _asbp_police_post)))
          (bind _output_get (Variables|/Script/CableComponent.CableComponent|SetEndLocation _cable_2 (Math|Vector|MakeVector (.X (Math|Vector|BreakVector _endpoint)) (.Y (Math|Vector|BreakVector _endpoint)) 3e+01)))
          (Variables|/Script/CableComponent.CableComponent|SetCableLength _cable_2 (/ (Math|Vector|VectorLength _output_get) 1.5)))
        (:CastFailed
          (bind _endpoint_2 (CallFunction|GetDistance (Variables|/Script/Engine.Actor|GetRootComponent _endactor)))
          (bind _output_get_2 (Variables|/Script/CableComponent.CableComponent|SetEndLocation _cable (+ _endpoint_2 "0, 0,30.000000")))
          (Variables|/Script/CableComponent.CableComponent|SetCableLength _cable (/ (Math|Vector|VectorLength _output_get_2) 1.5)))))))

(event Custom|AttachRopeStart
  (params (ActorToAttach :type Actor%20Object%20Reference))
  (Variables|Default|SetEndActor ActorToAttach)
  (Rendering|SetVisibility (Variables|Default|GetRopeInPole) true false)
  (Rendering|SetVisibility (Variables|Default|GetCable) true false)
  (Variables|Default|SetRopeAttachedToStart true))

(event Custom|AttachRopeEnd
  (params (ActorToAttach :type Actor%20Object%20Reference))
  (Variables|Default|SetEndActor ActorToAttach)
  (Variables|Default|SetRopeAttachedToEnd true))

(event Custom|DetachRopeStart)

(event Custom|DetachRopeEnd
  (params (ActorToAttach :type Actor%20Object%20Reference))
  (Variables|Default|SetEndActor ActorToAttach)
  (Variables|Default|SetRopeAttachedToEnd false))

(event EventBeginPlay
  (Rendering|SetVisibility (Variables|Default|GetRopeInPole) false false)
  (Rendering|SetVisibility (Variables|Default|GetCable) false false))

(event EventTick
  (params (DeltaSeconds :type Float%20%28single-precision%29))
  (CallFunction|RopeEndMoving))

(fn ConstructionScript)

(fn GetDistance
  (params (EndActor :type Scene%20Component%20Object%20Reference))
  (return (- (Transformation|GetWorldLocation EndActor) (Transformation|GetWorldLocation (Variables|Default|GetRopeInPole)))))