(event Custom|CheckIfUserIdSelect
  (params (Data :type Array%20of%20My%20SQL%20Data%20Table%20Structures))
  (bind _output (Utilities|Array|Get(acopy) Data 1))
  (bind _output_2 (Utilities|Array|Get(acopy) (.columndata _output)))
  (if (Math|Boolean|ANDBoolean (== (Utilities|Array|Length Data) 2) (Utilities|Enum|Equal(Enum) (.columnname (Utilities|Array|Get(acopy) Data)) "id") (Utilities|Enum|Equal(Enum) (.columnname (Utilities|Array|Get(acopy) Data 1)) "user_name"))
    (bind _asrr_game_instance (Utilities|Casting|CastToRR_GameInstance (Game|GetGameInstance)))
    (if (Utilities|Enum|Equal(Enum) (Variables|/Game/Game/Blueprints/RR_GameInstance.RR_GameInstance_C|GetPlayerName _asrr_game_instance) _output_2)
      (Default|SetPlayerData _asrr_game_instance (Math|Conversions|ToInteger(Byte) (Utilities|Array|Get(acopy) (.columndata (Utilities|Array|Get(acopy) Data)))) _output_2))))

(event Custom|CloseDatabase
  (Variables|Default|SetNeedToStop true)
  (if (Variables|Default|GetCanStop)
    (Class|MySQLDBConnectionActor|CloseConnection (Variables|Default|GetConnection%20ID))
    (Utilities|FlowControl|Delay 1.0)
    (Default|CallEDServerDatabaseClosed)))

(event Custom|ConnectToDataBase
  ;[1 1 1] Connect to Database
  (Networking|SwitchHasAuthority
    (:Authority
      (Class|MySQLDBConnectionActor|CloseAllConnections)
      (Class|MySQLDBConnectionActor|CreateNewConnection "medusa.fdi.ucm.es" "adarve-db" "root" "root" 3306))))

(event EventBeginPlay
  (CallFunction|ConnecttoDataBase))

(event EventCreateMoveEventQuery
  (params (Data :type F%20Move%20Events%20Table%20Item%20Structure))
  (bind (_event_id _user_id _scenary_type _move_type _start_datetime _end_datetime _start_position _end_position _distance) (Utilities|Struct|BreakF_MoveEventsTableItem Data))
  (bind _datetimes (CallFunction|DatetimetoString _start_datetime))
  (bind _datetimes_2 (CallFunction|DatetimetoString _end_datetime))
  (bind _asrr_game_instance (Utilities|Casting|CastToRR_GameInstance (Game|GetGameInstance)))
  (CallFunction|AddUpdateQuery (Utilities|String|ToString(Text) (Utilities|Text|FormatText "INSERT INTO {schema}.move_events (user_id, scenary_type, move_type, start_datetime, end_datetime, start_position, end_position, distance) VALUES({user_id}, \"{scenary_type}\", \"{move_type}\", \"{start_datetime}\", \"{end_datetime}\", \"{start_position}\", \"{end_position}\", \"{distance}\")" (Variables|Default|GetDB%20Schema%20Name) _user_id (Utilities|String|EnumtoString (Variables|/Game/Game/Blueprints/RR_GameInstance.RR_GameInstance_C|GetCurrentScenary _asrr_game_instance)) (Utilities|String|EnumtoString _move_type) _datetimes _datetimes_2 (Utilities|String|ToString(Vector) _start_position) (Utilities|String|ToString(Vector) _end_position) (Utilities|String|ToString(Float) _distance)))))

(event EventAddSelectQuery
  (params (Query :type String))
  ;[1 1 1] Select
  (Networking|SwitchHasAuthority
    (:Authority
      (if (not (Variables|Default|GetNeedToStop))
        (Variables|Default|SetSelectQuery Query)
        (Variables|Default|SetWaitingSelectQuerys true)))))

(event EventOnQueryUpdateStatusChanged
  (params (ConnectionID :type Integer) (QueryID :type Integer) (IsSuccessful :type Boolean) (ErrorMessage :type String))
  ;[1 1 1] Insert Query
  (Networking|SwitchHasAuthority
    (:Authority
      (if IsSuccessful
        _
        (else
          (Development|PrintString ErrorMessage true true "(R=1.000000,G=0.000000,B=0.000000,A=1.000000)")))
      (Variables|Default|SetCanInsertNextQuery true)
      (bind _empty (CallFunction|IsUpdateQuerysQueueEmpty))
      (if _empty
        (Variables|Default|SetWaitingUpdateQuerys false)
        (Variables|Default|SetCanStop true)
        (Development|PrintString "Puedes cerrar")))))

(event EventOnQuerySelectStatusChanged
  (params (ConnectionID :type Integer) (QueryID :type Integer) (IsSuccessful :type Boolean) (ErrorMessage :type String) (ResultByColumn :type Array%20of%20My%20SQL%20Data%20Table%20Structures) (ResultByRow :type Array%20of%20My%20SQL%20Data%20Row%20Structures))
  ;[1 1 1] Select
  (Networking|SwitchHasAuthority
    (:Authority
      (if IsSuccessful
        (CallFunction|CheckifUserIdSelect ResultByColumn)
        (else
          (Development|PrintString ErrorMessage true true "(R=1.000000,G=0.000000,B=0.000000,A=1.000000)")))
      (bind _empty (CallFunction|IsSelectQuerysQueueEmpty))
      (if _empty
        (Variables|Default|SetWaitingSelectQuerys false)
        (Variables|Default|SetCanStop true)))))

(event EventTick
  (params (DeltaSeconds :type Float%20%28single-precision%29))
  (if (and (not (Variables|Default|GetConnectionFailed)) (Variables|Default|GetConnected))
    (Utilities|FlowControl|Sequence
      (:then_0
        (if (Variables|Default|GetWaitingUpdateQuerys)
          (if (Variables|Default|GetCanInsertNextQuery)
            (Variables|Default|SetCanStop false)
            (CallFunction|SendUpdateQuerystoDB))))
      (:then_1
        (if (Variables|Default|GetWaitingSelectQuerys)
          (Utilities|FlowControl|Delay 0.2)
          (Variables|Default|SetCanStop false)
          (CallFunction|SendSelectQuerystoDB)))
      (:then_2
        (if (Variables|Default|GetNeedToStop)
          (CallFunction|CloseDatabase))))))

(event EventAddUpdateQuery
  (params (Query :type String))
  ;[1 1 1] Insert Query
  (Networking|SwitchHasAuthority
    (:Authority
      (if (not (Variables|Default|GetNeedToStop))
        (Utilities|Array|Add (Variables|Default|GetUpdateQueryQueue) Query)
        (Variables|Default|SetWaitingUpdateQuerys true)))))

(event EventOnConnectionStateChanged
  (params (ConnectionStatus :type Boolean) (ConnectionID :type Integer) (ErrorMessage :type String))
  ;[1 1 1] Connect to Database
  (if (not (Variables|Default|GetConnectionFailed))
    (Networking|SwitchHasAuthority
      (:Authority
        (if ConnectionStatus
          (Variables|Default|SetConnected true)
          (Variables|Default|SetConnection%20ID ConnectionID)
          (else
            (Development|PrintString ErrorMessage true true "(R=1.000000,G=0.000000,B=0.000000,A=1.000000)")
            (Variables|Default|SetConnectionFailed true)))))))

(event EventSendSelectQuerystoDB
  ;[1 1 1] Select
  (Networking|SwitchHasAuthority
    (:Authority
      (bind _empty (CallFunction|IsSelectQuerysQueueEmpty))
      (if (not _empty)
        (Class|MySQLDBConnectionActor|SelectDatafromQuery (Variables|Default|GetConnection%20ID) (Variables|Default|GetSelectQuery))
        (Variables|Default|SetSelectQuery "")))))

(event EventSendUpdateQuerystoDB
  ;[1 1 1] Insert Query
  (Networking|SwitchHasAuthority
    (:Authority
      (bind _empty (CallFunction|IsUpdateQuerysQueueEmpty))
      (if (not _empty)
        (Class|MySQLDBConnectionActor|UpdateDatafromMultipleQueries (Variables|Default|GetConnection%20ID) (Variables|Default|GetUpdateQueryQueue))
        (Variables|Default|SetCanInsertNextQuery false)
        (Utilities|Array|Clear (Variables|Default|GetUpdateQueryQueue))))))

(fn ConstructionScript)

(fn IsUpdateQuerysQueueEmpty
  (return (== (Utilities|Array|Length (Variables|Default|GetUpdateQueryQueue)) 0)))

(fn IsSelectQuerysQueueEmpty
  (return (Utilities|Enum|Equal(Enum) (Variables|Default|GetSelectQuery) "")))

(fn CreateExperimentInsertQuery
  (params (Data :type F%20Experiment%20Table%20Item%20Structure))
  (return))

(fn CreateGameplayEventInsertQuery
  (params (Data :type F%20Gameplay%20Events%20Table%20Item%20Structure))
  (bind (_event_id _user_id _scenary_type _event_type _event_datetime) (Utilities|Struct|BreakF_GameplayEventsTableItem Data))
  (bind _datetimes (CallFunction|DatetimetoString _event_datetime))
  (bind _asrr_game_instance (Utilities|Casting|CastToRR_GameInstance (Game|GetGameInstance)))
  (CallFunction|AddUpdateQuery (Utilities|String|ToString(Text) (Utilities|Text|FormatText "INSERT INTO {schema}.gameplay_events (user_id, scenary_type, event_type, event_datetime) VALUES(\"{user_id}\",\"{scenary_type}\", \"{event_type}\", \"{event_datetime}\")" (Variables|Default|GetDB%20Schema%20Name) _user_id (Utilities|String|EnumtoString (Variables|/Game/Game/Blueprints/RR_GameInstance.RR_GameInstance_C|GetCurrentScenary _asrr_game_instance)) (Utilities|String|EnumtoString _event_type) _datetimes)))
  (return))

(fn CreateInteractEventInsertQuery
  (params (Data :type F%20Interact%20Events%20Table%20Item%20Structure))
  (bind (_event_id _actor_id _user_id _scenary_type _event_type _event_datetime) (Utilities|Struct|BreakF_InteractEventsTableItem Data))
  (bind _datetimes (CallFunction|DatetimetoString _event_datetime))
  (bind _asrr_game_instance (Utilities|Casting|CastToRR_GameInstance (Game|GetGameInstance)))
  (CallFunction|AddUpdateQuery (Utilities|String|ToString(Text) (Utilities|Text|FormatText "INSERT INTO {schema}.interact_events (actor_id, user_id, scenary_type, event_type, event_datetime) VALUES({actor_id}, {user_id}, \"{scenary_type}\",\"{event_type}\", \"{event_datetime}\")" (Variables|Default|GetDB%20Schema%20Name) _actor_id _user_id (Utilities|String|EnumtoString (Variables|/Game/Game/Blueprints/RR_GameInstance.RR_GameInstance_C|GetCurrentScenary _asrr_game_instance)) (Utilities|String|EnumtoString _event_type) _datetimes)))
  (return))

(fn CreateSessionInsertQuery
  (params (Data :type F%20Session%20Table%20Item%20Structure))
  (return))

(fn CreateTeamInsertQuery
  (params (Data :type F%20Team%20Table%20Item%20Structure))
  (return))

(fn CreateUserInsertQuery
  (params (Data :type F%20User%20Table%20Item%20Structure))
  (bind (_user_id _user_name _user_type) (Utilities|Struct|BreakF_UserTableItem Data))
  (CallFunction|AddUpdateQuery (Utilities|String|ToString(Text) (Utilities|Text|FormatText "INSERT INTO {schema}.users (user_name, user_type) VALUES(\"{user_name}\", \"{user_type}\")" (Variables|Default|GetDB%20Schema%20Name) _user_name (Utilities|String|EnumtoString _user_type))))
  (return))

(fn DatetimetoString
  (params (Datetime :type Date%20Time%20Structure))
  (return (Utilities|String|Append (Utilities|String|ToString(Integer) (.year Datetime)) "-" (Utilities|String|ToString(Integer) (.month Datetime)) "-" (Utilities|String|ToString(Integer) (.day Datetime)) " " (Utilities|String|ToString(Integer) (.hour Datetime)) ":" (Utilities|String|ToString(Integer) (.minute Datetime)) ":" (Utilities|String|ToString(Integer) (.second Datetime)))))

(fn GetUserId
  (params (Player%20Name :type String))
  (CallFunction|AddSelectQuery (Utilities|String|ToString(Text) (Utilities|Text|FormatText "SELECT id, user_name FROM {schema}.users WHERE user_name = '{user_name}' ORDER BY id DESC LIMIT 0, 1" (Variables|Default|GetDB%20Schema%20Name) Player%20Name)))
  (return))