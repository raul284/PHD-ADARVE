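; Actor component that tracks an actor's progress through an ordered list of phases.
; SetCurrentPhase copies the indexed list entry into CurrentPhase, printing a warning if the list is empty, and NextPhase advances the index up to the last entry.
; Check functions test whether a phase is current, or current or earlier; the latter also returns true for phases missing from the list while the index is non-negative.
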(event EventBeginPlay)

(event EventTick
  (params (DeltaSeconds :type Float%20%28single-precision%29)))

(fn SetCurrentPhase
  (bind _empty (CallFunction|IsPhaseListEmpty))
  (if _empty
    (Development|PrintString "No hay fases en este actor.")
    (else
      (Variables|Default|SetCurrentPhase (Utilities|Array|Get(acopy) (Variables|Default|GetPhasesList) (Variables|Default|GetCurrentPhaseIndex))))))

(fn IsPhaseListEmpty
  (return (== (Utilities|Array|Length (Variables|Default|GetPhasesList)) 0)))

(fn NextPhase
  (if (< (Variables|Default|GetCurrentPhaseIndex) (- (Utilities|Array|Length (Variables|Default|GetPhasesList)) 1))
    (Variables|Default|SetCurrentPhaseIndex (+ (Variables|Default|GetCurrentPhaseIndex) 1))
    (CallFunction|SetCurrentPhase)))

(fn CheckCurrentPhase
  (params (Phase :type E_ActorPhaseTypes%20Enum :default "NewEnumerator3"))
  (return (Utilities|Enum|Equal(Enum) (Variables|Default|GetCurrentPhase) Phase)))

(fn CheckCurrentorPrePhase
  (params (Phase :type E_ActorPhaseTypes%20Enum :default "NewEnumerator3"))
  (bind _correct (CallFunction|CheckCurrentPhase Phase))
  (return (or _correct (< (Utilities|Array|FindItem (Variables|Default|GetPhasesList) Phase) (Variables|Default|GetCurrentPhaseIndex)))))