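; BP_Van is an interactable van actor that layers its own look-at and interact handling on the parent item behavior.
; Interacting logs the actor, user and timestamp to the database through DBManager when it is valid.
; Both handlers cast to the third-person (TFP) and VR players with no follow-up logic.
; Logic that swaps in the open-van mesh and completes a gameplay step is disconnected and never runs.
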(event EventBeginPlay
  (|CallParentFunction) ; This node is disabled and will not be called.\nDrag off pins to build functionality.
)

(event EventInteractwith
  (params (Player :type BP%20Player%20Object%20Reference))
  (|CallParentFunction Player)
  (Utilities|FlowControl|Sequence
    (:then_0
      (bind _dbmanager (Variables|Default|GetDBManager)
        (:then
          (Default|SendInteractEventtoDB _dbmanager (Utilities|Struct|MakeF_InteractEventsTableItem 0 (Variables|Default|GetActorId) (Variables|/Game/Game/Blueprints/Characters/Players/BP_Player.BP_Player_C|GetUserId Player) "NewEnumerator0" "NewEnumerator4" (Math|DateTime|Now))))
        (:else)))
    (:then_2
      (Utilities|FlowControl|Sequence
        (:then_0
          (Utilities|Casting|CastToBP_Player_TFP Player))
        (:then_1
          (Utilities|Casting|CastToBP_Player_VR Player))))))

(event EventStartLookat
  (params (Player :type BP%20Player%20Object%20Reference))
  (|CallParentFunction Player)
  (Utilities|FlowControl|Sequence
    (:then_0
      (Utilities|Casting|CastToBP_Player_TFP Player))
    (:then_1
      (Utilities|Casting|CastToBP_Player_VR Player))))

(fn ConstructionScript
  (|CallParentFunction))