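; Fire truck Blueprint that spawns objective items when a firefighter mate NPC overlaps its trigger during one specific objective type.
; A data table row matching the GameplayManager's scenario and objective types supplies the item classes and counts.
; A self-calling, one-second delayed event places items at unoccupied BP_SpawnItemPoint actors, retrying when none is free and tracking spawn progress with flags.
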(event OnComponentBeginOverlap(NPCTrigger)
  (params (OverlappedComponent :type Primitive%20Component%20Object%20Reference) (OtherActor :type Actor%20Object%20Reference) (OtherComp :type Primitive%20Component%20Object%20Reference) (OtherBodyIndex :type Integer) (bFromSweep :type Boolean) (SweepResult :type Hit%20Result%20Structure%20%28by%20ref%29))
  (Utilities|Casting|CastToBP_NPC_FirefighterMate OtherActor)
  (if (Utilities|Enum|Equal(Enum) (Variables|/Game/Game/Blueprints/Gameplay/BP_GameplayManager.BP_GameplayManager_C|GetCurrentObjectiveType (Variables|Default|GetGameplayManager)) "NewEnumerator9")
    (if (not (Variables|SpawnItems|GetIsSpawning?))
      (CallFunction|SpawnItems))))

(event Custom|SpawnItems
  (bind _itemstospawn (CallFunction|GetItemstoSpawn))
  (for _array_element _itemstospawn
    (for _index (range 0 (- (.NumOfItems (Utilities|Struct|BreakF_SpawnItemInfo _array_element)) 1))
      (Utilities|Array|Add (Variables|SpawnItems|GetCurrentClassesToSpawn) (.Item (Utilities|Struct|BreakF_SpawnItemInfo _array_element))))
    (Variables|SpawnItems|SetIsSpawning? true)
    (Variables|SpawnItems|SetAllSpawned? false)
    (CallFunction|SpawnOneItem)))

(event Custom|SpawnOneItem
  (bind _pointtospawn (CallFunction|GetSpawnPointtoSpawn))
  (Utilities|IsValid _pointtospawn
    (:Is%20Valid
      (bind _returnvalue (Game|SpawnActorfromClass (Utilities|Array|Get(acopy) (Variables|SpawnItems|GetCurrentClassesToSpawn) (Variables|SpawnItems|GetCurrentItemSpawnIndex)) (Math|Transform|MakeTransform (.location (Transformation|GetWorldTransform (Variables|/Script/Engine.Actor|GetRootComponent _pointtospawn))) (.rotation (Transformation|GetWorldTransform (Variables|/Script/Engine.Actor|GetRootComponent _pointtospawn)))) "Undefined" 0 0))
      (Variables|/Game/Game/Blueprints/BP_SpawnItemPoint.BP_SpawnItemPoint_C|SetItemSpawned _pointtospawn _returnvalue)
      (Variables|SpawnItems|SetCurrentItemSpawnIndex (Math|Integer|Clamp(Integer) (+ (Variables|SpawnItems|GetCurrentItemSpawnIndex) 1) 0 (Utilities|Array|Length (Variables|SpawnItems|GetCurrentClassesToSpawn)))))
    (:Is%20Not%20Valid
      _))
  (Utilities|FlowControl|Delay 1.0)
  (if (< (Variables|SpawnItems|GetCurrentItemSpawnIndex) (Utilities|Array|Length (Variables|SpawnItems|GetCurrentClassesToSpawn)))
    (CallFunction|SpawnOneItem)
    (else
      (Variables|SpawnItems|SetIsSpawning? false)
      (Variables|SpawnItems|SetAllSpawned? true))))

(event EventBeginPlay
  (bind _returnvalue (Actor|GetActorOfClass "/Game/Game/Blueprints/Gameplay/BP_GameplayManager.BP_GameplayManager_C"))
  (Variables|Default|SetGameplayManager _returnvalue)
  (bind _outactors (Actor|GetAllActorsOfClass "/Game/Game/Blueprints/BP_SpawnItemPoint.BP_SpawnItemPoint_C"))
  (Variables|SpawnItems|SetSpawnPoints _outactors))

(fn ConstructionScript)

(fn GetItemstoSpawn
  (bind _spawnitem_datatable (Variables|SpawnItems|GetSpawnItem%20Datatable))
  (bind _gameplaymanager (Variables|Default|GetGameplayManager))
  (bind _outrownames (DataTable|GetDataTableRowNames _spawnitem_datatable))
  (for _array_element _outrownames
    (bind _returnvalue (Utilities|GetDataTableRow _spawnitem_datatable _array_element)
      (:then
        (if (and (Utilities|Enum|Equal(Enum) (.ScenaryType (Utilities|Struct|BreakF_SpawnItemsByObjective _returnvalue)) (Variables|/Game/Game/Blueprints/Gameplay/BP_GameplayManager.BP_GameplayManager_C|GetScenaryType _gameplaymanager)) (Utilities|Enum|Equal(Enum) (.ObjectiveType (Utilities|Struct|BreakF_SpawnItemsByObjective _returnvalue)) (Variables|/Game/Game/Blueprints/Gameplay/BP_GameplayManager.BP_GameplayManager_C|GetCurrentObjectiveType _gameplaymanager)))
          (return (.ItemsToSpawn (Utilities|Struct|BreakF_SpawnItemsByObjective _returnvalue)))))))
  (return 0))

(fn GetSpawnPointtoSpawn
  (for _array_element (Variables|SpawnItems|GetSpawnPoints)
    (bind _occupied (Default|IsOccupied? _array_element))
    (if (not _occupied)
      (return _array_element)))
  (return 0))