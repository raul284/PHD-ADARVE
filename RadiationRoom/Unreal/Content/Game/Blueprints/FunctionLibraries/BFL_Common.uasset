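; BFL_Common is a Blueprint function library of global getters for the game's core objects.
; It casts the game instance and game mode to their RR_ classes, returning nothing further if a cast fails.
; The player, database manager and gameplay manager are read from RR_GameInstance, and the tutorial manager is reached through the gameplay manager.
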(fn GetMyGameInstance
  (bind _asrr_game_instance (Utilities|Casting|CastToRR_GameInstance (Game|GetGameInstance)))
  (return _asrr_game_instance))

(fn GetMyPlayer
  (return (Variables|/Game/Game/Blueprints/RR_GameInstance.RR_GameInstance_C|GetCurrentPlayer (CallFunction|GetMyGameInstance))))

(fn GetMyGameMode
  (bind _asrr_game_mode (Utilities|Casting|CastToRR_GameMode (Game|GetGameMode)))
  (return _asrr_game_mode))

(fn GetMyDatabase
  (return (Variables|/Game/Game/Blueprints/RR_GameInstance.RR_GameInstance_C|GetDatabase%20Manager (CallFunction|GetMyGameInstance))))

(fn GetMyGameplayManager
  (return (Variables|/Game/Game/Blueprints/RR_GameInstance.RR_GameInstance_C|GetGameplayManager (CallFunction|GetMyGameInstance))))

(fn GetMyTutorialManager
  (return (Variables|/Game/Game/Blueprints/Gameplay/BP_GameplayManager.BP_GameplayManager_C|GetTutorialManager (CallFunction|GetMyGameplayManager))))