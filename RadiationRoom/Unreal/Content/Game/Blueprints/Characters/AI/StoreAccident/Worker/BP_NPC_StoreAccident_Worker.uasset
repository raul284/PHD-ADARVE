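; Worker NPC character for the store accident scenario, which can carry radiation and be sent to exam and radiation points.
; On BeginPlay it picks a random skeletal mesh and, by a coin flip, may set its radiation component's absorbed dose to a random value within a default range.
; GoToExamPoint and RadiationMeasured events forward destinations and the measured radioactive result to its Controller_NPC_StoreAccident_Worker AI controller, which handles movement.
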(event Custom|SetInitialRadiation
  (if (!= (Math|Random|RandomInteger 2) 0)
    (Variables|/Game/Game/Blueprints/Components/AC_Radiation.AC_Radiation_C|SetDoseAbsorption (Variables|Default|GetAC_Radiation) (Math|Random|RandomFloatinRange (Variables|RadiationData|GetDefaultRadiationMin) (Variables|RadiationData|GetDefaultRadiationMax)))))

(event Custom|GoToExamPoint
  (params (DestinyPoint :type Actor%20Object%20Reference))
  (bind _asradiactive_npc_controller (Utilities|Casting|CastToController_NPC_StoreAccident_Worker (AI|GetAIController self)))
  (Default|GotoExamPoint _asradiactive_npc_controller DestinyPoint))

(event Custom|SetRandomMesh
  (bind _charactermeshes (Variables|Default|GetCharacterMeshes))
  (Class|SkinnedMeshComponent|SetSkeletalMesh (Variables|Character|GetMesh) (Utilities|Array|Get(acopy) _charactermeshes (Math|Random|RandomInteger (Utilities|Array|Length _charactermeshes))) true))

(event Custom|RadiationMeasured
  (params (Is%20Radiactive? :type Boolean) (DestinationPoint :type Actor%20Object%20Reference))
  (bind _asradiactive_npc_controller (Utilities|Casting|CastToController_NPC_StoreAccident_Worker (AI|GetAIController self)))
  (Default|MovetoRadiactivePoint _asradiactive_npc_controller Is%20Radiactive? DestinationPoint))

(event EventBeginPlay
  (|CallParentFunction)
  (CallFunction|SetRandomMesh)
  (CallFunction|SetInitialRadiation))

(event EventTick
  (params (DeltaSeconds :type Float%20%28single-precision%29))
  (|CallParentFunction DeltaSeconds))

(fn ConstructionScript
  (|CallParentFunction))