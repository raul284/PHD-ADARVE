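; Gameplay manager for scenario S2, a VR training scenario covering traffic control, witness and driver handling, radiation measurement and radio reports to the office.
; It binds events from the player destination point, RBQ van, spawned walkie-talkies and SABG100 dosimeters, cone placement and NPCs to complete gameplay steps.
; Tutorial buddy dialog completions and delayed TutorialManager calls drive the guided sequence from introduction through free play to final conversation and data save.
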(event EventBeginPlay
  (|CallParentFunction)
  (Utilities|FlowControl|Sequence
    (:then_0
      (CallFunction|BindItemActions)
      (CallFunction|BindNPCActions)
      (Collision|SetActorEnableCollision (Variables|Default|GetTrafficWall) false))
    (:then_1
      (bind _rbqdestinationpoint (Variables|Default|GetRBQDestinationPoint)
        (:then
          (Default|SetActive _rbqdestinationpoint false))
        (:else
          (Default|Log (Variables|Default|GetGameInstance) "NewEnumerator2" "Falta el RBQ Destination Point" false))))
    (:then_2
      (bind _tutorialmanager (Variables|Default|GetTutorialManager)
        (:then
          (Variables|/Game/Game/Blueprints/Tutorial/BP_TutorialManager.BP_TutorialManager_C|SetPlayerCanDemandTuddy _tutorialmanager false))
        (:else
          (Default|Log (Variables|Default|GetGameInstance) "NewEnumerator2" "Falta el TutorialManager" false))))))

(event EventAddItemtoGameManagerImportantList
  (params (ItemType :type E_ItemType%20Enum :default "NewEnumerator2") (Actor :type Actor%20Object%20Reference))
  (switch Utilities|FlowControl|Switch|SwitchonE_ItemType ItemType
    (:NewEnumerator1
      (bind _asbp_dosimeter_sabg100 (Utilities|Casting|CastToBP_Dosimeter_SABG100 Actor))
      (CallFunction|BindSAGB100Actions _asbp_dosimeter_sabg100)
      (Utilities|Array|Add (Variables|Dosimeters|GetSABG100List) _asbp_dosimeter_sabg100))
    (:NewEnumerator3
      (Utilities|Casting|CastToBP_Dosimeter_EPD Actor))
    (:NewEnumerator5
      (bind _asbp_walkie_talkie (Utilities|Casting|CastToBP_WalkieTalkie Actor))
      (Default|SetInitialConditions _asbp_walkie_talkie (Variables|WalkieReports|GetInitialReportCompleted) (Variables|WalkieReports|GetFinalReportCompleted))
      (CallFunction|BindWalkieTalkieEvents _asbp_walkie_talkie)
      (Utilities|Array|Add (Variables|WalkieReports|GetWalkieTalkieList) _asbp_walkie_talkie))))

(event EventSetPlayerData
  (|CallParentFunction)
  (CallFunction|BindPlayerActions)
  (Utilities|FlowControl|Sequence
    (:then_0
      (bind _asbp_player_vr (Utilities|Casting|CastToBP_Player_VR (Variables|Default|GetPlayer)))
      (bind _output_get (Variables|Tutorial|SetTutorialBuddy (Variables|/Game/Game/Blueprints/Characters/Players/BP_Player_VR.BP_Player_VR_C|GetTutorialBuddyActor _asbp_player_vr)))
      (bind _tutorialmanager (Variables|Default|GetTutorialManager)
        (:then
          (Default|SetCurrentTutorialBuddy _tutorialmanager _output_get)
          (CallFunction|BindTuddyActions))
        (:else
          (Default|Log (Variables|Default|GetGameInstance) "NewEnumerator2" "Falta el TutorialManager" false))))
    (:then_1
      (CallFunction|StartScenario)
      (CallFunction|CompleteStep "NewEnumerator9"))))

(event EventStartScenario
  (|CallParentFunction)
  (Utilities|FlowControl|Delay 3.0)
  (CallFunction|SetCurrentGameplayStep "NewEnumerator50")
  (Default|StartExtraLinesDialog (Variables|Default|GetTutorialManager) "NewEnumerator5"))

(event Custom|OnPlayerExitOfRQBDestinationPoint
  (Variables|Default|SetPlayerInRBQDestinationPoint false))

(event Custom|PlayerOnDestinationPoint
  (if (Variables|Default|GetPlayerInRBQDestinationPoint)
    (bind _yes (CallFunction|IsCurrentStep "NewEnumerator51"))
    (if _yes
      (CallFunction|CompleteStep "NewEnumerator51")
      (Default|SetActive (Variables|Default|GetRBQDestinationPoint) false)
      (Utilities|FlowControl|Delay 0.5)
      (CallFunction|SetCurrentGameplayStep "NewEnumerator52")
      (Default|StartExtraLinesDialog (Variables|Default|GetTutorialManager) "NewEnumerator7"))))

(event Custom|OnPlayerEnterOnRQBDestinationPoint
  (Variables|Default|SetPlayerInRBQDestinationPoint true)
  (bind _yes (CallFunction|IsCurrentStep "NewEnumerator51"))
  (if _yes
    (CallFunction|CompleteStep "NewEnumerator51")
    (Default|SetActive (Variables|Default|GetRBQDestinationPoint) false)
    (Utilities|FlowControl|Delay 0.5)
    (CallFunction|SetCurrentGameplayStep "NewEnumerator52")
    (Default|StartExtraLinesDialog (Variables|Default|GetTutorialManager) "NewEnumerator7")))

(event EventBindPlayerActions
  (|CallParentFunction)
  (bind _rbqdestinationpoint (Variables|Default|GetRBQDestinationPoint)
    (:then
      (EventDispatchers|BindEventtoEDPlayerEnteronDestinationPoint _rbqdestinationpoint (delegate Custom|OnPlayerEnterOnRQBDestinationPoint))
      (EventDispatchers|AssignEDPlayerExitOfDestinationPoint _rbqdestinationpoint (delegate Custom|OnPlayerExitOfRQBDestinationPoint)))
    (:else
      (Default|Log (Variables|Default|GetGameInstance) "NewEnumerator2" "Falta RBQ Destination Point" false))))

(event Custom|OnDescriptionCompleted
  (bind _yes (CallFunction|IsCurrentStep "NewEnumerator50"))
  (if _yes
    (CallFunction|CompleteStep "NewEnumerator50")
    (CallFunction|SetCurrentGameplayStep "NewEnumerator51")
    (Utilities|FlowControl|Delay 2.0)
    (Default|StartExtraLinesDialog (Variables|Default|GetTutorialManager) "NewEnumerator6")
    (Default|SetActive (Variables|Default|GetRBQDestinationPoint) true)
    (Utilities|FlowControl|Delay 1.0)
    (CallFunction|PlayeronDestinationPoint)))

(event Custom|BindWalkieTalkieEvents
  (params (WalkieTalkie :type BP%20Walkie%20Talkie%20Object%20Reference))
  (EventDispatchers|BindEventtoEDInteractionStarted WalkieTalkie (delegate Custom|OnWalkieGrabbed))
  (EventDispatchers|BindEventtoEDInitialReportCompleted WalkieTalkie (delegate Custom|OnWalkieInitialReportCompleted))
  (EventDispatchers|BindEventtoEDFinalReportCompleted WalkieTalkie (delegate Custom|OnWalkieFinalReportCompleted)))

(event Custom|BindSAGB100Actions
  (params (SABG100 :type BP%20Dosimeter%20SABG100%20Object%20Reference))
  (EventDispatchers|AssignEDItemRadiationMeasured SABG100 (delegate Custom|OnSABG100ItemRadiationMeasured))
  (EventDispatchers|AssignEDNPCRadiationMeasured SABG100 (delegate Custom|ONSABG100NPCRadiationMeasured)))

(event Custom|BindEPDActions
  (params (EPD :type BP%20Dosimeter%20EPD%20Object%20Reference)))

(event Custom|OnSABG100ItemRadiationMeasured
  (params (Actor :type BP%20Interact%20Item%20Parent%20Object%20Reference))
  (if (== Actor (Variables|Dosimeters|GetRadiactiveItem))
    (CallFunction|CompleteStep "NewEnumerator5")))

(event Custom|ONSABG100NPCRadiationMeasured
  (params (Actor :type BP%20NPC%20Object%20Reference))
  (Utilities|Casting|CastToBP_NPC_S2_Driver Actor)
  (CallFunction|CompleteStep "NewEnumerator4"))

(event Custom|OnRBQItemSpawned
  (params (Actor :type BP%20Item%20Initial%20State%20Object%20Reference))
  (switch Utilities|FlowControl|Switch|SwitchonE_ItemType (Variables|/Game/Game/Blueprints/Actors/Items/BP_ItemInitialState.BP_ItemInitialState_C|GetItemType Actor)
    (:NewEnumerator5
      (Variables|WalkieReports|SetWalkieSpawned true)
      (CallFunction|OnWalkieIsSpawned))))

(event Custom|OnWalkieInitialReportCompleted
  (bind _yes (CallFunction|IsCurrentStep "NewEnumerator49"))
  (Variables|WalkieReports|SetInitialReportCompleted _yes)
  (for _array_element (Variables|WalkieReports|GetWalkieTalkieList)
    (Default|SetInitialConditions _array_element (Variables|WalkieReports|GetInitialReportCompleted) (Variables|WalkieReports|GetFinalReportCompleted)))
  (CallFunction|CompleteStep "NewEnumerator49")
  (Utilities|FlowControl|Delay 1.0)
  (CallFunction|SetCurrentGameplayStep "NewEnumerator55")
  (Default|StartExtraLinesDialog (Variables|Default|GetTutorialManager) "NewEnumerator9"))

(event Custom|OnWalkieFinalReportCompleted
  (Variables|WalkieReports|SetFinalReportCompleted true)
  (for _array_element (Variables|WalkieReports|GetWalkieTalkieList)
    (Default|SetInitialConditions _array_element (Variables|WalkieReports|GetInitialReportCompleted) (Variables|WalkieReports|GetFinalReportCompleted))
    (CallFunction|CompleteStep "NewEnumerator6")
    (Utilities|FlowControl|Delay 1.0)
    (CallFunction|SetCurrentGameplayStep "NewEnumerator54")
    (Default|StartExtraLinesDialog (Variables|Default|GetTutorialManager) "NewEnumerator11")))

(event Custom|BindRBQVanEvents
  (bind _rbqvan (Variables|Default|GetRBQVan)
    (:then
      (EventDispatchers|BindEventtoEDItemSpawned _rbqvan (delegate Custom|OnRBQItemSpawned)))
    (:else
      (Default|Log (Variables|Default|GetGameInstance) "NewEnumerator2" "Falta RBQ Van" false))))

(event Custom|BindDescriptionPanelEvents
  (bind _descriptionpanel (Variables|Default|GetDescriptionPanel)
    (:then
      (EventDispatchers|BindEventtoEDDescriptionCompleted _descriptionpanel (delegate Custom|OnDescriptionCompleted)))
    (:else
      (Default|Log (Variables|Default|GetGameInstance) "NewEnumerator2" "Falta el DescriptionPanel" false))))

(event Custom|OnWalkieIsSpawned
  (if (Variables|WalkieReports|GetWalkieSpawned)
    (bind _yes (CallFunction|IsCurrentStep "NewEnumerator52"))
    (if _yes
      (CallFunction|CompleteStep "NewEnumerator52")
      (Default|HideAutomaticHintPanel (Variables|Default|GetTutorialManager))
      (Utilities|FlowControl|Delay 1.0)
      (CallFunction|SetCurrentGameplayStep "NewEnumerator49")
      (Default|ShowCurrentTuddy (Variables|Default|GetTutorialManager))
      (Default|AutomaticCall (Variables|Default|GetTutorialManager) "NewEnumerator17"))))

(event Custom|OnWalkieGrabbed
  (bind _yes (CallFunction|IsCurrentStep "NewEnumerator49"))
  (if _yes
    (Default|HideAutomaticHintPanel (Variables|Default|GetTutorialManager))
    (Default|HideCurrentTuddy (Variables|Default|GetTutorialManager))))

(event Custom|OnOneTrafficConeHasBeenPlaced
  (params (Item :type BP%20Pickable%20Item%20Object%20Reference) (PlacePoint :type BP%20Place%20Point%20Object%20Reference))
  (CallFunction|CompleteStep "NewEnumerator3")
  (Collision|SetActorEnableCollision (Variables|Default|GetTrafficWall) true))

(event EventBindItemActions
  (|CallParentFunction)
  (CallFunction|BindDescriptionPanelEvents)
  (CallFunction|BindRBQVanEvents)
  (CallFunction|BindPlacePointsActions))

(event EventBindPlacePointsActions
  (|CallParentFunction)
  (bind _trafficconeplacepointmanager (Variables|Default|GetTrafficConePlacePointManager)
    (:then
      (EventDispatchers|AssignEDOneItemHasBeenPlaced _trafficconeplacepointmanager (delegate Custom|OnOneTrafficConeHasBeenPlaced)))
    (:else
      (Default|Log (Variables|Default|GetGameInstance) "NewEnumerator2" "Falta el PlacePointManager de los \"conos de tráfico\"" false))))

(event Custom|BindNPCWitnessActions
  (bind _npc_witness (Variables|NPCs|GetNPC%20Witness)
    (:then
      (EventDispatchers|BindEventtoEDConversationFinished _npc_witness (delegate Custom|OnNPCWitnessConversationFinished)))
    (:else
      (Default|Log (Variables|Default|GetGameInstance) "NewEnumerator2" "Falta NPC Witness" false))))

(event Custom|BindNPCDriverActions
  (bind _npc_driver (Variables|NPCs|GetNPC%20Driver)
    (:then
      (EventDispatchers|BindEventtoEDConversationFinished _npc_driver (delegate Custom|OnNPCDriverConversationFinished))
      (EventDispatchers|BindEventtoEDNPCProtected _npc_driver (delegate Custom|OnNPCDriverProtected)))
    (:else
      (Default|Log (Variables|Default|GetGameInstance) "NewEnumerator2" "Falta NPC Driver" false))))

(event Custom|OnNPCWitnessConversationFinished
  (params (ConversationNumber :type Integer))
  (switch int ConversationNumber
    (:0
      (CallFunction|CompleteStep "NewEnumerator0"))))

(event Custom|OnNPCDriverConversationFinished
  (params (ConversationNumber :type Integer))
  (switch int ConversationNumber
    (:1
      (CallFunction|CompleteStep "NewEnumerator2"))))

(event Custom|OnNPCDriverProtected
  (CallFunction|CompleteStep "NewEnumerator1"))

(event EventBindNPCActions
  (|CallParentFunction)
  (CallFunction|BindNPCWitnessActions)
  (CallFunction|BindNPCDriverActions))

(event Custom|OnRBQVanExplained
  (bind _yes (CallFunction|IsCurrentStep "NewEnumerator52"))
  (if _yes
    (Default|AutomaticCall (Variables|Default|GetTutorialManager) "NewEnumerator16")
    (CallFunction|OnWalkieIsSpawned)))

(event Custom|OnTuddyIntroductionCompleted
  (Default|StartDescription (Variables|Default|GetDescriptionPanel)))

(event Custom|OnHelpPanelExtraLines
  (bind _yes (CallFunction|IsCurrentStep "NewEnumerator55"))
  (if _yes
    (Default|AutomaticCall (Variables|Default|GetTutorialManager) "NewEnumerator10")
    (Variables|/Game/Game/Blueprints/Tutorial/BP_TutorialManager.BP_TutorialManager_C|SetPlayerCanDemandTuddy (Variables|Default|GetTutorialManager) true)))

(event Custom|BindTutorialManagerActions
  (EventDispatchers|BindEventtoEDTutorialDemanded (Variables|Default|GetTutorialManager) (delegate Custom|OnTutorialDemanded)))

(event Custom|OnTutorialDemanded
  (bind _yes (CallFunction|IsCurrentStep "NewEnumerator55"))
  (if _yes
    (bind _result (Math|Integer|IncrementInt (Variables|Tutorial|GetTutorialDemandedTimes))
      (:%20%20
        (bind _output_get (Variables|Tutorial|SetTutorialDemandedTimes _result))
        (if (>= _output_get 3)
          (Variables|/Game/Game/Blueprints/Tutorial/BP_TutorialManager.BP_TutorialManager_C|SetPlayerCanDemandTuddy (Variables|Default|GetTutorialManager) false)
          (CallFunction|CompleteStep "NewEnumerator55")
          (Utilities|FlowControl|Delay 0.5)
          (CallFunction|SetCurrentGameplayStep "NewEnumerator53")
          (Default|StartExtraLinesDialog (Variables|Default|GetTutorialManager) "NewEnumerator10"))))))

(event Custom|OnTuddyFreedomCompleted
  (bind _yes (CallFunction|IsCurrentStep "NewEnumerator53"))
  (if _yes
    (CallFunction|CompleteStep "NewEnumerator53")
    (Variables|/Game/Game/Blueprints/Tutorial/BP_TutorialManager.BP_TutorialManager_C|SetPlayerCanDemandTuddy (Variables|Default|GetTutorialManager) true)
    (Default|HideCurrentTuddy (Variables|Default|GetTutorialManager))))

(event Custom|OnFinalConversationCompleted
  (bind _yes (CallFunction|IsCurrentStep "NewEnumerator54"))
  (if _yes
    (CallFunction|CompleteStep "NewEnumerator54")
    (CallFunction|CompleteStep "NewEnumerator7")
    (Default|SaveData (Variables|Default|GetTutorialManager))))

(event Custom|OnTuddyDialogCompleted
  (params (CurrentTuddyDialogType :type E_TuddyDialogLinesType%20Enum :default "NewEnumerator0") (CurrentExtraLineType :type E_TuddyExtraLineTypes%20Enum :default "NewEnumerator1"))
  (switch Utilities|FlowControl|Switch|SwitchonE_GameplayStepTypes (Variables|Default|GetCurrentStepType)
    (:NewEnumerator50
      (CallFunction|OnTuddyIntroductionCompleted))
    (:NewEnumerator52
      (CallFunction|OnRBQVanExplained))
    (:NewEnumerator55
      (CallFunction|OnHelpPanelExtraLines))
    (:NewEnumerator53
      (CallFunction|OnTuddyFreedomCompleted))
    (:NewEnumerator54
      (CallFunction|OnFinalConversationCompleted))))

(event EventBindTuddyActions
  (|CallParentFunction)
  (EventDispatchers|BindEventtoEDDialogCompleted (Variables|/Game/Game/Blueprints/Tutorial/BP_TutorialBuddy.BP_TutorialBuddy_C|GetAC_TuddyDialogManager (Variables|/Game/Game/Blueprints/Tutorial/BP_TutorialManager.BP_TutorialManager_C|GetCurrentTutorialBuddy (Variables|Default|GetTutorialManager))) (delegate Custom|OnTuddyDialogCompleted))
  (CallFunction|BindTutorialManagerActions))

(fn ConstructionScript
  (|CallParentFunction))