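; BP_ExplainBillboard is a billboard actor that displays a text message and turns to face the player.
; On BeginPlay it applies its Text variable to the TextRender and caches the BP_Player actor.
; Each Tick, LookAtPlayer rotates the Billboard component toward the player's mesh using the look-at yaw and roll, keeping its current pitch so it does not tilt up or down.
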(event Custom|LookAtPlayer
  (bind _billboard (Variables|Default|GetBillboard))
  (bind _player (Variables|Default|GetPlayer))
  (bind _returnvalue (Transformation|GetWorldLocation _billboard))
  (bind _mesh (Variables|/Script/Engine.Character|GetMesh _player))
  (bind _returnvalue_2 (Transformation|GetWorldLocation _mesh))
  (bind _returnvalue_3 (Math|Rotator|FindLookatRotation _returnvalue _returnvalue_2))
  (Variables|Default|GetPlayer
    (:then
      (Transformation|SetWorldRotation (Variables|Default|GetBillboard) (Math|Rotator|MakeRotator (.roll _returnvalue_3) (.pitch (Transformation|GetWorldRotation _billboard)) (.yaw _returnvalue_3)) false false))
    (:else)))

(event EventBeginPlay
  (Rendering|Components|TextRender|SetText (Variables|Default|GetTextRender) (Variables|Default|GetText))
  (bind _returnvalue (Actor|GetActorOfClass "/Game/Game/Blueprints/Characters/Players/BP_Player.BP_Player_C"))
  (Variables|Default|SetPlayer _returnvalue))

(event Collision|EventActorBeginOverlap
  (params (OtherActor :type Actor%20Object%20Reference)))

(event EventTick
  (params (DeltaSeconds :type Float%20%28single-precision%29))
  (CallFunction|LookatPlayer))

(fn ConstructionScript)