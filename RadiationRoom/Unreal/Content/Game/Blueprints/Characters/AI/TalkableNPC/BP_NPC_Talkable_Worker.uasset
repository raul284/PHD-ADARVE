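; Talkable worker NPC Blueprint that ties its conversation to game phase progression.
; On interaction it stores the player, then runs the parent interaction only if GameplayManager reports its hard-coded phase as current or pre-phase.
; When the conversation stops, it calls the parent logic and completes that same phase through GameplayManager.
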(event EventBeginPlay
  (|CallParentFunction) ; This node is disabled and will not be called.\nDrag off pins to build functionality.
)

(event EventStopConversation
  (|CallParentFunction)
  (Default|CompletePhase (Variables|Default|GetGameplayManager) "NewEnumerator0"))

(event EventInteractwith
  (params (Player :type BP%20Player%20Object%20Reference))
  (Utilities|FlowControl|Sequence
    (:then_0
      (Variables|Default|SetPlayer Player))
    (:then_1
      (bind _currentorprephase (Default|CheckCurrentorPrePhase (Variables|Default|GetGameplayManager) "NewEnumerator0"))
      (if _currentorprephase
        (|CallParentFunction Player)))))

(fn ConstructionScript
  (|CallParentFunction))