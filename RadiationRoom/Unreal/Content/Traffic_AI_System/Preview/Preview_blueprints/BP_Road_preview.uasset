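; Preview-only road Blueprint that builds a road from spline meshes along an editable spline.
; The construction script optionally line-traces spline points onto WorldStatic ground with slight random height jitter, then adds fixed-length segments with clamped tangents, a material and width scaling.
; The Applyspline event deforms the first landscape found in the level along the spline, using a scaled width and wide side falloff.
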(event Custom|Apply%20spline
  (bind _scale (Variables|Default|GetScale))
  (bind _returnvalue (* _scale 1.5e+02))
  ;[1 0.1402 0] Deform landscape - this blueprint is made only for preview
  (bind _outactors (Actor|GetAllActorsOfClass "/Script/Landscape.LandscapeProxy"))
  (Landscape|Editor|EditorApplySpline (Utilities|Array|Get(acopy) _outactors) (Variables|Default|GetSpline) _returnvalue _returnvalue 1.5e+03 1.5e+03 0.0 0.0 (Math|Float|Truncate (/ (Spline|GetSplineLength (Variables|Default|GetSpline)) 1e+02)) true true 0 "None"))

(fn ConstructionScript
  (bind _segment_length (Variables|Default|GetSegment%20Length))
  (bind _spline (Variables|Default|GetSpline))
  (bind _spline_2 (Variables|Default|GetSpline))
  ;[1 0.4219 0.4219] Line trace to stick road to the ground
  (for _index (range 0 (Spline|GetNumberOfSplinePoints (Variables|Default|GetSpline)))
    (if (Variables|Default|GetStick%20to%20ground?)
      (bind (_outhit _returnvalue) (Collision|LineTraceForObjects (+ (Spline|GetLocationatSplinePoint (Variables|Default|GetSpline) _index "World") "0.000000, 0,1000.000000") (- (Spline|GetLocationatSplinePoint (Variables|Default|GetSpline) _index "World") "0, 0,5000.000000") (Utilities|Array|MakeArray "ObjectTypeQuery1") false 0 "None"))
      (if _returnvalue
        (Spline|SetLocationatSplinePoint (Variables|Default|GetSpline) _index (+ (.ImpactPoint (Collision|BreakHitResult _outhit)) (Math|Vector|MakeVector 0.0 0.0 (Math|Random|RandomFloatinRange -2.0 2.0))) "World" true))))
  ;[1 0.7061 0.2479] Set spline mesh locations and scale
  (for _index_2 (range 0 (Math|Float|Floor (/ (Spline|GetSplineLength (Variables|Default|GetSpline)) (Variables|Default|GetSegment%20Length))))
    (bind _returnvalue_2 (AddComponent|AddSplineMeshComponent false (Math|Transform|MakeTransform (Variables|Default|GetRelative%20Transform%20Location) "0, 0, 0" "1,1,1")))
    (Rendering|Material|SetMaterial _returnvalue_2 0 (Variables|Default|GetMaterial))
    (SplineMesh|SetStartandEnd _returnvalue_2 (Spline|GetLocationatDistanceAlongSpline _spline_2 (* _index_2 (Variables|Default|GetSegment%20Length)) "Local") (Math|Vector|ClampVectorSize (Spline|GetTangentatDistanceAlongSpline _spline_2 (* _index_2 (Variables|Default|GetSegment%20Length)) "Local") 0.0 (Variables|Default|GetSegment%20Length)) (Spline|GetLocationatDistanceAlongSpline _spline (* (+ _index_2 1) _segment_length) "Local") (Math|Vector|ClampVectorSize (Spline|GetTangentatDistanceAlongSpline _spline (* (+ _index_2 1) _segment_length) "Local") 0.0 (Variables|Default|GetSegment%20Length)) true :!class /Script/Engine.SplineMeshComponent)
    (SplineMesh|SetStartScale _returnvalue_2 (Math|Vector2D|MakeVector2D (* (.y (Class|SplineComponent|GetScaleatDistanceAlongSpline _spline_2 (* _index_2 (Variables|Default|GetSegment%20Length)))) (Variables|Default|GetScale)) 1.0) true :!class /Script/Engine.SplineMeshComponent)
    (SplineMesh|SetEndScale _returnvalue_2 (Math|Vector2D|MakeVector2D (* (.y (Class|SplineComponent|GetScaleatDistanceAlongSpline _spline _segment_length)) (Variables|Default|GetScale)) 1.0) true :!class /Script/Engine.SplineMeshComponent)
    (Class|SplineMeshComponent|SetEndRoll _returnvalue_2 0.0 true)
    (Class|SplineMeshComponent|SetStartRoll _returnvalue_2 0.0 true)))