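; BP_NPC_StoreAccident_Mate is the Mate NPC character for the StoreAccident scenario.
; Its StartFollowPlayer event first stops the current conversation and advances to the next one, but only while the dialog manager is on conversation index zero.
; It then hands the player to its Controller_NPC_StoreAccident_Mate AI controller, which is told to start following.
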(event Custom|StartFollowPlayer
  (params (Player :type BP%20Player%20Object%20Reference))
  (bind _ac_dialogmanager (Variables|Default|GetAC_DialogManager))
  (Utilities|FlowControl|Sequence
    (:then_0
      (if (== (Variables|/Game/Game/Blueprints/Components/AC_DialogManager.AC_DialogManager_C|GetConversationIndex (Variables|Default|GetAC_DialogManager)) 0)
        (Default|StopConversation _ac_dialogmanager)
        (Default|NextConversation _ac_dialogmanager)))
    (:then_1
      (bind _ascontroller_npc_store_accident_mate (Utilities|Casting|CastToController_NPC_StoreAccident_Mate (AI|GetAIController self)))
      (Default|StartFollowPlayer _ascontroller_npc_store_accident_mate Player))))

(event EventBeginPlay
  (|CallParentFunction))

(fn ConstructionScript
  (|CallParentFunction))