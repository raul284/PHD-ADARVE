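; Car accident driver NPC that the player talks to and that walks to a safe point as part of the objectives.
; Interaction reaches the parent class only when the driver is not walking and one of two objectives is current or preceding.
; Finished conversations complete objectives, and the first also sets the sit-to-stand and walking flags.
; StartWalking delegates movement to the AI controller; StopWalking faces the player, advances dialogue and marks the driver protected.
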(event Custom|StartWalking
  (bind _ascontroller_npc_car_accident_driver (Utilities|Casting|CastToController_NPC_CarAccident_Driver (AI|GetAIController self)))
  (Default|GotoSafePoint _ascontroller_npc_car_accident_driver (Variables|Default|GetDestinationPoint)))

(event Custom|StopWalking
  (Variables|Default|SetWalking false)
  (Variables|Animation|SetWalkToIdle true)
  (CallFunction|LookatPlayer)
  (Variables|Default|SetCanLookPlayer true)
  (Default|NextConversation (Variables|Default|GetAC_DialogManager))
  (Variables|Default|SetProtected true))

(event EventStopLookat
  (params (Player :type BP%20Player%20Object%20Reference))
  ;[1 1 1] Look at
  (|CallParentFunction Player))

(event EventTick
  (params (DeltaSeconds :type Float%20%28single-precision%29))
  (|CallParentFunction DeltaSeconds))

(event EventInteractwith
  (params (Player :type BP%20Player%20Object%20Reference))
  (bind _gameplaymanager (Variables|Default|GetGameplayManager))
  ;[1 1 1] Interact
  (Utilities|FlowControl|Sequence
    (:then_0
      (Variables|Default|SetPlayer Player))
    (:then_1
      (if (not (Variables|Default|GetWalking))
        (bind _currentorprephase (Default|CheckCurrentorPreObjective _gameplaymanager "NewEnumerator1"))
        (bind _currentorprephase_2 (Default|CheckCurrentorPreObjective _gameplaymanager "NewEnumerator2"))
        (if (or _currentorprephase_2 _currentorprephase)
          (|CallParentFunction Player))))))

(event EventStartLookat
  (params (Player :type BP%20Player%20Object%20Reference))
  ;[1 1 1] Look at
  (|CallParentFunction Player))

(event EventCancelInteract
  (params (Player :type BP%20Player%20Object%20Reference))
  ;[1 1 1] Interact
  (|CallParentFunction Player))

(event EventBeginPlay
  (|CallParentFunction) ; This node is disabled and will not be called.\nDrag off pins to build functionality.
)

(event EventConversationFinished
  (params (Conversation%20Number :type Integer))
  (bind _gameplaymanager (Variables|Default|GetGameplayManager))
  (|CallParentFunction Conversation%20Number)
  (switch int Conversation%20Number
    (:0
      (Utilities|FlowControl|Sequence
        (:then_0
          (if (not (Variables|Animation|GetSitToStand))
            (Variables|Animation|SetSitToStand true)
            (Variables|Default|SetWalking true)))
        (:then_1
          (Default|CompleteObjective _gameplaymanager "NewEnumerator1")
          (Default|NextConversation (Variables|Default|GetAC_DialogManager)))))
    (:1
      (Default|CompleteObjective _gameplaymanager "NewEnumerator2"))))

(fn ConstructionScript
  (|CallParentFunction))