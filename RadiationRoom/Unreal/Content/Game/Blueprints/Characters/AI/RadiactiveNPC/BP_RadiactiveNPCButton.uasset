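; An interactable button for the radioactive NPC sorting mechanic, reporting the player's verdict to the BP_RadiactiveNPCManager it finds at BeginPlay.
; Its direction setting makes it green (right, "go to heaven") or red (left, "go to hell"), and an outline mesh mirrors the button mesh.
; Interacting briefly depresses the mesh, plays that side's sound, then after a delay calls NPCRadiationMeasured with false for right, true for left.
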(event Custom|PushButton
  (Transformation|SetWorldLocation (Variables|Default|GetStaticMesh1) (- (Transformation|GetWorldLocation (Variables|Default|GetStaticMesh1)) "0, 0,1.500000") false false)
  (Utilities|FlowControl|Delay 0.2)
  (Transformation|SetWorldLocation (Variables|Default|GetStaticMesh1) (+ (Transformation|GetWorldLocation (Variables|Default|GetStaticMesh1)) "0, 0,1.500000") false false))

(event EventBeginPlay
  (bind _staticmesh1 (Variables|Default|GetStaticMesh1))
  (bind _outlinemesh (Variables|Default|GetOutlineMesh))
  (bind _staticmesh1_2 (Variables|Default|GetStaticMesh1))
  (|CallParentFunction)
  (bind _returnvalue (Actor|GetActorOfClass "/Game/Game/Blueprints/Characters/AI/RadiactiveNPC/BP_RadiactiveNPCManager.BP_RadiactiveNPCManager_C"))
  (Variables|Default|SetRadiactiveNPCManager _returnvalue)
  (Components|StaticMesh|SetStaticMesh _outlinemesh (Variables|/Script/Engine.StaticMeshComponent|GetStaticMesh _staticmesh1_2))
  (Transformation|SetWorldTransform _outlinemesh (Transformation|GetWorldTransform _staticmesh1_2) false false)
  (switch Utilities|FlowControl|Switch|SwitchonE_RadiactiveNPCDirection (Variables|Default|GetRadiactiveNPCDirection)
    (:NewEnumerator0
      (Rendering|Material|SetMaterial _staticmesh1 0 "/Game/Game/Materials/M_Green.M_Green"))
    (:NewEnumerator1
      (Rendering|Material|SetMaterial _staticmesh1 0 "/Game/Game/Materials/M_Red.M_Red"))))

(event Collision|EventActorBeginOverlap
  (params (OtherActor :type Actor%20Object%20Reference)))

(event EventTick
  (params (DeltaSeconds :type Float%20%28single-precision%29)))

(event EventInteractwith
  (params (Player :type BP%20Player%20Object%20Reference))
  (bind _returnvalue (Transformation|GetActorLocation))
  (bind _radiactivenpcmanager (Variables|Default|GetRadiactiveNPCManager))
  (|CallParentFunction Player)
  (CallFunction|PushButton)
  (switch Utilities|FlowControl|Switch|SwitchonE_RadiactiveNPCDirection (Variables|Default|GetRadiactiveNPCDirection)
    (:NewEnumerator0
      (Audio|PlaySoundatLocation "/Game/Game/Assets/Sounds/dialogs/player/go_to_heaven.go_to_heaven" _returnvalue "0, 0, 0" 1.0 1.0 0.0 0 0 0)
      (Utilities|FlowControl|Delay 1.0)
      (Default|NPCRadiationMeasured _radiactivenpcmanager false))
    (:NewEnumerator1
      (Audio|PlaySoundatLocation "/Game/Game/Assets/Sounds/dialogs/player/go_to_hell.go_to_hell" _returnvalue "0, 0, 0" 1.0 1.0 0.0 0 0 0)
      (Utilities|FlowControl|Delay 1.0)
      (Default|NPCRadiationMeasured _radiactivenpcmanager true))))

(fn ConstructionScript
  (|CallParentFunction))