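; Dialog manager component for talkable NPCs that loads conversations from a data table and runs them as player and NPC lines in a WBP_Dialog widget.
; Interacting starts or advances a conversation, and typewriter completion auto-advances it after a short delay.
; It also toggles NPC audio, turns the widget toward the player each tick and logs interactions through the player's DBManager.
; Per-line voice playback exists but is disconnected.
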(event Custom|OnTypewriterFinished
  (Utilities|FlowControl|Delay 1.0)
  (if (Variables|Default|GetIsTalking?)
    (bind _continue (CallFunction|NextDialog))
    (if _continue
      (CallFunction|ProcessDialog)
      (else
        (CallFunction|StopConversation)))))

(event Custom|ProcessDialog
  ;[1 1 1] Process Dialog
  (if (Variables|Default|GetIsTalking?)
    (bind _dialog (CallFunction|GetCurrentDialog))
    (Utilities|FlowControl|Delay (.TimetoPlay (Utilities|Struct|BreakF_DialogLine _dialog)))
    (switch Utilities|FlowControl|Switch|SwitchonE_DialogType (.Type (Utilities|Struct|BreakF_DialogLine _dialog))
      (:NewEnumerator2
        (Development|PrintString "Un diálogo que no tiene dueño :(" true true "(R=1.000000,G=0.000000,B=0.000000,A=1.000000)"))
      (:NewEnumerator0
        (CallFunction|CreatePlayerDialog))
      (:NewEnumerator1
        (CallFunction|CreateNPCDialog)))))

(event Custom|Interact%20With
  ;[1 1 1] Interact with
  (if (not (Variables|Default|GetIsTalking?))
    (CallFunction|StartConversation)
    (CallFunction|SendDialogEventtoDB "NewEnumerator10")
    (Default|CallEDConversationStarted (Variables|Default|GetOwner))
    (else
      (bind _continue (CallFunction|NextDialog))
      (if _continue
        (CallFunction|ContinueDialog)
        (else
          (CallFunction|StopConversation)))
      (CallFunction|SendDialogEventtoDB "NewEnumerator20"))))

(event Custom|SetTypewriterComponent
  (params (TypewriterComponent :type Typewriter%20Text%20Component%20Object%20Reference))
  (bind _output_get (Variables|Default|SetTypewriterComponent TypewriterComponent))
  (bind _output_get_2 (Variables|/Game/Game/Blueprints/UI/Dialogs/WBP_Dialog.WBP_Dialog_C|SetTypewriterComponent (Variables|Default|GetWidget) _output_get))
  (EventDispatchers|BindEventtoOnCompleted _output_get_2 (delegate Custom|OnTypewriterFinished)))

(event Custom|StartConversation
  ;[1 1 1] Conversation
  (bind _isempty (CallFunction|IsConversationEmpty))
  (if (and (not _isempty) (Variables|Default|GetCanStartConversation?))
    (Variables|Default|SetIsTalking? true)
    (Audio|Components|Audio|Play (Variables|/Game/Game/Blueprints/Characters/AI/BP_NPC.BP_NPC_C|GetAudio (Variables|Default|GetOwner)) 0.0)
    (Variables|Default|SetDialogIndex 0)
    (CallFunction|ProcessDialog)
    (if (Variables|Default|GetShowDialogPanel)
      (Development|SetHiddeninGame (Variables|/Game/Game/Blueprints/Characters/AI/BP_NPC_Talkable.BP_NPC_Talkable_C|GetDialogWidget (Variables|Default|GetOwner)) false false)
      (Default|ShowDialogBox (Variables|Default|GetWidget)))))

(event Custom|ContinueDialog
  ;[1 1 1] Process Dialog
  (CallFunction|ProcessDialog))

(event Custom|SendDialogEventToDB
  (params (Event%20Type :type E_InteractEventType%20Enum :default "NewEnumerator4"))
  (bind _owner (Variables|Default|GetOwner))
  (bind _player (Variables|/Game/Game/Blueprints/Characters/AI/BP_NPC.BP_NPC_C|GetPlayer _owner))
  ;[1 1 1] Database
  (bind _dbmanager (Variables|/Game/Game/Blueprints/Characters/Players/BP_Player.BP_Player_C|GetDBManager _player)
    (:then
      (Default|SendInteractEventtoDB _dbmanager (Utilities|Struct|MakeF_InteractEventsTableItem 0 (Variables|/Game/Game/Blueprints/Characters/AI/BP_NPC.BP_NPC_C|GetActorId (Variables|Default|GetOwner)) (Variables|/Game/Game/Blueprints/Characters/Players/BP_Player.BP_Player_C|GetUserId _player) "NewEnumerator0" Event%20Type (Math|DateTime|Now))))
    (:else)))

(event Custom|FaceWidgetToPlayer
  (bind _owner (Variables|Default|GetOwner))
  (bind _player (Variables|/Game/Game/Blueprints/Characters/AI/BP_NPC.BP_NPC_C|GetPlayer _owner))
  (bind _dialogwidget (Variables|/Game/Game/Blueprints/Characters/AI/BP_NPC_Talkable.BP_NPC_Talkable_C|GetDialogWidget _owner))
  (bind _returnvalue (Transformation|GetWorldLocation _dialogwidget))
  (bind _mesh (Variables|/Script/Engine.Character|GetMesh _player))
  (bind _returnvalue_2 (Transformation|GetWorldLocation _mesh))
  (bind _returnvalue_3 (Math|Rotator|FindLookatRotation _returnvalue _returnvalue_2))
  ;[1 1 1] Widget
  (if (Variables|Default|GetShowDialogPanel)
    (if (Variables|Default|GetIsTalking?)
      (Variables|Default|GetOwner
        (:then
          (Transformation|SetWorldRotation _dialogwidget (Math|Rotator|MakeRotator (.roll _returnvalue_3) (.pitch (Transformation|GetWorldRotation _dialogwidget)) (.yaw _returnvalue_3)) false false))
        (:else)))))

(event Custom|PlayDialogSound
  (bind _owner (Variables|Default|GetOwner))
  (bind _audio (Variables|/Game/Game/Blueprints/Characters/AI/BP_NPC.BP_NPC_C|GetAudio _owner))
  ;[1 1 1] Sound
  (bind _dialog (CallFunction|GetCurrentDialog))
  (Audio|Components|Audio|SetSound _audio (.voice _dialog))
  (Audio|Components|Audio|Play _audio 0.0)
  (EventDispatchers|BindEventtoOnAudioFinished _audio (delegate Custom|OnDialogSoundFinished)))

(event Custom|OnDialogSoundFinished
  ;[1 1 1] Sound
  (if (and (Variables|Default|GetIsTalking?) (not false))
    (Utilities|FlowControl|Delay 0.2)
    (bind _continue (CallFunction|NextDialog))
    (if _continue
      (CallFunction|ProcessDialog)
      (else
        (CallFunction|StopConversation)))))

(event Custom|StopConversation
  ;[1 1 1] Conversation
  (Variables|Default|SetIsTalking? false)
  (Audio|Components|Audio|Stop (Variables|/Game/Game/Blueprints/Characters/AI/BP_NPC.BP_NPC_C|GetAudio (Variables|Default|GetOwner)))
  (Default|CallConversationFinished (Variables|Default|GetConversationIndex))
  (if (Variables|Default|GetShowDialogPanel)
    (Development|SetHiddeninGame (Variables|/Game/Game/Blueprints/Characters/AI/BP_NPC_Talkable.BP_NPC_Talkable_C|GetDialogWidget (Variables|Default|GetOwner)) true false)
    (Default|HideDialogBox (Variables|Default|GetWidget))))

(event EventBeginPlay
  (Utilities|FlowControl|Sequence
    (:then_0
      (bind _asbp_npc_talkable (Utilities|Casting|CastToBP_NPC_Talkable (Components|GetOwner)))
      (Variables|Default|SetOwner _asbp_npc_talkable))
    (:then_1
      (bind _dialogwidget (Variables|/Game/Game/Blueprints/Characters/AI/BP_NPC_Talkable.BP_NPC_Talkable_C|GetDialogWidget (Variables|Default|GetOwner))
        (:then
          (Development|SetHiddeninGame _dialogwidget false false)
          (bind _aswbp_dialog (Utilities|Casting|CastToWBP_Dialog (UserInterface|GetWidget _dialogwidget)))
          (bind _output_get (Variables|Default|SetWidget _aswbp_dialog))
          (Default|SetOwner _output_get (Variables|Default|GetOwner)))
        (:else
          (Development|PrintString "El NPC no tiene el Widget para los \"diálogos\"" true true "(R=1.000000,G=0.000000,B=0.000000,A=1.000000)"))))
    (:then_2
      (CallFunction|SetDialogsfromDataTable))))

(event EventTick
  (params (DeltaSeconds :type Float%20%28single-precision%29))
  (CallFunction|FaceWidgettoPlayer))

(fn NextDialog
  (bind _conversations (Variables|Default|GetConversations))
  (bind _conversationindex (Variables|Default|GetConversationIndex))
  (bind _output (Utilities|Array|Get(acopy) _conversations _conversationindex))
  (bind _dialogdata (Utilities|Struct|BreakF_Conversation _output))
  (bind _returnvalue (Utilities|Array|Length _dialogdata))
  (if (and (> _returnvalue 0) (< (+ (Variables|Default|GetDialogIndex) 1) _returnvalue))
    (Math|Integer|IncrementInt (Variables|Default|GetDialogIndex)
      (:%20%20
        (return true)))
    (else
      (return false))))

(fn NextConversation
  (bind _isempty (CallFunction|IsConversationEmpty))
  (if (and (not _isempty) (< (Variables|Default|GetConversationIndex) (- (Utilities|Array|Length (Variables|Default|GetConversations)) 1)))
    (Variables|Default|SetConversationIndex (+ (Variables|Default|GetConversationIndex) 1))))

(fn SetDialogsfromDataTable
  (Utilities|Array|Clear (Variables|Default|GetConversations))
  (bind _dialog_data_table (Variables|Default|GetDialog%20Data%20Table)
    (:then
      (bind _outrownames (DataTable|GetDataTableRowNames _dialog_data_table))
      (for _array_element _outrownames
        (bind _returnvalue (Utilities|GetDataTableRow _dialog_data_table _array_element)
          (:then
            (Utilities|Array|Add (Variables|Default|GetConversations) (Utilities|Struct|MakeF_Conversation (.ConversationNumber (Utilities|Struct|BreakF_Conversation _returnvalue)) (.DialogData (Utilities|Struct|BreakF_Conversation _returnvalue))))))))
    (:else)))

(fn GetNumberOfConversations
  (params (List%20of%20Dialogs :type Array%20of%20Strings))
  (for _array_element List%20of%20Dialogs
    (Utilities|Set|Add (LocalVariables|GetAuxSet) _array_element))
  (return (Utilities|Set|Length (LocalVariables|GetAuxSet))))

(fn GetCurrentDialog
  (return (Utilities|Array|Get(acopy) (.DialogData (Utilities|Struct|BreakF_Conversation (Utilities|Array|Get(acopy) (Variables|Default|GetConversations) (Variables|Default|GetConversationIndex)))) (Variables|Default|GetDialogIndex))))

(fn GetCurrentConversation
  (return (Utilities|Array|Get(acopy) (Variables|Default|GetConversations) (Variables|Default|GetConversationIndex))))

(fn IsConversationEmpty
  (return (== (Utilities|Array|Length (Variables|Default|GetConversations)) 0)))

(fn CreatePlayerDialog
  (if (Variables|Default|GetShowDialogPanel)
    (bind _dialog (CallFunction|GetCurrentDialog))
    (Default|CreatePlayerText (Variables|Default|GetWidget) (Utilities|Text|ToText(String) (Variables|/Game/Game/Blueprints/Characters/Players/BP_Player.BP_Player_C|GetName (Variables|/Game/Game/Blueprints/Characters/AI/BP_NPC.BP_NPC_C|GetPlayer (Variables|Default|GetOwner)))) (.Text (Utilities|Struct|BreakF_DialogLine _dialog)))))

(fn CreateNPCDialog
  (if (Variables|Default|GetShowDialogPanel)
    (bind _dialog (CallFunction|GetCurrentDialog))
    (Default|CreateNPCText (Variables|Default|GetWidget) (Utilities|Text|ToText(String) (Variables|/Game/Game/Blueprints/Characters/AI/BP_NPC.BP_NPC_C|GetName (Variables|Default|GetOwner))) (.Text (Utilities|Struct|BreakF_DialogLine _dialog)))))