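; BP_GameplayManager_Develop is a child gameplay manager, named as a development variant, that wires up the VR player and tutorial buddy before starting the scenario.
; On SetPlayerData it runs the parent logic, binds player actions, then passes the BP_Player_VR's TutorialBuddyActor to the TutorialManager and binds the buddy's actions.
; A missing TutorialManager is logged, and a Sequence node calls StartScenario even if the cast or manager check fails.
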(event EventBeginPlay
  (|CallParentFunction))

(event EventSetPlayerData
  (|CallParentFunction)
  (CallFunction|BindPlayerActions)
  (Utilities|FlowControl|Sequence
    (:then_0
      (bind _asbp_player_vr (Utilities|Casting|CastToBP_Player_VR (Variables|Default|GetPlayer)))
      (bind _tutorialmanager (Variables|Default|GetTutorialManager)
        (:then
          (Default|SetCurrentTutorialBuddy _tutorialmanager (Variables|/Game/Game/Blueprints/Characters/Players/BP_Player_VR.BP_Player_VR_C|GetTutorialBuddyActor _asbp_player_vr))
          (CallFunction|BindTuddyActions))
        (:else
          (Default|Log (Variables|Default|GetGameInstance) "NewEnumerator2" "Falta el TutorialManager" false))))
    (:then_1
      (CallFunction|StartScenario))))

(fn ConstructionScript
  (|CallParentFunction))