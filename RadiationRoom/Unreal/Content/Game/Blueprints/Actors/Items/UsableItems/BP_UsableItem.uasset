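; BP_UsableItem is a usable item that works as a radiation meter for both TFP and VR players.
; TFP players trigger a reading through Use With, while VR players trigger it when the item's box overlaps an actor.
; MeasureRadiation queries the target's AC_Radiation component, shows DoseAbsorption in mSv/hour on RadiationText and logs an interaction event through DBManager.
; Look-at, interact and cancel events only call the parent, followed by empty player-type casts.
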(event OnComponentBeginOverlap(Box)
  (params (OverlappedComponent :type Primitive%20Component%20Object%20Reference) (OtherActor :type Actor%20Object%20Reference) (OtherComp :type Primitive%20Component%20Object%20Reference) (OtherBodyIndex :type Integer) (bFromSweep :type Boolean) (SweepResult :type Hit%20Result%20Structure%20%28by%20ref%29))
  ;[1 1 1] Interact
  (bind _player (Variables|Default|GetPlayer)
    (:then
      (bind _asbp_player_vr (Utilities|Casting|CastToBP_Player_VR _player))
      (|CallParentFunction OtherActor _asbp_player_vr)
      (CallFunction|MeasureRadiation OtherActor _asbp_player_vr))
    (:else)))

(event Custom|MeasureRadiation
  (params (Actor :type Actor%20Object%20Reference) (Player :type BP%20Player%20Object%20Reference))
  (bind _returnvalue (Actor|GetComponentbyClass Actor "/Game/Game/Blueprints/Components/AC_Radiation.AC_Radiation_C"))
  ;[1 1 1] Interact
  (Utilities|IsValid _returnvalue
    (:Is%20Valid
      (Default|MeasureRadiation _returnvalue)
      (Rendering|Components|TextRender|SetText (Variables|Default|GetRadiationText) (Utilities|Text|FormatText "{radiacion} mSv/hora" (Variables|/Game/Game/Blueprints/Components/AC_Radiation.AC_Radiation_C|GetDoseAbsorption _returnvalue)))
      (bind _dbmanager (Variables|Default|GetDBManager)
        (:then
          (Default|SendInteractEventtoDB _dbmanager (Utilities|Struct|MakeF_InteractEventsTableItem 0 (Variables|Default|GetActorId) (Variables|/Game/Game/Blueprints/Characters/Players/BP_Player.BP_Player_C|GetUserId Player) "NewEnumerator0" "NewEnumerator25" (Math|DateTime|Now))))
        (:else)))))

(event EventBeginPlay
  (|CallParentFunction))

(event EventStartLookat
  (params (Player :type BP%20Player%20Object%20Reference))
  ;[1 1 1] Look At
  (|CallParentFunction Player)
  (Utilities|FlowControl|Sequence
    (:then_0
      (Utilities|Casting|CastToBP_Player_TFP Player))
    (:then_1
      (Utilities|Casting|CastToBP_Player_VR Player))))

(event EventTick
  (params (DeltaSeconds :type Float%20%28single-precision%29))
  (|CallParentFunction DeltaSeconds))

(event EventInteractwith
  (params (Player :type BP%20Player%20Object%20Reference))
  ;[1 1 1] Interact
  (|CallParentFunction Player)
  (Utilities|FlowControl|Sequence
    (:then_0
      (Utilities|Casting|CastToBP_Player_TFP Player))
    (:then_1
      (Utilities|Casting|CastToBP_Player_VR Player))))

(event EventCancelInteract
  (params (Player :type BP%20Player%20Object%20Reference))
  ;[1 1 1] Interact
  (|CallParentFunction Player)
  (Utilities|FlowControl|Sequence
    (:then_0
      (Utilities|Casting|CastToBP_Player_TFP Player))
    (:then_1
      (Utilities|Casting|CastToBP_Player_VR Player))))

(event EventStopLookat
  (params (Player :type BP%20Player%20Object%20Reference))
  ;[1 1 1] Look At
  (|CallParentFunction Player)
  (Utilities|FlowControl|Sequence
    (:then_0
      (Utilities|Casting|CastToBP_Player_TFP Player))
    (:then_1
      (Utilities|Casting|CastToBP_Player_VR Player))))

(event EventUsewith
  (params (UsePoint :type Actor%20Object%20Reference) (Player :type BP%20Player%20Object%20Reference))
  ;[1 1 1] Interact
  (bind _asbp_player_tfp (Utilities|Casting|CastToBP_Player_TFP Player))
  (|CallParentFunction UsePoint _asbp_player_tfp)
  (CallFunction|MeasureRadiation UsePoint _asbp_player_tfp))

(fn ConstructionScript
  (|CallParentFunction))

(fn CanUsewith
  (params (Use%20Point :type Actor%20Object%20Reference))
  (return (== (Utilities|GetClass Use%20Point) 0)))