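; BP_RBQVan is a van actor that delivers items from a shopping list onto its plane.
; On BeginPlay it binds SpawnItems to the spawn event of its child BP_ShoppingListActor.
; For each item ID and count received, it spawns BP_ItemInitialState actors at random points just above the plane's bounds.
; Each spawned item is initialized with the row matching its ID, found by scanning the item data table.
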(event Custom|SpawnItems
  (params (Items :type Map%20of%20E_ItemtID%20Enums%20to%20Integers :default "NewEnumerator2"))
  (bind _plane (Variables|Default|GetPlane))
  (bind (_origin _boxextent) (Collision|GetComponentBounds _plane))
  (bind _keys (Utilities|Map|Keys Items))
  (for _array_element _keys
    (for _index (range 0 (- (.Value (Utilities|Map|Find Items _array_element)) 1))
      (bind _returnvalue (Game|SpawnActorfromClass "/Game/Game/Blueprints/Actors/BP_ItemInitialState.BP_ItemInitialState_C" (Math|Transform|MakeTransform (+ (Math|Random|RandomPointinBoundingBox _origin _boxextent) "0.000000,0.000000,20.000000")) "AdjustIfPossibleButAlwaysSpawn" "MultiplyWithRoot" 0 0))
      (bind _itemdata (CallFunction|GetItemDatatoSpawn _array_element))
      (Default|CreateItem _returnvalue _itemdata))))

(event EventBeginPlay
  (bind _asbp_shopping_list_actor (Utilities|Casting|CastToBP_ShoppingListActor (Variables|/Script/Engine.ChildActorComponent|GetChildActor (Variables|Default|GetChildActor))))
  (EventDispatchers|BindEventtoEDSpawnItems _asbp_shopping_list_actor (delegate Custom|SpawnItems)))

(fn ConstructionScript)

(fn GetItemDatatoSpawn
  (params (ItemId :type E_ItemtID%20Enum :default "NewEnumerator2"))
  (bind _itemdata_datatable (Variables|SpawnItems|GetItemData%20Datatable))
  (bind _outrownames (DataTable|GetDataTableRowNames _itemdata_datatable))
  (for _array_element _outrownames
    (bind _returnvalue (Utilities|GetDataTableRow _itemdata_datatable _array_element)
      (:then
        (if (Utilities|Enum|Equal(Enum) (.Id (Utilities|Struct|BreakF_ItemData _returnvalue)) ItemId)
          (LocalVariables|SetCurrentItemData _returnvalue)))))
  (return (LocalVariables|GetCurrentItemData)))