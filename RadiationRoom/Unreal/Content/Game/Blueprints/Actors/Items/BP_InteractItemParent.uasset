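; Base interactable item actor that handles look-at and point-at feedback and serves as parent for items the player interacts with.
; An outline mesh copy with a dynamic material shows focus in interact or grab colors, while a name label turns toward the player.
; Look and point events are logged through the database manager; look-at also updates the TFP player's HUD.
; Hitting an actor with a radiation component marks the item contaminated.
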(event OnComponentHit(StaticMesh)
  (params (HitComponent :type Primitive%20Component%20Object%20Reference) (OtherActor :type Actor%20Object%20Reference) (OtherComp :type Primitive%20Component%20Object%20Reference) (NormalImpulse :type Vector :default "0, 0, 0") (Hit :type Hit%20Result%20Structure%20%28by%20ref%29))
  (Utilities|IsValid (Actor|GetComponentbyClass OtherActor "/Game/Game/Blueprints/Components/AC_Radiation.AC_Radiation_C")
    (:Is%20Valid
      (Variables|/Game/Game/Blueprints/Components/AC_Radiation.AC_Radiation_C|SetIsContamined? (Variables|Default|GetAC_Radiation) true))))

(event Custom|ShowHideOutline
  (params (Show :type Boolean) (Grab :type Boolean))
  (bind _outlinematerial (Variables|Outline|GetOutlineMaterial))
  (Rendering|SetVisibility (Variables|Default|GetOutlineMesh) Show false)
  (if Grab
    (Rendering|Material|SetVectorParameterValue _outlinematerial "Color" (Variables|Outline|GetGrabOutlineColor) :!class /Script/Engine.MaterialInstanceDynamic)
    (else
      (Rendering|Material|SetVectorParameterValue _outlinematerial "Color" (Variables|Outline|GetInteractOutlineColor) :!class /Script/Engine.MaterialInstanceDynamic))))

(event Custom|NameFaceToPlayer
  (bind _player (Variables|Player|GetPlayer)
    (:then
      (Transformation|SetWorldRotation (Variables|Default|GetTextName) (Math|Rotator|FindLookatRotation (Transformation|GetActorLocation) (Transformation|GetActorLocation _player)) false false))
    (:else)))

(event EventStopLookat
  (params (Player :type BP%20Player%20Object%20Reference))
  ;[1 1 1] Look At
  (Utilities|FlowControl|Sequence
    (:then_0
      (bind _dbmanager (Variables|Default|GetDBManager)
        (:then
          (Default|SendInteractEventtoDB _dbmanager (Utilities|Struct|MakeF_InteractEventsTableItem 0 (Variables|ItemInfo|GetActorId) (Variables|/Game/Game/Blueprints/Characters/Players/BP_Player.BP_Player_C|GetUserId Player) "NewEnumerator0" "NewEnumerator16" (Math|DateTime|Now))))
        (:else)))
    (:then_1
      (Utilities|FlowControl|Sequence
        (:then_0
          (Utilities|Casting|CastToBP_Player_TFP Player)
          (CallFunction|ShowHideOutline false false))
        (:then_1
          (Utilities|Casting|CastToBP_Player_VR Player))))
    (:then_2
      (Rendering|SetVisibility (Variables|Default|GetTextName) false false))))

(event EventUsewith
  (params (UsePoint :type Actor%20Object%20Reference) (Player :type BP%20Player%20Object%20Reference))
  ;[1 1 1] Interact
  (Variables|Player|SetPlayer Player))

(event EventBeginPlay
  (bind _outlinemesh (Variables|Default|GetOutlineMesh))
  (|CallParentFunction)
  (Rendering|Components|TextRender|SetText (Variables|Default|GetTextName) (Utilities|Text|ToText(String) (Variables|ItemInfo|GetName)))
  (bind _returnvalue (Actor|GetActorOfClass "/Game/Game/Blueprints/Gameplay/BP_GameplayManager.BP_GameplayManager_C"))
  (Variables|Default|SetGameplayManager _returnvalue)
  (bind _returnvalue_2 (Actor|GetActorOfClass "/Game/Game/Blueprints/Database/BP_DataBase_Manager.BP_DataBase_Manager_C"))
  (Variables|Default|SetDBManager _returnvalue_2)
  (Components|StaticMesh|SetStaticMesh (Variables|Default|GetOutlineMesh) (Variables|/Script/Engine.StaticMeshComponent|GetStaticMesh (Variables|Default|GetStaticMesh)))
  (bind _returnvalue_3 (Rendering|Material|CreateDynamicMaterialInstance _outlinemesh 0 "/Game/Game/Materials/M_Outline.M_Outline" "None" :!class /Script/Engine.PrimitiveComponent))
  (bind _output_get (Variables|Outline|SetOutlineMaterial _returnvalue_3))
  (Rendering|Material|SetMaterial _outlinemesh 0 _output_get)
  (CallFunction|ShowHideOutline false false))

(event EventStartPointto
  (params (Player :type BP%20Player%20Object%20Reference))
  ;[1 1 1] Point to
  (Utilities|FlowControl|Sequence
    (:then_0
      (bind _dbmanager (Variables|Default|GetDBManager)
        (:then
          (Default|SendInteractEventtoDB _dbmanager (Utilities|Struct|MakeF_InteractEventsTableItem 0 (Variables|ItemInfo|GetActorId) (Variables|/Game/Game/Blueprints/Characters/Players/BP_Player.BP_Player_C|GetUserId Player) "NewEnumerator0" "NewEnumerator21" (Math|DateTime|Now))))
        (:else)))
    (:then_1
      (Utilities|Casting|CastToBP_PickableItem self
        (:CastFailed
          (CallFunction|ShowHideOutline true false))))))

(event EventInteractwith
  (params (Player :type BP%20Player%20Object%20Reference))
  ;[1 1 1] Interact
  (Variables|Player|SetPlayer Player))

(event EventStartLookat
  (params (Player :type BP%20Player%20Object%20Reference))
  ;[1 1 1] Look At
  (Variables|Player|SetPlayer Player)
  (Utilities|FlowControl|Sequence
    (:then_0
      (bind _dbmanager (Variables|Default|GetDBManager)
        (:then
          (Default|SendInteractEventtoDB _dbmanager (Utilities|Struct|MakeF_InteractEventsTableItem 0 (Variables|ItemInfo|GetActorId) (Variables|/Game/Game/Blueprints/Characters/Players/BP_Player.BP_Player_C|GetUserId Player) "NewEnumerator0" "NewEnumerator5" (Math|DateTime|Now))))
        (:else)))
    (:then_1
      (Utilities|FlowControl|Sequence
        (:then_0
          (bind _asbp_player_tfp (Utilities|Casting|CastToBP_Player_TFP Player))
          (Utilities|FlowControl|Sequence
            (:then_0
              (bind _iteminteracthud (Variables|/Game/Game/Blueprints/Characters/Players/BP_Player_TFP.BP_Player_TFP_C|GetItemInteractHUD _asbp_player_tfp)
                (:then
                  (Default|ChangeInteractionText _iteminteracthud (Utilities|IsValid (Variables|/Game/Game/Blueprints/Characters/Players/BP_Player.BP_Player_C|GetCurrentHeldItem _asbp_player_tfp)) "NewEnumerator0"))
                (:else)))
            (:then_1
              (bind _currenthelditem (Variables|/Game/Game/Blueprints/Characters/Players/BP_Player.BP_Player_C|GetCurrentHeldItem _asbp_player_tfp)
                (:then
                  (if (not (== _currenthelditem self))
                    (CallFunction|ShowHideOutline true false :!label _label)))
                (:else
                  (goto _label))))))
        (:then_1
          (Utilities|Casting|CastToBP_Player_VR Player))))
    (:then_2
      (Rendering|SetVisibility (Variables|Default|GetTextName) true false))))

(event EventCancelInteract
  (params (Player :type BP%20Player%20Object%20Reference))
  ;[1 1 1] Interact
  (Variables|Player|SetPlayer Player))

(event EventStopPointto
  (params (Player :type BP%20Player%20Object%20Reference))
  ;[1 1 1] Point to
  (Utilities|FlowControl|Sequence
    (:then_0
      (bind _dbmanager (Variables|Default|GetDBManager)
        (:then
          (Default|SendInteractEventtoDB _dbmanager (Utilities|Struct|MakeF_InteractEventsTableItem 0 (Variables|ItemInfo|GetActorId) (Variables|/Game/Game/Blueprints/Characters/Players/BP_Player.BP_Player_C|GetUserId Player) "NewEnumerator0" "NewEnumerator22" (Math|DateTime|Now))))
        (:else)))
    (:then_1
      (CallFunction|ShowHideOutline false false))))

(event EventTick
  (params (DeltaSeconds :type Float%20%28single-precision%29))
  (CallFunction|NameFacetoPlayer))

(fn ConstructionScript)