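; BP_ItemInitialState is an item actor that displays a data-driven static mesh fitted inside a capsule.
; BeginPlay refreshes ItemData by searching the data table for a matching Id, then attaches the mesh component to the capsule.
; CreateItem stores the supplied data and applies its mesh.
; It then uses component bounds to shrink oversized meshes within the capsule's radius and align their bounds centers, compensating for off-center pivots.
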(event Custom|SetItemScale
  (bind _item (Variables|Default|GetItem))
  (bind _capsule (Variables|Default|GetCapsule))
  (bind _sphereradius (Collision|GetComponentBounds _item))
  (bind _sphereradius_2 (Collision|GetComponentBounds _capsule))
  (bind _returnvalue (/ _sphereradius_2 _sphereradius))
  (bind _returnvalue_2 (* _returnvalue 0.8))
  (if (< _returnvalue_2 1.0)
    (Transformation|SetWorldScale3D (Variables|Default|GetItem) (* (Transformation|GetWorldScale (Variables|Default|GetItem)) _returnvalue_2))))

(event Custom|SetItemLocation
  (Transformation|SetWorldLocation (Variables|Default|GetItem) (- (Transformation|GetWorldLocation (Variables|Default|GetItem)) (- (.Origin (Collision|GetComponentBounds (Variables|Default|GetItem))) (.Origin (Collision|GetComponentBounds (Variables|Default|GetCapsule))))) false false))

(event Custom|CreateItem
  (params (Data :type F%20Item%20Data%20Structure))
  (bind _output_get (Variables|Default|SetItemData Data))
  (Components|StaticMesh|SetStaticMesh (Variables|Default|GetItem) (.mesh _output_get))
  (CallFunction|SetItemScale)
  (CallFunction|SetItemLocation))

(event EventBeginPlay
  (CallFunction|GetDatafromDataTable)
  (Transformation|AttachComponentToComponent (Variables|Default|GetItem) (Variables|Default|GetCapsule) "None" "KeepRelative" "KeepRelative" "KeepWorld" true))

(fn ConstructionScript)

(fn GetDatafromDataTable
  (bind _outrownames (DataTable|GetDataTableRowNames (Variables|Default|GetItemData%20DataTable)))
  (for _array_element _outrownames
    (bind _returnvalue (Utilities|GetDataTableRow (Variables|Default|GetItemData%20DataTable) _array_element)
      (:then
        (if (Utilities|Enum|Equal(Enum) (.Id (Utilities|Struct|BreakF_ItemData _returnvalue)) (.id (Variables|Default|GetItemData)))
          (Variables|Default|SetItemData _returnvalue)
          (return))))))