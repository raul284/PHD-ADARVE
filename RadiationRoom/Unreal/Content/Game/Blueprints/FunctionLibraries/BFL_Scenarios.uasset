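; Blueprint function library that gives access to the current scenario's data and its neighbouring levels.
; The base getter resolves the data table row handle stored on the game instance, and thin getters expose its fields, including control vars, walkie conversation and tutorial items.
; Previous and next scenarios are looked up by row name in DT_ScenarioData.
; A separate helper stores the first player start differing from the current one on the game instance.
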(fn GetCurrentScenarioData
  (bind _gameinstance (CallFunction|GetMyGameInstance))
  (bind _current_scenario_data (Variables|/Game/Game/Blueprints/RR_GameInstance.RR_GameInstance_C|GetCurrent%20Scenario%20Data _gameinstance))
  (bind _returnvalue (Utilities|GetDataTableRow (.datatable _current_scenario_data) (.rowname _current_scenario_data))
    (:then
      (return _returnvalue))))

(fn GetCurrentScenarioSpecificData
  (return (.SpecificData (Utilities|Struct|BreakF_ScenarioData (CallFunction|GetCurrentScenarioData)))))

(fn GetCurrentScenarioId
  (return (.id (CallFunction|GetCurrentScenarioData))))

(fn GetCurrentScenarioControlVars
  (return (.ControlVars (Utilities|Struct|BreakF_Scenario_SpecificData (CallFunction|GetCurrentScenarioSpecificData)))))

(fn GetCurrentScenarioWalkieConversation
  (return (.DefaultWalkieConversation (Utilities|Struct|BreakF_Scenario_SpecificData (CallFunction|GetCurrentScenarioSpecificData)))))

(fn GetCurrentScenarioActiveTutorialItems
  (return (.TutorialItems (Utilities|Struct|BreakF_Scenario_SpecificData (CallFunction|GetCurrentScenarioSpecificData)))))

(fn GetCurrentScenarioDescription
  (return (.description (CallFunction|GetCurrentScenarioData))))

(fn GetCurrentScenarioPreData
  (bind _returnvalue (Utilities|GetDataTableRow "/Game/Game/DataStructures/Scenarios/DT_ScenarioData.DT_ScenarioData" (.previouslevel (CallFunction|GetCurrentScenarioData)))
    (:then
      (return _returnvalue))))

(fn GetCurrentScenarioNextData
  (bind _returnvalue (Utilities|GetDataTableRow "/Game/Game/DataStructures/Scenarios/DT_ScenarioData.DT_ScenarioData" (.nextlevel (CallFunction|GetCurrentScenarioData)))
    (:then
      (return _returnvalue))))

(fn GetCurrentScenarioName
  (return (.bplevelname (CallFunction|GetCurrentScenarioData))))

(fn GetNewPlayerStartLocation
  (params (All%20Player%20Starts :type Array%20of%20BP%20Streaming%20Level%20Player%20Start%20Object%20References))
  (bind _array_element (Utilities|Array|ForEachLoopwithBreak All%20Player%20Starts :!label _label)
    (:LoopBody
      (if (!= (Variables|/Game/Game/Blueprints/RR_GameInstance.RR_GameInstance_C|GetCurrentPlayerStartPoint (CallFunction|GetMyGameInstance)) _array_element)
        (goto _label Break)))
    (:Completed
      (Variables|/Game/Game/Blueprints/RR_GameInstance.RR_GameInstance_C|SetCurrentPlayerStartPoint (CallFunction|GetMyGameInstance) _array_element))))