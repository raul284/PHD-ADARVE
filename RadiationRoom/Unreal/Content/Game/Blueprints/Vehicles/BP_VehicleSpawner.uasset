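; BP_VehicleSpawner is a vehicle spawner actor meant to emit BP_AutomaticVehicle actors from its own transform.
; BeginPlay calls SpawnVehicleOnServer, but that event is empty, so nothing spawns as wired.
; The disconnected spawn chain waits a random delay, checks CanSpawn, spawns a vehicle with a random mesh and the configured Velocity, then calls the event again to repeat.
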(event Custom|Spawn%20Vehicle%20On%20Server)

(event EventBeginPlay
  (CallFunction|SpawnVehicleonServer))

(event Collision|EventActorBeginOverlap
  (params (OtherActor :type Actor%20Object%20Reference)))

(event EventTick
  (params (DeltaSeconds :type Float%20%28single-precision%29)))

(fn ConstructionScript)