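; Talkable driver NPC Blueprint that gates its conversations to two story phases and walks to a destination between them.
; Interaction opens dialogue only when not walking and the GameplayManager is in or before either phase.
; Ending the first talk sets sit-to-stand and walking flags; StartWalking issues an AI MoveTo toward DestinationPoint.
; Tick checks 2D distance to stop on arrival, face the player and advance the conversation, so later endings complete the second phase.
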(event Custom|StartWalking
  (AI|Navigation|MovetoActor (AI|GetAIController self) (Variables|Default|GetDestinationPoint) -1.0 true true true 0))

(event Custom|StopWalking
  (bind _returnvalue (Transformation|GetActorLocation))
  (bind _destinationpoint (Variables|Default|GetDestinationPoint))
  (bind (_x _y) (Math|Vector|BreakVector _returnvalue))
  (bind _returnvalue_2 (Transformation|GetActorLocation _destinationpoint))
  (bind (_x_2 _y_2) (Math|Vector|BreakVector _returnvalue_2))
  (if (Variables|Default|GetWalking)
    (if (< (Math|Vector|Distance(Vector) (Math|Vector|MakeVector _x _y 0.0) (Math|Vector|MakeVector _x_2 _y_2 0.0)) 1e+02)
      (AI|Navigation|StopMovement (AI|GetAIController self))
      (Variables|Default|SetWalking false)
      (Variables|Animation|SetWalkToIdle true)
      (CallFunction|LookatPlayer)
      (Variables|Default|SetCanLookPlayer true)
      (CallFunction|NextConversation)
      (Variables|Default|SetProtected true))))

(event EventStopLookat
  (params (Player :type BP%20Player%20Object%20Reference))
  ;[1 1 1] Look at
  (|CallParentFunction Player))

(event EventTick
  (params (DeltaSeconds :type Float%20%28single-precision%29))
  (|CallParentFunction DeltaSeconds)
  (CallFunction|StopWalking))

(event EventStopConversation
  (bind _gameplaymanager (Variables|Default|GetGameplayManager))
  (|CallParentFunction)
  (Utilities|FlowControl|Sequence
    (:then_0
      (if (not (Variables|Animation|GetSitToStand))
        (Variables|Animation|SetSitToStand true)
        (Variables|Default|SetWalking true)))
    (:then_1
      (if (not (Variables|Default|GetProtected))
        (Default|CompletePhase _gameplaymanager "NewEnumerator1")
        (else
          (Default|CompletePhase _gameplaymanager "NewEnumerator2"))))))

(event EventInteractwith
  (params (Player :type BP%20Player%20Object%20Reference))
  (bind _gameplaymanager (Variables|Default|GetGameplayManager))
  ;[1 1 1] Interact
  (Utilities|FlowControl|Sequence
    (:then_0
      (Variables|Default|SetPlayer Player))
    (:then_1
      (if (not (Variables|Default|GetWalking))
        (bind _currentorprephase (Default|CheckCurrentorPrePhase _gameplaymanager "NewEnumerator1"))
        (bind _currentorprephase_2 (Default|CheckCurrentorPrePhase _gameplaymanager "NewEnumerator2"))
        (if (or _currentorprephase_2 _currentorprephase)
          (|CallParentFunction Player))))))

(event EventStartLookat
  (params (Player :type BP%20Player%20Object%20Reference))
  ;[1 1 1] Look at
  (|CallParentFunction Player))

(event EventCancelInteract
  (params (Player :type BP%20Player%20Object%20Reference))
  ;[1 1 1] Interact
  (|CallParentFunction Player))

(event EventBeginPlay
  (|CallParentFunction) ; This node is disabled and will not be called.\nDrag off pins to build functionality.
)

(fn ConstructionScript
  (|CallParentFunction))