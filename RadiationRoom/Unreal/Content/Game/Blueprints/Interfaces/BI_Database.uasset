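; BI_Database is a Blueprint interface for the game's database access, apparently for logging experiment and gameplay data.
; It declares builders for insert queries on experiments, sessions, teams, users, interact events and gameplay events, plus a move event query.
; It also declares functions to add update and select queries and send each kind to the database.
; Helper functions get a user ID from a player name and convert datetimes to strings.
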(fn CreateInteractEventInsertQuery
  (params (Data :type F%20Interact%20Events%20Table%20Item%20Structure))
  (return))

(fn CreateGameplayEventInsertQuery
  (params (Data :type F%20Gameplay%20Events%20Table%20Item%20Structure))
  (return))

(fn CreateMoveEventQuery
  (params (Data :type F%20Move%20Events%20Table%20Item%20Structure))
  (return))

(fn CreateUserInsertQuery
  (params (Data :type F%20User%20Table%20Item%20Structure))
  (return))

(fn CreateTeamInsertQuery
  (params (Data :type F%20Team%20Table%20Item%20Structure))
  (return))

(fn CreateSessionInsertQuery
  (params (Data :type F%20Session%20Table%20Item%20Structure))
  (return))

(fn CreateExperimentInsertQuery
  (params (Data :type F%20Experiment%20Table%20Item%20Structure))
  (return))

(fn SendUpdateQuerystoDB)

(fn SendSelectQuerystoDB)

(fn AddUpdateQuery
  (params (Query :type String)))

(fn AddSelectQuery
  (params (Query :type String)))

(fn GetUserId
  (params (Player%20Name :type String))
  (return))

(fn DatetimetoString
  (params (Datetime :type Date%20Time%20Structure))
  (return ""))