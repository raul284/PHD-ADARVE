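; Gameplay manager for the T1 tutorial scenario, guiding the player from introduction through teleporting, detecting, grabbing, NPC conversations and tidying up to the exit.
; It extends a parent manager's binding hooks, reacting to Tuddy tutorial buddy dialogs, player, item, place point and NPC events.
; Step-guarded handlers complete and advance steps, trigger Tuddy calls and unlock items, place points and doors.
; Detection, grab and tidy-up phases finish only when all relevant objects qualify.
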(event Custom|OnCountdownEnded
  (Transformation|SetActorLocation (Variables|Default|GetPlayer) (Transformation|GetActorLocation (Variables|Default|GetInitialTeleportPoint)) false true))

(event EventBeginPlay
  (|CallParentFunction)
  (Utilities|FlowControl|Sequence
    (:then_0
      (CallFunction|BindItemActions)
      (CallFunction|BindPlacePointsActions)
      (CallFunction|BindNPCActions))
    (:then_1
      (CallFunction|StartScenario)
      (Utilities|FlowControl|Delay 0.2)
      (CallFunction|CompleteStep "NewEnumerator9"))))

(event EventSetPlayerData
  (|CallParentFunction)
  (CallFunction|BindPlayerActions))

(event EventStartScenario
  (bind _welcomewidget (Variables|Default|GetWelcomeWidget))
  (|CallParentFunction)
  (Utilities|FlowControl|Delay 2.0)
  (Default|StartCountdown _welcomewidget)
  (EventDispatchers|BindEventtoEDCountdownEnded _welcomewidget (delegate Custom|OnCountdownEnded)))

(event Custom|OnTuddyIntroductionDialogCompleted
  (bind _yes (CallFunction|IsCurrentStep "NewEnumerator39"))
  (if _yes
    (CallFunction|CompleteStep "NewEnumerator39")
    (CallFunction|SetCurrentGameplayStep "NewEnumerator42")
    (Default|AutomaticCall (Variables|Default|GetTutorialManager) "NewEnumerator2")))

(event Custom|OnTuddyIsOnHand
  (bind _yes (CallFunction|IsCurrentStep "NewEnumerator43"))
  (if _yes
    (CallFunction|CompleteStep "NewEnumerator43")
    (CallFunction|SetCurrentGameplayStep "NewEnumerator44")
    (Default|AutomaticCall (Variables|Default|GetTutorialManager) "NewEnumerator7")))

(event Custom|OnFinalConversationCompleted
  (bind _yes (CallFunction|IsCurrentStep "NewEnumerator47"))
  (if _yes
    (CallFunction|CompleteStep "NewEnumerator47")
    (CallFunction|SetCurrentGameplayStep "NewEnumerator7")
    (Utilities|FlowControl|Delay 0.5)
    (Default|HideCurrentTuddy (Variables|Default|GetTutorialManager))
    (Default|AutomaticOpenandLockDoor (Variables|Door|GetExitDoor))))

(event Custom|OnTuddyDialogCompleted
  (params (CurrentTuddyDialogType :type E_TuddyDialogLinesType%20Enum :default "NewEnumerator0") (CurrentExtraLineType :type E_TuddyExtraLineTypes%20Enum :default "NewEnumerator1"))
  (switch Utilities|FlowControl|Switch|SwitchonE_GameplayStepTypes (Variables|Default|GetCurrentStepType)
    (:NewEnumerator39
      (CallFunction|OnTuddyIntroductionDialogCompleted))
    (:NewEnumerator40
      (for _array_element 0
        (Variables|/Game/Game/Blueprints/Actors/Items/BP_TutorialPickableItem.BP_TutorialPickableItem_C|SetCanBeDetected _array_element true)))
    (:NewEnumerator41
      (for _array_element_2 0
        (Variables|/Game/Game/Blueprints/Actors/Items/BP_TutorialPickableItem.BP_TutorialPickableItem_C|SetCanBeGrabbed _array_element_2 true)))
    (:NewEnumerator48
      (Default|AutomaticOpenandLockDoor (Variables|Door|GetBigRoomDoor)))
    (:NewEnumerator43
      (CallFunction|OnTuddyIsonHand))
    (:NewEnumerator47
      (CallFunction|OnFinalConversationCompleted))))

(event EventBindTuddyActions
  (|CallParentFunction)
  (EventDispatchers|BindEventtoEDDialogCompleted (Variables|/Game/Game/Blueprints/Tutorial/BP_TutorialBuddy.BP_TutorialBuddy_C|GetAC_TuddyDialogManager (Variables|/Game/Game/Blueprints/Tutorial/BP_TutorialManager.BP_TutorialManager_C|GetCurrentTutorialBuddy (Variables|Default|GetTutorialManager))) (delegate Custom|OnTuddyDialogCompleted)))

(event Custom|UserEnterExitRoom
  (params (OverlappedActor :type Actor%20Object%20Reference) (OtherActor :type Actor%20Object%20Reference))
  (bind _yes (CallFunction|IsCurrentStep "NewEnumerator7"))
  (if _yes
    (if (== OtherActor (Variables|Default|GetPlayer))
      (CallFunction|CompleteStep "NewEnumerator7")
      (CallFunction|EndGameplay))))

(event Custom|OnPlayerTeleported
  (bind _yes (CallFunction|IsCurrentStep "NewEnumerator42"))
  (if _yes
    (bind _output_get (Variables|Default|SetTimesTeleported (+ (Variables|Default|GetTimesTeleported) 1)))
    (if (== _output_get 5)
      (CallFunction|CompleteStep "NewEnumerator42"))))

(event EventBindPlayerActions
  (|CallParentFunction)
  (EventDispatchers|BindEventtoEDTeleported (Variables|Default|GetPlayer) (delegate Custom|OnPlayerTeleported))
  (Collision|BindEventtoOnActorBeginOverlap (Variables|Triggers|GetExitRoomTrigger) (delegate Custom|UserEnterExitRoom)))

(event Custom|OnTutorialItemDetected
  (params (Actor :type BP%20Interact%20Item%20Parent%20Object%20Reference))
  (bind _yes (CallFunction|IsCurrentStep "NewEnumerator40"))
  (if _yes
    (bind _completed (CallFunction|IsTutorialItemDetectionPhaseCompleted?))
    (if _completed
      (Default|HideAutomaticHintPanel (Variables|Default|GetTutorialManager))
      (CallFunction|CompleteStep "NewEnumerator40")
      (CallFunction|SetCurrentGameplayStep "NewEnumerator41")
      (Utilities|FlowControl|Delay 2.0)
      (Default|AutomaticCall (Variables|Default|GetTutorialManager) "NewEnumerator5"))))

(event Custom|OnTutorialItemGrabbed
  (params (Actor :type BP%20Interact%20Item%20Parent%20Object%20Reference))
  (bind _yes (CallFunction|IsCurrentStep "NewEnumerator41"))
  (if _yes
    (bind _completed (CallFunction|IsTutorialItemGrabPhaseCompleted?))
    (if _completed
      (Default|HideAutomaticHintPanel (Variables|Default|GetTutorialManager))
      (CallFunction|CompleteStep "NewEnumerator41")
      (CallFunction|SetCurrentGameplayStep "NewEnumerator48")
      (Utilities|FlowControl|Delay 2.0)
      (Default|StartExtraLinesDialog (Variables|Default|GetTutorialManager) "NewEnumerator2"))))

(event Custom|OnPlacePointManagerCompleted
  (bind _yes (CallFunction|IsCurrentStep "NewEnumerator45"))
  (if _yes
    (bind _completed (CallFunction|IsTidyUpPhaseCompleted?))
    (if _completed
      (CallFunction|CompleteStep "NewEnumerator45")
      (Default|NextConversation (Variables|Default|GetNPC))
      (CallFunction|SetCurrentGameplayStep "NewEnumerator46"))))

(event Custom|OnFirstRoomItemsSpawned
  (Utilities|FlowControl|Delay 1.0)
  (CallFunction|SetCurrentGameplayStep "NewEnumerator40")
  (Default|AutomaticCall (Variables|Default|GetTutorialManager) "NewEnumerator4"))

(event EventBindItemActions
  (|CallParentFunction)
  (EventDispatchers|BindEventtoEDFirstRoomItemsSpawned (delegate Custom|OnFirstRoomItemsSpawned))
  (for _array_element 0
    (EventDispatchers|BindEventtoEDDetectionStarted _array_element (delegate Custom|OnTutorialItemDetected))
    (EventDispatchers|AssignEDInteractionStarted _array_element (delegate Custom|OnTutorialItemGrabbed))))

(event EventBindPlacePointsActions
  (|CallParentFunction)
  (for _array_element (Variables|Default|GetPlacePointManagers)
    (EventDispatchers|BindEventtoEDAllPlacePointswithItems _array_element (delegate Custom|OnPlacePointManagerCompleted))))

(event Custom|OnNPCConversationFinished
  (params (ConversationNumber :type Integer))
  (switch Utilities|FlowControl|Switch|SwitchonE_GameplayStepTypes (Variables|Default|GetCurrentStepType)
    (:NewEnumerator44
      (CallFunction|OnNPCIntroductionCompleted))
    (:NewEnumerator46
      (CallFunction|OnInformtoNPCCompleted))))

(event Custom|OnNPCIntroductionCompleted
  (bind _yes (CallFunction|IsCurrentStep "NewEnumerator44"))
  (if _yes
    (CallFunction|CompleteStep "NewEnumerator44")
    (CallFunction|SetCurrentGameplayStep "NewEnumerator45")
    (Default|NextConversation (Variables|Default|GetNPC))
    (Utilities|FlowControl|Delay 1.0)
    (Default|ShowCurrentTuddy (Variables|Default|GetTutorialManager))
    (Utilities|FlowControl|Delay 1.0)
    (Default|AutomaticCall (Variables|Default|GetTutorialManager) "NewEnumerator15")
    (for _array_element (Variables|Default|GetPlacePointManagers)
      (Variables|/Game/Game/Blueprints/Actors/Items/PlacePoints/BP_PlacePointManager.BP_PlacePointManager_C|SetCanActivatePoints _array_element true)
      (Default|ShowInfoWidget _array_element))))

(event Custom|OnInformToNPCCompleted
  (bind _yes (CallFunction|IsCurrentStep "NewEnumerator46"))
  (if _yes
    (CallFunction|CompleteStep "NewEnumerator46")
    (CallFunction|SetCurrentGameplayStep "NewEnumerator47")
    (Utilities|FlowControl|Delay 1.0)
    (Default|StartExtraLinesDialog (Variables|Default|GetTutorialManager) "NewEnumerator4")))

(event Custom|OnNPCConversationStarted
  (switch Utilities|FlowControl|Switch|SwitchonE_GameplayStepTypes (Variables|Default|GetCurrentStepType)
    (:NewEnumerator44
      (Default|HideAutomaticHintPanel (Variables|Default|GetTutorialManager))
      (Default|HideCurrentTuddy (Variables|Default|GetTutorialManager)))))

(event EventBindNPCActions
  (|CallParentFunction)
  (bind _npc (Variables|Default|GetNPC)
    (:then
      (EventDispatchers|BindEventtoEDConversationStarted _npc (delegate Custom|OnNPCConversationStarted))
      (EventDispatchers|BindEventtoEDConversationFinished _npc (delegate Custom|OnNPCConversationFinished)))
    (:else
      (Default|Log (Variables|Default|GetGameInstance) "NewEnumerator2" "Falta NPC" false))))

(fn ConstructionScript)

(fn IsTutorialItemDetectionPhaseCompleted?
  (for _array_element 0
    (if (not (Variables|/Game/Game/Blueprints/Actors/Items/BP_TutorialPickableItem.BP_TutorialPickableItem_C|GetHasBeenDetected _array_element))
      (return false)))
  (return true))

(fn IsTutorialItemGrabPhaseCompleted?
  (for _array_element 0
    (if (not (Variables|/Game/Game/Blueprints/Actors/Items/BP_TutorialPickableItem.BP_TutorialPickableItem_C|GetLiar _array_element))
      (if (not (Variables|/Game/Game/Blueprints/Actors/Items/BP_TutorialPickableItem.BP_TutorialPickableItem_C|GetHasBeenGrabbed _array_element))
        (return false))))
  (return true))

(fn IsTidyUpPhaseCompleted?
  (for _array_element (Variables|Default|GetPlacePointManagers)
    (if (not (Variables|/Game/Game/Blueprints/Actors/Items/PlacePoints/BP_PlacePointManager.BP_PlacePointManager_C|GetAllPointsUsed _array_element))
      (return false)))
  (return true))