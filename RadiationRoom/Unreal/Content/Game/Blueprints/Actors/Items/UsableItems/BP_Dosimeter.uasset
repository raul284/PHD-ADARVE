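; BP_Dosimeter is a usable dosimeter item that supports both first-person (TFP) and VR players.
; For TFP players, a valid use completes a gameplay phase through GameplayManager if it is the current or preceding phase.
; In VR, a box overlap forwards the use to the parent and calls MeasureRadiation on the target's AC_Radiation component.
; Correct use beeps and briefly shows a light; incorrect use does nothing.
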(event OnComponentBeginOverlap(Box_0)
  (params (OverlappedComponent :type Primitive%20Component%20Object%20Reference) (OtherActor :type Actor%20Object%20Reference) (OtherComp :type Primitive%20Component%20Object%20Reference) (OtherBodyIndex :type Integer) (bFromSweep :type Boolean) (SweepResult :type Hit%20Result%20Structure%20%28by%20ref%29))
  (bind _returnvalue (Actor|GetComponentbyClass OtherActor "/Game/Game/Blueprints/Components/AC_Radiation.AC_Radiation_C"))
  (bind _player (Variables|Default|GetPlayer)
    (:then
      (bind _asbp_player_vr (Utilities|Casting|CastToBP_Player_VR _player))
      (|CallParentFunction OtherActor _asbp_player_vr)
      (Utilities|IsValid _returnvalue
        (:Is%20Valid
          (Default|MeasureRadiation _returnvalue)
          (if (> (Variables|/Game/Game/Blueprints/Components/AC_Radiation.AC_Radiation_C|GetRadiation _returnvalue) 0.0)
            _))))
    (:else)))

(event EventBeginPlay
  (|CallParentFunction))

(event EventStartLookat
  (params (Player :type BP%20Player%20Object%20Reference))
  ;[1 1 1] Look At
  (|CallParentFunction Player)
  (Utilities|FlowControl|Sequence
    (:then_0
      (Utilities|Casting|CastToBP_Player_TFP Player))
    (:then_1
      (Utilities|Casting|CastToBP_Player_VR Player))))

(event EventTick
  (params (DeltaSeconds :type Float%20%28single-precision%29))
  (|CallParentFunction DeltaSeconds))

(event EventInteractwith
  (params (Player :type BP%20Player%20Object%20Reference))
  (|CallParentFunction Player)
  (Utilities|FlowControl|Sequence
    (:then_0
      (Utilities|Casting|CastToBP_Player_TFP Player))
    (:then_1
      (Utilities|Casting|CastToBP_Player_VR Player))))

(event EventCancelInteract
  (params (Player :type BP%20Player%20Object%20Reference))
  (|CallParentFunction Player)
  (Utilities|FlowControl|Sequence
    (:then_0
      (Utilities|Casting|CastToBP_Player_TFP Player))
    (:then_1
      (Utilities|Casting|CastToBP_Player_VR Player))))

(event EventStopLookat
  (params (Player :type BP%20Player%20Object%20Reference))
  ;[1 1 1] Look At
  (|CallParentFunction Player)
  (Utilities|FlowControl|Sequence
    (:then_0
      (Utilities|Casting|CastToBP_Player_TFP Player))
    (:then_1
      (Utilities|Casting|CastToBP_Player_VR Player))))

(event EventUsewith
  (params (UsePoint :type Actor%20Object%20Reference) (Player :type BP%20Player%20Object%20Reference))
  (bind _asbp_player_tfp (Utilities|Casting|CastToBP_Player_TFP Player))
  (|CallParentFunction UsePoint _asbp_player_tfp)
  (bind _can (CallFunction|CanUsewith UsePoint))
  (if _can
    (bind _currentorprephase (Default|CheckCurrentorPrePhase (Variables|Default|GetGameplayManager) "NewEnumerator5"))
    (if _currentorprephase
      (Default|CompletePhase (Variables|Default|GetGameplayManager) "NewEnumerator5"))))

(event EventUseCorrect
  (params (Player :type BP%20Player%20Object%20Reference))
  (bind _pointlight (Variables|Default|GetPointLight))
  (Audio|PlaySoundatLocation "/Game/Game/Assets/Sounds/effects/beep_positive.beep_positive" (Transformation|GetActorLocation) "0, 0, 0" 1.0 1.0 0.0 0 0 0)
  (Rendering|SetVisibility _pointlight true false)
  (Utilities|FlowControl|Delay 2.0)
  (Rendering|SetVisibility _pointlight false false))

(event EventUseIncorrect
  (params (Player :type BP%20Player%20Object%20Reference)))

(fn ConstructionScript
  (|CallParentFunction))