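; BP_Spawner is a start point that stays hidden without collision for ten seconds after BeginPlay, then serves as a gameplay completion trigger.
; When a player overlaps its capsule and the GameplayManager's phase check passes, it completes that phase and calls the player's GameplayCompleted.
; Ending the overlap calls SetVisibility on the player's end widget.
; Each tick, its text render turns toward the local player's mesh, keeping its own pitch.
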(event OnComponentBeginOverlap(Capsule)
  (params (OverlappedComponent :type Primitive%20Component%20Object%20Reference) (OtherActor :type Actor%20Object%20Reference) (OtherComp :type Primitive%20Component%20Object%20Reference) (OtherBodyIndex :type Integer) (bFromSweep :type Boolean) (SweepResult :type Hit%20Result%20Structure%20%28by%20ref%29))
  (bind _asbp_player (Utilities|Casting|CastToBP_Player OtherActor))
  (bind _currentorprephase (Default|CheckCurrentorPrePhase (Variables|Default|GetGameplayManager) "NewEnumerator7"))
  (if _currentorprephase
    (Default|GameplayCompleted _asbp_player)
    (Default|CompletePhase (Variables|Default|GetGameplayManager) "NewEnumerator7")))

(event OnComponentEndOverlap(Capsule)
  (params (OverlappedComponent :type Primitive%20Component%20Object%20Reference) (OtherActor :type Actor%20Object%20Reference) (OtherComp :type Primitive%20Component%20Object%20Reference) (OtherBodyIndex :type Integer))
  (bind _asbp_player (Utilities|Casting|CastToBP_Player OtherActor))
  (Rendering|SetVisibility (Variables|/Game/Game/Blueprints/Characters/Players/BP_Player.BP_Player_C|GetTheEndWidget _asbp_player) false false))

(event Custom|EnableStartPoint
  (Rendering|SetActorHiddenInGame false)
  (Collision|SetCollisionEnabled (Variables|Default|GetCapsule) "QueryAndPhysics"))

(event Custom|LookAtPlayer
  (bind _returnvalue (Game|GetPlayerController 0))
  (bind _textrender (Variables|Default|GetTextRender))
  (if (Pawn|IsLocalController _returnvalue)
    (bind _asbp_player (Utilities|Casting|CastToBP_Player (Pawn|GetControlledPawn _returnvalue)))
    (Transformation|SetWorldRotation (Variables|Default|GetTextRender) (Math|Rotator|MakeRotator (.roll (Math|Rotator|FindLookatRotation (Transformation|GetWorldLocation _textrender) (Transformation|GetWorldLocation (Variables|/Script/Engine.Character|GetMesh _asbp_player)))) (.pitch (Transformation|GetWorldRotation _textrender)) (.yaw (Math|Rotator|FindLookatRotation (Transformation|GetWorldLocation _textrender) (Transformation|GetWorldLocation (Variables|/Script/Engine.Character|GetMesh _asbp_player))))) false false)))

(event EventBeginPlay
  (bind _returnvalue (Actor|GetActorOfClass "/Game/Game/Blueprints/Gameplay/BP_GameplayManager.BP_GameplayManager_C"))
  (Variables|Default|SetGameplayManager _returnvalue)
  (Rendering|SetActorHiddenInGame true)
  (Collision|SetCollisionEnabled (Variables|Default|GetCapsule) "NoCollision")
  (Utilities|FlowControl|Delay 1e+01)
  (CallFunction|EnableStartPoint))

(event EventTick
  (params (DeltaSeconds :type Float%20%28single-precision%29))
  (CallFunction|LookatPlayer))

(fn ConstructionScript)