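; BP_DestinationPoint is a VR destination marker that signals when the player enters or leaves it.
; Each Tick it turns its Arrows to face the player's mesh on yaw only, first finding and caching BP_Player if the reference is invalid.
; Capsule overlaps with BP_Player fire the enter and exit event dispatchers.
; SetActive stores the Active flag and shows or hides the actor, but the overlap events do not check that flag.
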(event OnComponentBeginOverlap(Capsule)
  (params (OverlappedComponent :type Primitive%20Component%20Object%20Reference) (OtherActor :type Actor%20Object%20Reference) (OtherComp :type Primitive%20Component%20Object%20Reference) (OtherBodyIndex :type Integer) (bFromSweep :type Boolean) (SweepResult :type Hit%20Result%20Structure%20%28by%20ref%29))
  (Utilities|Casting|CastToBP_Player OtherActor)
  (Default|CallEDPlayerEnteronDestinationPoint))

(event OnComponentEndOverlap(Capsule)
  (params (OverlappedComponent :type Primitive%20Component%20Object%20Reference) (OtherActor :type Actor%20Object%20Reference) (OtherComp :type Primitive%20Component%20Object%20Reference) (OtherBodyIndex :type Integer))
  (Utilities|Casting|CastToBP_Player OtherActor)
  (Default|CallEDPlayerExitOfDestinationPoint))

(event Custom|LookAtPlayer
  (bind _arrows (Variables|Default|GetArrows))
  (bind _returnvalue (Transformation|GetWorldRotation _arrows))
  (Transformation|SetWorldRotation (Variables|Default|GetArrows) (Math|Rotator|MakeRotator (.roll _returnvalue) (.pitch _returnvalue) (- (.Yaw (Math|Rotator|BreakRotator (Math|Rotator|FindLookatRotation (Transformation|GetWorldLocation (Variables|Default|GetArrows)) (Transformation|GetWorldLocation (Variables|/Script/Engine.Character|GetMesh (Variables|Default|GetPlayer)))))) 9e+01)) false false))

(event Custom|SetActive
  (params (Activate :type Boolean))
  (bind _output_get (Variables|Default|SetActive Activate))
  (Rendering|SetActorHiddenInGame (not _output_get)))

(event EventTick
  (params (DeltaSeconds :type Float%20%28single-precision%29))
  (Variables|Default|GetPlayer
    (:then
      (CallFunction|LookatPlayer))
    (:else
      (bind _returnvalue (Actor|GetActorOfClass "/Game/Game/Blueprints/Characters/Players/BP_Player.BP_Player_C"))
      (Variables|Default|SetPlayer _returnvalue))))

(fn ConstructionScript)