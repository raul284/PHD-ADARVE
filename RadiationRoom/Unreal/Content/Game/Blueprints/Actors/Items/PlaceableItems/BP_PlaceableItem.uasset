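; Placeable item that a desktop (TFP) or VR player picks up and sets onto place points, logging correct and incorrect attempts to a database.
; On BeginPlay it gathers place-item managers matching its class, then toggles their points on interact, correct placement or cancel.
; UseWith, or overlap for VR, asks the BP_PlacePoint to validate the item.
; A valid placement releases the item and snaps it to the point at original scale.
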(event Custom|PlaceCorrect
  (params (Player :type BP%20Player%20Object%20Reference))
  ;[1 1 1] Interact
  (Utilities|FlowControl|Sequence
    (:then_0
      (bind _dbmanager (Variables|Default|GetDBManager)
        (:then
          (Default|SendInteractEventtoDB _dbmanager (Utilities|Struct|MakeF_InteractEventsTableItem 0 (Variables|Default|GetActorId) (Variables|/Game/Game/Blueprints/Characters/Players/BP_Player.BP_Player_C|GetUserId Player) "NewEnumerator0" "NewEnumerator15" (Math|DateTime|Now))))
        (:else)))
    (:then_1
      (Utilities|FlowControl|Sequence
        (:then_0
          (bind _asbp_player_tfp (Utilities|Casting|CastToBP_Player_TFP Player))
          (Utilities|FlowControl|Sequence
            (:then_0
              (CallFunction|Drop _asbp_player_tfp)
              (Transformation|SetActorTransform (Transformation|GetActorTransform (Variables|Default|GetUsePoint)))
              (Transformation|SetActorScale3D (Variables|Default|GetOriScale))
              (Physics|SetSimulatePhysics (Variables|Default|GetStaticMesh) false))
            (:then_1
              (for _array_element (Variables|Default|GetPlaceItemManager)
                (Default|ActivateAllPoints _array_element false)))))
        (:then_1
          (bind _asbp_player_vr (Utilities|Casting|CastToBP_Player_VR Player))
          (Default|PlaceItem _asbp_player_vr)
          (Transformation|SetActorTransform (Transformation|GetActorTransform (Variables|Default|GetUsePoint)))
          (Transformation|SetActorScale3D (Variables|Default|GetOriScale))
          (for _array_element_2 (Variables|Default|GetPlaceItemManager)
            (Default|ActivateAllPoints _array_element_2 false)))))))

(event Custom|PlaceIncorrect
  (params (Player :type BP%20Player%20Object%20Reference))
  ;[1 1 1] Interact
  (Utilities|FlowControl|Sequence
    (:then_0
      (bind _dbmanager (Variables|Default|GetDBManager)
        (:then
          (Default|SendInteractEventtoDB _dbmanager (Utilities|Struct|MakeF_InteractEventsTableItem 0 (Variables|Default|GetActorId) (Variables|/Game/Game/Blueprints/Characters/Players/BP_Player.BP_Player_C|GetUserId Player) "NewEnumerator0" "NewEnumerator19" (Math|DateTime|Now))))
        (:else)))
    (:then_1
      (Utilities|FlowControl|Sequence
        (:then_0
          (Utilities|Casting|CastToBP_Player_TFP Player))
        (:then_1
          (Utilities|Casting|CastToBP_Player_VR Player))))))

(event EventBeginPlay
  (|CallParentFunction)
  (bind _outactors (Actor|GetAllActorsOfClass "/Game/Game/Blueprints/Actors/Items/PlaceableItems/BP_PlaceItemManager.BP_PlaceItemManager_C"))
  (for _array_element _outactors
    (if (== (Variables|/Game/Game/Blueprints/Actors/Items/PlaceableItems/BP_PlaceItemManager.BP_PlaceItemManager_C|GetItemClass _array_element) (Utilities|GetClass self))
      (Utilities|Array|Add (Variables|Default|GetPlaceItemManager) _array_element))))

(event EventStartLookat
  (params (Player :type BP%20Player%20Object%20Reference))
  ;[1 1 1] Look At
  (|CallParentFunction Player)
  (Utilities|FlowControl|Sequence
    (:then_0
      (Utilities|Casting|CastToBP_Player_TFP Player))
    (:then_1
      (Utilities|Casting|CastToBP_Player_VR Player))))

(event EventTick
  (params (DeltaSeconds :type Float%20%28single-precision%29))
  (|CallParentFunction DeltaSeconds))

(event EventInteractwith
  (params (Player :type BP%20Player%20Object%20Reference))
  ;[1 1 1] Interact
  (|CallParentFunction Player)
  (Utilities|FlowControl|Sequence
    (:then_0
      (bind _usepoint (Variables|Default|GetUsePoint)
        (:then
          (Default|RemoveItemfromPlacePoint _usepoint))
        (:else
          _))
      (for _array_element (Variables|Default|GetPlaceItemManager)
        (Default|ActivateAllPoints _array_element true)))
    (:then_1
      (Utilities|Casting|CastToBP_Player_TFP Player))
    (:then_2
      (Utilities|Casting|CastToBP_Player_VR Player))))

(event EventCancelInteract
  (params (Player :type BP%20Player%20Object%20Reference))
  ;[1 1 1] Interact
  (|CallParentFunction Player)
  (Utilities|FlowControl|Sequence
    (:then_0
      (for _array_element (Variables|Default|GetPlaceItemManager)
        (Default|ActivateAllPoints _array_element false)
        (Physics|SetSimulatePhysics (Variables|Default|GetStaticMesh) true)))
    (:then_1
      (Utilities|Casting|CastToBP_Player_TFP Player))
    (:then_2
      (Utilities|Casting|CastToBP_Player_VR Player))))

(event EventStopLookat
  (params (Player :type BP%20Player%20Object%20Reference))
  ;[1 1 1] Look At
  (|CallParentFunction Player)
  (Utilities|FlowControl|Sequence
    (:then_0
      (Utilities|Casting|CastToBP_Player_TFP Player))
    (:then_1
      (Utilities|Casting|CastToBP_Player_VR Player))))

(event EventUsewith
  (params (UsePoint :type Actor%20Object%20Reference) (Player :type BP%20Player%20Object%20Reference))
  ;[1 1 1] Interact
  (|CallParentFunction UsePoint Player)
  (bind _asbp_place_point (Utilities|Casting|CastToBP_PlacePoint UsePoint))
  (bind _output_get (Variables|Default|SetUsePoint _asbp_place_point))
  (bind _used (Class|BIUse|UseHere(Message) _output_get self))
  (if _used
    (CallFunction|PlaceCorrect Player)
    (else
      (CallFunction|PlaceIncorrect Player))))

(event Collision|EventActorBeginOverlap
  (params (OtherActor :type Actor%20Object%20Reference))
  (bind _player (Variables|Default|GetPlayer)
    (:then
      (bind _asbp_player_vr (Utilities|Casting|CastToBP_Player_VR _player))
      (bind _asbp_place_point (Utilities|Casting|CastToBP_PlacePoint OtherActor))
      (bind _output_get (Variables|Default|SetUsePoint _asbp_place_point))
      (bind _used (Class|BIUse|UseHere(Message) _output_get self))
      (if _used
        (CallFunction|PlaceCorrect _asbp_player_vr)
        (else
          (CallFunction|PlaceIncorrect _asbp_player_vr))))
    (:else)))

(fn ConstructionScript
  (|CallParentFunction))