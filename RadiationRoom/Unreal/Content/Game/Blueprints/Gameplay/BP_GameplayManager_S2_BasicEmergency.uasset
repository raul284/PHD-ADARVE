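; Gameplay manager for scenario S2, Basic Emergency, guiding a VR player through tutorial steps with the Tuddy buddy.
; Events from the description panel, destination point, RBQ van, walkie-talkies and TutorialManager advance steps through reports, help panel and freedom.
; Report flags propagate to every registered walkie-talkie.
; StartScenario currently skips to a completed initial report, landing on the help-panel step; the introduction start is disconnected.
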(event EventBeginPlay
  (|CallParentFunction)
  (Utilities|FlowControl|Sequence
    (:then_0
      (CallFunction|BindItemActions)
      (CallFunction|BindNPCActions))
    (:then_1
      (Default|SetActive (Variables|Default|GetRBPDestinationPoint) false))
    (:then_2
      (Variables|/Game/Game/Blueprints/Tutorial/BP_TutorialManager.BP_TutorialManager_C|SetPlayerCanDemandTuddy (Variables|Default|GetTutorialManager) false))))

(event EventAddItemtoGameManagerImportantList
  (params (ItemType :type E_ItemType%20Enum :default "NewEnumerator2") (Actor :type Actor%20Object%20Reference))
  (switch Utilities|FlowControl|Switch|SwitchonE_ItemType ItemType
    (:NewEnumerator5
      (bind _asbp_walkie_talkie (Utilities|Casting|CastToBP_WalkieTalkie Actor))
      (Default|SetInitialConditions _asbp_walkie_talkie (Variables|WalkieReports|GetInitialReportCompleted) (Variables|WalkieReports|GetFinalReportCompleted))
      (CallFunction|BindWalkieTalkieEvents _asbp_walkie_talkie)
      (Utilities|Array|Add (Variables|WalkieReports|GetWalkieTalkieList) 0))))

(event EventSetPlayerData
  (|CallParentFunction)
  (CallFunction|BindPlayerActions)
  (bind _asbp_player_vr (Utilities|Casting|CastToBP_Player_VR (Variables|Default|GetPlayer)))
  (bind _output_get (Variables|Tutorial|SetTutorialBuddy (Variables|/Game/Game/Blueprints/Characters/Players/BP_Player_VR.BP_Player_VR_C|GetTutorialBuddyActor _asbp_player_vr)))
  (Default|SetCurrentTutorialBuddy (Variables|Default|GetTutorialManager) _output_get)
  (CallFunction|BindTuddyActions)
  (CallFunction|StartScenario)
  (CallFunction|CompleteStep "NewEnumerator9"))

(event EventStartScenario
  (|CallParentFunction)
  (Utilities|FlowControl|Delay 3.0)
  (CallFunction|SetCurrentGameplayStep "NewEnumerator49")
  (CallFunction|OnWalkieInitialReportCompleted))

(event Custom|OnPlayerEnterOnRQBDestinationPoint
  (bind _yes (CallFunction|IsCurrentStep "NewEnumerator51"))
  (if _yes
    (CallFunction|CompleteStep "NewEnumerator51")
    (Default|SetActive (Variables|Default|GetRBPDestinationPoint) false)
    (Utilities|FlowControl|Delay 0.5)
    (CallFunction|SetCurrentGameplayStep "NewEnumerator52")
    (Default|StartExtraLinesDialog (Variables|Default|GetTutorialManager) "NewEnumerator7")))

(event EventBindPlayerActions
  (|CallParentFunction)
  (EventDispatchers|BindEventtoEDPlayerEnteronDestinationPoint (Variables|Default|GetRBPDestinationPoint) (delegate Custom|OnPlayerEnterOnRQBDestinationPoint)))

(event Custom|OnDescriptionCompleted
  (bind _yes (CallFunction|IsCurrentStep "NewEnumerator50"))
  (if _yes
    (CallFunction|CompleteStep "NewEnumerator50")
    (CallFunction|SetCurrentGameplayStep "NewEnumerator51")
    (Utilities|FlowControl|Delay 2.0)
    (Default|StartExtraLinesDialog (Variables|Default|GetTutorialManager) "NewEnumerator6")
    (Default|SetActive (Variables|Default|GetRBPDestinationPoint) true)))

(event Custom|BindWalkieTalkieEvents
  (params (WalkieTalkie :type BP%20Walkie%20Talkie%20Object%20Reference))
  (EventDispatchers|BindEventtoEDInteractionStarted WalkieTalkie (delegate Custom|OnWalkieGrabbed))
  (EventDispatchers|BindEventtoEDInitialReportCompleted WalkieTalkie (delegate Custom|OnWalkieInitialReportCompleted))
  (EventDispatchers|BindEventtoEDFinalReportCompleted WalkieTalkie (delegate Custom|OnWalkieFinalReportCompleted)))

(event Custom|OnWalkieInitialReportCompleted
  (bind _yes (CallFunction|IsCurrentStep "NewEnumerator49"))
  (Variables|WalkieReports|SetInitialReportCompleted _yes)
  (for _array_element (Variables|WalkieReports|GetWalkieTalkieList)
    (Default|SetInitialConditions _array_element (Variables|WalkieReports|GetInitialReportCompleted) (Variables|WalkieReports|GetFinalReportCompleted)))
  (CallFunction|CompleteStep "NewEnumerator49")
  (Utilities|FlowControl|Delay 1.0)
  (CallFunction|SetCurrentGameplayStep "NewEnumerator55")
  (Default|StartExtraLinesDialog (Variables|Default|GetTutorialManager) "NewEnumerator9"))

(event Custom|OnWalkieFinalReportCompleted
  (Variables|WalkieReports|SetFinalReportCompleted true)
  (for _array_element (Variables|WalkieReports|GetWalkieTalkieList)
    (Default|SetInitialConditions _array_element (Variables|WalkieReports|GetInitialReportCompleted) (Variables|WalkieReports|GetFinalReportCompleted))))

(event Custom|BindRBQVanEvents
  (bind _rbqvan (Variables|Default|GetRBQVan)
    (:then
      (EventDispatchers|BindEventtoEDItemSpawned _rbqvan (delegate Custom|OnRBQItemSpawned)))
    (:else
      (Development|PrintString "GameManager S2 no tiene RBQVan" true true "(R=1.000000,G=0.000000,B=0.000000,A=1.000000)"))))

(event Custom|BindDescriptionPanelEvents
  (bind _descriptionpanel (Variables|Default|GetDescriptionPanel)
    (:then
      (EventDispatchers|BindEventtoEDDescriptionCompleted _descriptionpanel (delegate Custom|OnDescriptionCompleted)))
    (:else
      (Development|PrintString "GameManager S2 no tiene DescriptionPanel" true true "(R=1.000000,G=0.000000,B=0.000000,A=1.000000)"))))

(event Custom|OnRBQItemSpawned
  (params (ItemType :type E_ItemType%20Enum :default "NewEnumerator2") (NumOfItems :type Integer))
  (switch Utilities|FlowControl|Switch|SwitchonE_ItemType ItemType
    (:NewEnumerator5
      (Variables|WalkieReports|SetWalkieSpawned true)
      (CallFunction|OnWalkieIsSpawned))))

(event Custom|OnWalkieIsSpawned
  (if (Variables|WalkieReports|GetWalkieSpawned)
    (bind _yes (CallFunction|IsCurrentStep "NewEnumerator52"))
    (if _yes
      (CallFunction|CompleteStep "NewEnumerator52")
      (Default|HideAutomaticHintPanel (Variables|Default|GetTutorialManager))
      (Utilities|FlowControl|Delay 1.0)
      (CallFunction|SetCurrentGameplayStep "NewEnumerator49")
      (Default|AutomaticCall (Variables|Default|GetTutorialManager) "NewEnumerator17"))))

(event Custom|OnWalkieGrabbed
  (bind _yes (CallFunction|IsCurrentStep "NewEnumerator49"))
  (if _yes
    (Default|HideAutomaticHintPanel (Variables|Default|GetTutorialManager))
    (Default|HideCurrentTuddy (Variables|Default|GetTutorialManager))))

(event EventBindItemActions
  (|CallParentFunction)
  (CallFunction|BindDescriptionPanelEvents)
  (CallFunction|BindRBQVanEvents)
  (CallFunction|BindPlacePointsActions))

(event EventBindPlacePointsActions
  (|CallParentFunction))

(event EventBindNPCActions
  (|CallParentFunction))

(event Custom|OnRBQVanExplained
  (bind _yes (CallFunction|IsCurrentStep "NewEnumerator52"))
  (if _yes
    (Default|AutomaticCall (Variables|Default|GetTutorialManager) "NewEnumerator16")
    (CallFunction|OnWalkieIsSpawned)))

(event Custom|OnTuddyIntroductionCompleted
  (Default|StartDescription (Variables|Default|GetDescriptionPanel)))

(event Custom|OnHelpPanelExtraLines
  (bind _yes (CallFunction|IsCurrentStep "NewEnumerator55"))
  (if _yes
    (Default|AutomaticCall (Variables|Default|GetTutorialManager) "NewEnumerator10")
    (Variables|/Game/Game/Blueprints/Tutorial/BP_TutorialManager.BP_TutorialManager_C|SetPlayerCanDemandTuddy (Variables|Default|GetTutorialManager) true)))

(event Custom|BindTutorialManagerActions
  (EventDispatchers|BindEventtoEDTutorialDemanded (Variables|Default|GetTutorialManager) (delegate Custom|OnTutorialDemanded)))

(event Custom|OnTutorialDemanded
  (bind _yes (CallFunction|IsCurrentStep "NewEnumerator55"))
  (if _yes
    (bind _result (Math|Integer|IncrementInt (Variables|Tutorial|GetTutorialDemandedTimes))
      (:%20%20
        (bind _output_get (Variables|Tutorial|SetTutorialDemandedTimes _result))
        (if (>= _output_get 3)
          (Variables|/Game/Game/Blueprints/Tutorial/BP_TutorialManager.BP_TutorialManager_C|SetPlayerCanDemandTuddy (Variables|Default|GetTutorialManager) false)
          (CallFunction|CompleteStep "NewEnumerator55")
          (Utilities|FlowControl|Delay 0.5)
          (CallFunction|SetCurrentGameplayStep "NewEnumerator53")
          (Default|StartExtraLinesDialog (Variables|Default|GetTutorialManager) "NewEnumerator10"))))))

(event Custom|OnTuddyFreedomCompleted
  (bind _yes (CallFunction|IsCurrentStep "NewEnumerator53"))
  (if _yes
    (CallFunction|CompleteStep "NewEnumerator53")
    (Variables|/Game/Game/Blueprints/Tutorial/BP_TutorialManager.BP_TutorialManager_C|SetPlayerCanDemandTuddy (Variables|Default|GetTutorialManager) true)
    (Default|HideCurrentTuddy (Variables|Default|GetTutorialManager))))

(event Custom|OnTuddyDialogCompleted
  (params (CurrentTuddyDialogType :type E_TuddyDialogLinesType%20Enum :default "NewEnumerator0"))
  (switch Utilities|FlowControl|Switch|SwitchonE_GameplayStepTypes (Variables|Default|GetCurrentStepType)
    (:NewEnumerator50
      (CallFunction|OnTuddyIntroductionCompleted))
    (:NewEnumerator52
      (CallFunction|OnRBQVanExplained))
    (:NewEnumerator55
      (CallFunction|OnHelpPanelExtraLines))
    (:NewEnumerator53
      (CallFunction|OnTuddyFreedomCompleted))))

(event EventBindTuddyActions
  (|CallParentFunction)
  (EventDispatchers|BindEventtoEDDialogCompleted (Variables|/Game/Game/Blueprints/Tutorial/BP_TutorialBuddy.BP_TutorialBuddy_C|GetAC_TuddyDialogManager (Variables|/Game/Game/Blueprints/Tutorial/BP_TutorialManager.BP_TutorialManager_C|GetCurrentTutorialBuddy (Variables|Default|GetTutorialManager))) (delegate Custom|OnTuddyDialogCompleted))
  (CallFunction|BindTutorialManagerActions))

(fn ConstructionScript
  (|CallParentFunction))