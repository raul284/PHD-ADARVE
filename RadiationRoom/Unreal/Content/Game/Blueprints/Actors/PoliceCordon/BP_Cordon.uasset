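; BP_Cordon is a police cordon actor that strings rope between BP_PolicePost actors it overlaps.
; On each overlap it attaches the current post's rope end to the new post, then starts a rope from that post if none starts there.
; Each newly started post becomes current and joins an array, whose index sets its PostOrder, forming an ordered chain.
; Separate events forward rope detachment to posts.
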(event Custom|AttatchToPostEnd
  (params (Actor :type BP%20Police%20Post%20Object%20Reference))
  (bind _currentattachedpost (Variables|Default|GetCurrentAttachedPost))
  (if (!= _currentattachedpost Actor)
    (Default|AttachRopeEnd _currentattachedpost Actor)))

(event Custom|AttachToPostStart
  (params (Actor :type BP%20Police%20Post%20Object%20Reference))
  (Default|AttachRopeStart Actor self)
  (Variables|Default|SetCurrentAttachedPost Actor)
  (bind _returnvalue (Utilities|Array|Add (Variables|Default|GetAttachedPost) Actor))
  (Variables|/Game/Game/Blueprints/Actors/PoliceCordon/BP_PolicePost.BP_PolicePost_C|SetPostOrder Actor _returnvalue))

(event Custom|DetachToPostStart
  (params (Actor :type BP%20Police%20Post%20Object%20Reference))
  (Default|DetachRopeStart Actor))

(event Custom|DetachToPostEnd
  (params (Actor :type BP%20Police%20Post%20Object%20Reference))
  (Default|DetachRopeEnd Actor self))

(event Collision|EventActorBeginOverlap
  (params (OtherActor :type Actor%20Object%20Reference))
  (bind _asbp_police_post (Utilities|Casting|CastToBP_PolicePost OtherActor))
  (Utilities|FlowControl|Sequence
    (:then_0
      (bind _currentattachedpost (Variables|Default|GetCurrentAttachedPost)
        (:then
          (if (not (Variables|/Game/Game/Blueprints/Actors/PoliceCordon/BP_PolicePost.BP_PolicePost_C|GetRopeAttachedToEnd _currentattachedpost))
            (CallFunction|AttatchtoPostEnd _asbp_police_post)
            (Variables|Default|SetCurrentAttachedPost 0)))
        (:else)))
    (:then_1
      (if (not (Variables|/Game/Game/Blueprints/Actors/PoliceCordon/BP_PolicePost.BP_PolicePost_C|GetRopeAttachedToStart _asbp_police_post))
        (CallFunction|AttachtoPostStart _asbp_police_post)))))

(fn ConstructionScript)