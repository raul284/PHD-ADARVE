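; BP_PlaceItemManager coordinates the place points where items are placed in the level and tracks whether all are filled.
; On BeginPlay it gathers every BP_PlacePoint of its configured PointClass, registers itself on each and caches the BP_GameplayManager.
; Its events activate or deactivate one or all points.
; AllItemsPlaced scans the points and sets a completion flag, stopping at the first empty one.
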(event Custom|AllItemsPlaced
  (Variables|Default|SetAreAllItemPlaced true)
  (bind _array_element (Utilities|Array|ForEachLoopwithBreak (Variables|Default|GetPlaceInPoints) :!label _label)
    (:LoopBody
      (if (not (Variables|/Game/Game/Blueprints/Actors/Items/UsePoints/PlacePoints/BP_PlacePoint.BP_PlacePoint_C|GetHasItem _array_element))
        (Variables|Default|SetAreAllItemPlaced false)
        (goto _label Break)))))

(event Custom|ActivateAllPoints
  (params (Activate :type Boolean))
  ;[1 1 1] Activate Points
  (for _array_element (Variables|Default|GetPlaceInPoints)
    (CallFunction|ActivateOnePoint Activate _array_element)))

(event Custom|ActivateOnePoint
  (params (Activate :type Boolean) (Point :type BP%20Place%20Point%20Object%20Reference))
  ;[1 1 1] Activate Points
  (Default|ActivatePoint Point 0 Activate))

(event EventBeginPlay
  (Utilities|FlowControl|Sequence
    (:then_0
      (bind _outactors (Actor|GetAllActorsOfClass (Variables|Default|GetPointClass)))
      (for _array_element _outactors
        (bind _asbp_place_point (Utilities|Casting|CastToBP_PlacePoint _array_element))
        (Utilities|Array|Add (Variables|Default|GetPlaceInPoints) _asbp_place_point)
        (Variables|/Game/Game/Blueprints/Actors/Items/UsePoints/PlacePoints/BP_PlacePoint.BP_PlacePoint_C|SetPlaceItemManager _asbp_place_point self)))
    (:then_1
      (bind _returnvalue (Actor|GetActorOfClass "/Game/Game/Blueprints/Gameplay/BP_GameplayManager.BP_GameplayManager_C"))
      (Variables|Default|SetGameplayManager _returnvalue))))

(fn ConstructionScript)