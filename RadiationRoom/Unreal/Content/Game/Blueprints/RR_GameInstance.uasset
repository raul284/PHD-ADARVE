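; Game instance that carries player identity, experience selection and level progression across maps.
; It registers the player through BP_DataBase_Manager, fetching the assigned ID after a short delay, and loads control variable states from a data table at Init.
; A selected experience number gathers matching table rows into a level sequence.
; Closing the database opens the next level, or resets state and returns to the main menu after the last.
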(event Custom|SetScenary
  (params (Type :type E_ScenaryTypes%20Enum :default "NewEnumerator0"))
  (bind _output_get (Variables|Default|SetCurrentScenary Type))
  (Default|CallEDScenarySelected _output_get))

(event Custom|SetPlayerData
  (params (PlayerID :type Integer) (PlayerName :type String))
  (bind _player (Variables|Default|GetPlayer))
  (bind _output_get (Variables|PlayerData|SetPlayerID PlayerID))
  (Variables|/Game/Game/Blueprints/Characters/Players/BP_Player.BP_Player_C|SetUserId _player _output_get)
  (bind _output_get_2 (Variables|PlayerData|SetPlayerName PlayerName))
  (Variables|/Game/Game/Blueprints/Characters/Players/BP_Player.BP_Player_C|SetName _player _output_get_2)
  (Default|CallEDUserIdFound))

(event Custom|CloseDatabase
  (bind _returnvalue (Actor|GetActorOfClass "/Game/Game/Blueprints/Database/BP_DataBase_Manager.BP_DataBase_Manager_C"))
  (bind _output_get (Variables|Default|SetDatabase%20Manager _returnvalue))
  (EventDispatchers|BindEventtoEDDatabaseClosed _output_get (delegate Custom|DatabaseClosed))
  (Default|CloseDatabase _output_get))

(event Custom|CreateDatabasePlayer
  (params (Player%20Name :type String))
  (Variables|PlayerData|SetPlayerName Player%20Name)
  (bind _returnvalue (Actor|GetActorOfClass "/Game/Game/Blueprints/Characters/Players/BP_Player.BP_Player_C"))
  (Variables|Default|SetPlayer _returnvalue)
  (bind _returnvalue_2 (Actor|GetActorOfClass "/Game/Game/Blueprints/Database/BP_DataBase_Manager.BP_DataBase_Manager_C"))
  (Variables|Default|SetDatabase%20Manager _returnvalue_2)
  (bind _player (Variables|Default|GetPlayer)
    (:then
      (bind _database_manager (Variables|Default|GetDatabase%20Manager)
        (:then
          (Default|SendUsertoDB _database_manager (Utilities|Struct|MakeF_UserTableItem 0 (Variables|PlayerData|GetPlayerName) (Variables|/Game/Game/Blueprints/Characters/Players/BP_Player.BP_Player_C|GetUserType _player)))
          (Utilities|FlowControl|Delay 0.2)
          (Default|GetUserId _database_manager (Variables|PlayerData|GetPlayerName)))
        (:else)))
    (:else)))

(event Custom|SelectCurrentExperience
  (params (Experience%20Number :type Integer))
  (bind _experiencetable (Variables|Default|GetExperienceTable))
  (bind _outrownames (DataTable|GetDataTableRowNames _experiencetable))
  (for _array_element _outrownames
    (bind _returnvalue (Utilities|GetDataTableRow _experiencetable _array_element)
      (:then
        (if (== (.Number (Utilities|Struct|BreakF_ExperienceItem _returnvalue)) Experience%20Number)
          (Utilities|Array|Add (Variables|Default|GetCurrentExperience) _returnvalue))))))

(event Custom|GetIdFromDatabase
  (bind _database_manager (Variables|Default|GetDatabase%20Manager)
    (:then
      (Default|GetUserId _database_manager (Variables|PlayerData|GetPlayerName)))
    (:else)))

(event Custom|OpenNextLevel
  (if (< (Variables|Default|GetCurrentLevelIndex) (- (Utilities|Array|Length (Variables|Default|GetCurrentExperience)) 1))
    (bind _output_get (Variables|Default|SetCurrentLevelIndex (+ (Variables|Default|GetCurrentLevelIndex) 1)))
    (Variables|Default|SetCurrentScenary (.LevelType (Utilities|Struct|BreakF_ExperienceItem (Utilities|Array|Get(acopy) (Variables|Default|GetCurrentExperience) _output_get))))
    (Game|OpenLevel(byName) (Utilities|String|StringToName (.LevelName (Utilities|Struct|BreakF_ExperienceItem (Utilities|Array|Get(acopy) (Variables|Default|GetCurrentExperience) _output_get)))))
    (else
      (CallFunction|ResetValues)
      (Game|OpenLevel(byName) "MainMenuMap"))))

(event Custom|DatabaseClosed
  (CallFunction|OpenNextLevel))

(event Custom|ResetValues
  (Utilities|Array|Clear (Variables|Default|GetCurrentExperience))
  (Variables|Default|SetCurrentLevelIndex -1)
  (Variables|Default|SetDatabase%20Manager 0)
  (Variables|Default|SetCurrentScenary "NewEnumerator0")
  (CallFunction|SetPlayerData 2 "Developer")
  (Variables|Default|SetPlayer 0))

(event EventInit
  (CallFunction|GetControlVarsfromDataTable))

(fn GetControlVarsfromDataTable
  (bind _outrownames (DataTable|GetDataTableRowNames (Variables|Default|GetControlVars%20DataTable)))
  (for _array_element _outrownames
    (bind _returnvalue (Utilities|GetDataTableRow (Variables|Default|GetControlVars%20DataTable) _array_element)
      (:then
        (Utilities|Map|Add (Variables|Default|GetControlVars) (.ControlVarType (Utilities|Struct|BreakF_ControlVarData _returnvalue)) (.State (Utilities|Struct|BreakF_ControlVarData _returnvalue)))))))

(fn GetControlVar
  (params (ControlVar%20Type :type E_ControlVars%20Enum :default "NewEnumerator0"))
  (return (.Value (Utilities|Map|Find (Variables|Default|GetControlVars) ControlVar%20Type))))