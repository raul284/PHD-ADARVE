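; AC_Radiation is a component that tracks its owner's current radiation rate and accumulated dose.
; On BeginPlay it grabs a single BP_RadiationEmissionPoint through GetActorOfClass and starts measuring.
; A self-recalling one-second loop asks that point for a distance-based rate and adds 1/3600 of it to the total, treating it as hourly.
; The loop ends for good once CanMeasure is false or the point is invalid.
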(event Custom|MeasureRadiation
  (if (Variables|Default|GetCanMeasure?)
    (bind _radiactiveactor (Variables|Default|GetRadiactiveActor)
      (:then
        (bind _radiation (Default|CalculateRadiationwithDistance _radiactiveactor (Variables|Default|GetOwner)))
        (bind _output_get (Variables|Default|SetRadiationRate _radiation))
        (Variables|Default|SetAccumulatedRadiation (+ (/ _output_get 3.6e+03) (Variables|Default|GetAccumulatedRadiation)))
        (Utilities|FlowControl|Delay 1.0)
        (CallFunction|MeasureRadiation))
      (:else))))

(event EventBeginPlay
  (Variables|Default|SetOwner (Components|GetOwner))
  (bind _returnvalue (Actor|GetActorOfClass "/Game/Game/Blueprints/Actors/RadiationEmisors/BP_RadiationEmissionPoint.BP_RadiationEmissionPoint_C"))
  (Variables|Default|SetRadiactiveActor _returnvalue)
  (CallFunction|MeasureRadiation))