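; Electronic personal dosimeter (EPD) actor that displays radiation dose rate and absorption and logs them to the database.
; On BeginPlay it derives its ID from the count of EPD actors minus one and caches its widget.
; A self-repeating one-second loop updates the widget from ACRadiation.
; Each pass also sends readings, location, time and user/scenario info through the GameInstance's DatabaseManager, if a radiation emission point exists.
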(event Custom|ShowRadiation
  (bind _ac_radiation (Variables|Default|GetAC_Radiation))
  (Default|SetRadiationRate (Variables|Default|GetRadiationInfoWidgetActor) (Variables|/Game/Game/Blueprints/Components/AC_Radiation.AC_Radiation_C|GetDoseRate _ac_radiation) (Variables|/Game/Game/Blueprints/Components/AC_Radiation.AC_Radiation_C|GetDoseAbsorption _ac_radiation))
  (CallFunction|SendEPDRadiationEventtoDB)
  (Utilities|FlowControl|Delay 1.0)
  (CallFunction|ShowRadiation))

(event EventBeginPlay
  (|CallParentFunction)
  (CallFunction|SetEPDId)
  (bind _aswbp_dosimeter_for_dose_and_absortion_radiation_rate (Utilities|Casting|CastToWBP_DosimeterForDoseAndAbsortionRadiationRate (UserInterface|GetWidget (Variables|Default|GetRadiationInfoWidgetComponent))))
  (Variables|Default|SetRadiationInfoWidgetActor _aswbp_dosimeter_for_dose_and_absortion_radiation_rate)
  (CallFunction|ShowRadiation))

(event EventTick
  (params (DeltaSeconds :type Float%20%28single-precision%29))
  (|CallParentFunction DeltaSeconds))

(event EventInteractwith
  (params (Player :type BP%20Player%20Object%20Reference))
  (|CallParentFunction Player))

(event Custom|SendEPDRadiationEventToDB
  (bind _ac_radiation (Variables|Default|GetAC_Radiation))
  (bind _returnvalue (Actor|GetActorOfClass "/Game/Game/Blueprints/Actors/Radiation/BP_RadiationEmissionPoint.BP_RadiationEmissionPoint_C"))
  (Utilities|IsValid _returnvalue
    (:Is%20Valid
      (bind _data (Default|GetDataBaseMainInfoEvent (Variables|Default|GetGameInstance)))
      (bind _database_manager (Variables|/Game/Game/Blueprints/RR_GameInstance.RR_GameInstance_C|GetDatabase%20Manager (Variables|Default|GetGameInstance))
        (:then
          (Default|SendEPDRadiationEventtoDB _database_manager (Utilities|Struct|MakeF_EPDRadiationEvent 0 (.user_id (Utilities|Struct|BreakF_MainInfoEvent _data)) (.scenario_type (Utilities|Struct|BreakF_MainInfoEvent _data)) (Variables|Default|GetEPDId) (Variables|/Game/Game/Blueprints/Components/AC_Radiation.AC_Radiation_C|GetDoseRate _ac_radiation) (Variables|/Game/Game/Blueprints/Components/AC_Radiation.AC_Radiation_C|GetDoseAbsorption _ac_radiation) (Transformation|GetActorLocation) (Math|DateTime|Now))))
        (:else)))))

(fn ConstructionScript
  (|CallParentFunction))

(fn SetEPDId
  (bind _outactors (Actor|GetAllActorsOfClass "BP_Dosimeter_EPD_C"))
  (if (Utilities|Array|IsEmpty _outactors)
    (Variables|Default|SetEPDId 0)
    (Development|PrintString (Utilities|String|ToString(Integer) (Variables|Default|GetEPDId)))
    (else
      (Variables|Default|SetEPDId (- (Utilities|Array|Length _outactors) 1)))))