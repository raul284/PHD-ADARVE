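; BP_Manager_NPC_Pedestrian runs a one-at-a-time radiation screening queue for store-accident worker NPCs.
; On BeginPlay it gathers every BP_NPC_StoreAccident_Worker and sends the first to ExamPoint.
; NPCRadiationMeasured forwards the result to the current NPC with either the radiation or no-radiation destination point, then NextNPC advances the index and sends the next worker to be examined.
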(event Custom|NextNPC
  (bind _result (Math|Integer|IncrementInt (Variables|Default|GetIndex))
    (:%20%20
      (if (> (Utilities|Array|Length (Variables|Default|GetNPCs)) _result)
        (bind _output_get (Variables|Default|SetCurrentNPC (Utilities|Array|Get(acopy) (Variables|Default|GetNPCs) _result)))
        (Default|GotoExamPoint _output_get (Variables|Default|GetExamPoint))))))

(event Custom|NPCRadiationMeasured
  (params (Is%20Radiactive? :type Boolean))
  (if Is%20Radiactive?
    (Default|RadiationMeasured (Variables|Default|GetCurrentNPC) Is%20Radiactive? (Variables|Default|GetWithRadiationPoint))
    (else
      (Default|RadiationMeasured (Variables|Default|GetCurrentNPC) Is%20Radiactive? (Variables|Default|GetWithoutRadiationPoint))))
  (Variables|Default|SetCurrentNPC 0)
  (CallFunction|NextNPC))

(event EventBeginPlay
  (bind _outactors (Actor|GetAllActorsOfClass "/Game/Game/Blueprints/Characters/AI/StoreAccident/Worker/BP_NPC_StoreAccident_Worker.BP_NPC_StoreAccident_Worker_C"))
  (if (> (Utilities|Array|Length _outactors) 0)
    (bind _output_get (Variables|Default|SetNPCs _outactors))
    (bind _output_get_2 (Variables|Default|SetCurrentNPC (Utilities|Array|Get(acopy) _output_get (Variables|Default|GetIndex))))
    (Default|GotoExamPoint _output_get_2 (Variables|Default|GetExamPoint))))

(fn ConstructionScript)