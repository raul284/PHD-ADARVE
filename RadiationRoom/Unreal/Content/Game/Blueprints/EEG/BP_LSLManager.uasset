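; BP_LSLManager publishes gameplay telemetry as Lab Streaming Layer string markers and registers itself with RR_GameInstance on BeginPlay.
; Each SendLSL event formats its data struct (user, scenario, event details) into one string and pushes it to an LSL stream, usually one per category.
; NPC interactions share the item interaction stream, and move events send nothing because their push logic is disconnected.
; Helper functions serialize arrays into bracketed, semicolon-delimited strings.
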(event Custom|Send%20LSL%20Gameplay%20Event
  (params (Data :type F%20Gameplay%20Event%20Structure))
  (bind (_event_id _user_id _scenario_type _event_type _event_state) (Utilities|Struct|BreakF_GameplayEvent Data))
  (Class|LSLOutletComponent|PushSampleString (Variables|Default|GetLSL_GameplayEvent) (Utilities|Array|MakeArray (Utilities|String|ToString(Text) (Utilities|Text|FormatText "{user}: {scenario}, {type}, {state}" (Utilities|String|ToString(Integer) _user_id) (Utilities|String|EnumtoString _scenario_type) (Utilities|String|EnumtoString _event_type) (Utilities|String|EnumtoString _event_state))))))

(event Custom|Send%20LSL%20NPC%20Interaction%20Event
  (params (Data :type F%20NPC%20Interaction%20Event%20Structure))
  (bind (_event_id _user_id _scenario_type _actor_id _conversation_index _event_type _hand) (Utilities|Struct|BreakF_NPCInteractionEvent Data))
  (Class|LSLOutletComponent|PushSampleString (Variables|Default|GetLSL_ItemInteractionEvent) (Utilities|Array|MakeArray (Utilities|String|ToString(Text) (Utilities|Text|FormatText "{user}: {scenario}, {actor_id}, {conversation_index}, {type}, {hand}" (Utilities|String|ToString(Integer) _user_id) (Utilities|String|EnumtoString _scenario_type) (Utilities|String|ToString(Integer) _actor_id) (Utilities|String|ToString(Integer) _conversation_index) (Utilities|String|EnumtoString _event_type) (Utilities|String|EnumtoString _hand))))))

(event Custom|Send%20LSL%20Tip%20Event
  (params (Data :type F%20Tips%20Event%20Structure))
  (bind (_event_id _user_id _scenario_type _tip_type) (Utilities|Struct|BreakF_TipsEvent Data))
  (Class|LSLOutletComponent|PushSampleString (Variables|Default|GetLSL_TipEvent) (Utilities|Array|MakeArray (Utilities|String|ToString(Text) (Utilities|Text|FormatText "{user}: {scenario}, {type}" (Utilities|String|ToString(Integer) _user_id) (Utilities|String|EnumtoString _scenario_type) (Utilities|String|EnumtoString _tip_type))))))

(event Custom|Send%20LSL%20Help%20Panel%20Event
  (params (Data :type F%20Help%20Panel%20Event%20Structure))
  (bind (_event_id _user_id _scenario_type _event_type _tutorial_item_id) (Utilities|Struct|BreakF_HelpPanelEvent Data))
  (Class|LSLOutletComponent|PushSampleString (Variables|Default|GetLSL_HelpPanelEvent) (Utilities|Array|MakeArray (Utilities|String|ToString(Text) (Utilities|Text|FormatText "{user}: {scenario}, {type}, {item_id}" (Utilities|String|ToString(Integer) _user_id) (Utilities|String|EnumtoString _scenario_type) (Utilities|String|EnumtoString _event_type) (Utilities|String|EnumtoString _tutorial_item_id))))))

(event Custom|Send%20LSL%20NPC%20Radiation%20Event
  (params (Data :type F%20NPC%20Radiation%20Event%20Structure))
  (bind (_event_id _user_id _scenario_type _actor_id _dose_rate _dose_absortion) (Utilities|Struct|BreakF_NPCRadiationEvent Data))
  (Class|LSLOutletComponent|PushSampleString (Variables|Default|GetLSL_NPCRadiationEvent) (Utilities|Array|MakeArray (Utilities|String|ToString(Text) (Utilities|Text|FormatText "{user}: {scenario}, {actor_id}, {dose_rate}, {dose_absortion}" (Utilities|String|ToString(Integer) _user_id) (Utilities|String|EnumtoString _scenario_type) (Utilities|String|ToString(Integer) _actor_id) (Utilities|String|ToString(Float) _dose_rate) (Utilities|String|ToString(Float) _dose_absortion))))))

(event Custom|Send%20LSL%20Item%20Radiation%20Event
  (params (Data :type F%20Item%20Radiation%20Event%20Structure))
  (bind (_event_id _user_id _scenario_type _actor_id _actor_name _dose_rate _dose_absortion) (Utilities|Struct|BreakF_ItemRadiationEvent Data))
  (Class|LSLOutletComponent|PushSampleString (Variables|Default|GetLSL_ItemRadiationEvent) (Utilities|Array|MakeArray (Utilities|String|ToString(Text) (Utilities|Text|FormatText "{user}: {scenario}, {actor_id}, {actor_name}, {dose_rate}, {dose_absortion}" (Utilities|String|ToString(Integer) _user_id) (Utilities|String|EnumtoString _scenario_type) (Utilities|String|ToString(Integer) _actor_id) _actor_name (Utilities|String|ToString(Float) _dose_rate) (Utilities|String|ToString(Float) _dose_absortion))))))

(event Custom|Send%20LSL%20Walkie%20Report%20Event
  (params (Data :type F%20Walkie%20Report%20Event%20Structure))
  (bind (_event_id _user_id _scenario_type _conversation_type _question_index _answer_index) (Utilities|Struct|BreakF_WalkieReportEvent Data))
  (Class|LSLOutletComponent|PushSampleString (Variables|Default|GetLSL_WalkieReportEvent) (Utilities|Array|MakeArray (Utilities|String|ToString(Text) (Utilities|Text|FormatText "{user}: {scenario}, {conversation_type}, {question_index}, {answer_index}" (Utilities|String|ToString(Integer) _user_id) (Utilities|String|EnumtoString _scenario_type) (Utilities|String|EnumtoString _conversation_type) (Utilities|String|ToString(Integer) _question_index) (Utilities|String|ToString(Integer) _answer_index))))))

(event Custom|Send%20LSL%20Item%20Interaction%20Event
  (params (Data :type F%20Item%20Interaction%20Event%20Structure))
  (bind (_event_id _user_id _scenario_type _actor_id _actor_name _event_type _hand) (Utilities|Struct|BreakF_ItemInteractionEvent Data))
  (Class|LSLOutletComponent|PushSampleString (Variables|Default|GetLSL_ItemInteractionEvent) (Utilities|Array|MakeArray (Utilities|String|ToString(Text) (Utilities|Text|FormatText "{user}: {scenario}, {actor_id}, {actor_name}, {type}, {hand}" (Utilities|String|ToString(Integer) _user_id) (Utilities|String|EnumtoString _scenario_type) (Utilities|String|ToString(Integer) _actor_id) _actor_name (Utilities|String|EnumtoString _event_type) (Utilities|String|EnumtoString _hand))))))

(event Custom|Send%20LSL%20Place%20Point%20Event
  (params (Data :type F%20Place%20Point%20Event%20Structure))
  (bind (_event_id _user_id _scenario_type _actor_id _actor_name _place_point_name _event_type) (Utilities|Struct|BreakF_PlacePointEvent Data))
  (Class|LSLOutletComponent|PushSampleString (Variables|Default|GetLSL_PlacePointEvent) (Utilities|Array|MakeArray (Utilities|String|ToString(Text) (Utilities|Text|FormatText "{user}: {scenario}, {actor_id}, {actor_name}, {place_point_name}, {event_type}" (Utilities|String|ToString(Integer) _user_id) (Utilities|String|EnumtoString _scenario_type) (Utilities|String|ToString(Integer) _actor_id) _actor_name _place_point_name (Utilities|String|EnumtoString _event_type))))))

(event Custom|Send%20LSL%20Move%20Event
  (params (Data :type F%20Move%20Event%20Structure)))

(event Custom|Send%20LSL%20User%20Input%20Event
  (params (Data :type F%20User%20Input%20Event%20Structure))
  (bind (_event_id _user_id _scenario_type _input_type _input_state) (Utilities|Struct|BreakF_UserInputEvent Data))
  (Class|LSLOutletComponent|PushSampleString (Variables|Default|GetLSL_UserInputEvent) (Utilities|Array|MakeArray (Utilities|String|ToString(Text) (Utilities|Text|FormatText "{user}: {scenario}, {type}, {state}" (Utilities|String|ToString(Integer) _user_id) (Utilities|String|EnumtoString _scenario_type) (Utilities|GetDisplayName _input_type) (Utilities|String|EnumtoString _input_state))))))

(event Custom|Send%20LSL%20Inventory%20Event
  (params (Data :type F%20Inventory%20Event%20Structure))
  (bind (_event_id _user_id _scenario_type _actor_id _actor_name _event_type) (Utilities|Struct|BreakF_InventoryEvent Data))
  (Class|LSLOutletComponent|PushSampleString (Variables|Default|GetLSL_InventoryEvent) (Utilities|Array|MakeArray (Utilities|String|ToString(Text) (Utilities|Text|FormatText "{user}: {scenario}, {actor_id}, {actor_name}, {type}" (Utilities|String|ToString(Integer) _user_id) (Utilities|String|EnumtoString _scenario_type) (Utilities|String|ToString(Integer) _actor_id) _actor_name (Utilities|String|EnumtoString _event_type))))))

(event Custom|Send%20LSL%20RBQ%20Panel%20Event
  (params (Data :type F%20RBQ%20Event%20Structure))
  (bind (_event_id _user_id _scenario_type _actor_id _num_of_actors) (Utilities|Struct|BreakF_RBQEvent Data))
  (bind _string (CallFunction|StringfromArrayOfInts _actor_id))
  (bind _string_2 (CallFunction|StringfromArrayOfInts _num_of_actors))
  (Class|LSLOutletComponent|PushSampleString (Variables|Default|GetLSL_RBQPanelEvent) (Utilities|Array|MakeArray (Utilities|String|ToString(Text) (Utilities|Text|FormatText "{user}: {scenario}, {actor_id}, {num_of_actors}" (Utilities|String|ToString(Integer) _user_id) (Utilities|String|EnumtoString _scenario_type) _string _string_2)))))

(event EventBeginPlay
  (bind _asrr_game_instance (Utilities|Casting|CastToRR_GameInstance (Game|GetGameInstance)))
  (bind _output_get (Variables|Default|SetGame%20Instance _asrr_game_instance))
  (Default|SetLSLManager _output_get self))

(fn ConstructionScript)

(fn StringfromArrayOfFloats
  (params (ListOfFloats :type Array%20of%20Floats%20%28double-precision%29))
  (LocalVariables|SetString%20Of%20Floats "[")
  (for _array_element ListOfFloats
    (LocalVariables|SetString%20Of%20Floats (Utilities|String|Append (LocalVariables|GetString%20Of%20Floats) (Utilities|String|Append (Utilities|String|ToString(Float) _array_element) ";"))))
  (bind _output_get (LocalVariables|SetString%20Of%20Floats (Utilities|String|Append (LocalVariables|GetString%20Of%20Floats) "]")))
  (return _output_get))

(fn VectortoXYString
  (params (Vector :type Vector))
  (bind (_x _y) (Class|KismetMathLibrary|BreakVector3f Vector))
  (return (Utilities|String|Append "(" (Utilities|String|ToString(Float) _x) ";" (Utilities|String|ToString(Float) _y) ")")))

(fn StringfromArrayOfVectors
  (params (ListOfVectors :type Array%20of%20Vectors))
  (LocalVariables|SetString%20Of%20Vectors "[")
  (for _array_element ListOfVectors
    (bind _coordinates (CallFunction|VectortoXYString _array_element))
    (LocalVariables|SetString%20Of%20Vectors (Utilities|String|Append (LocalVariables|GetString%20Of%20Vectors) (Utilities|String|Append _coordinates ";"))))
  (bind _output_get (LocalVariables|SetString%20Of%20Vectors (Utilities|String|Append (LocalVariables|GetString%20Of%20Vectors) "]")))
  (return _output_get))

(fn StringfromArrayOfInts
  (params (ListOfInts :type Array%20of%20Integers))
  (LocalVariables|SetString%20Of%20Floats "[")
  (for _array_element ListOfInts
    (LocalVariables|SetString%20Of%20Floats (Utilities|String|Append (LocalVariables|GetString%20Of%20Floats) (Utilities|String|Append (Utilities|String|ToString(Integer) _array_element) ";"))))
  (bind _output_get (LocalVariables|SetString%20Of%20Floats (Utilities|String|Append (LocalVariables|GetString%20Of%20Floats) "]")))
  (return _output_get))