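; Interactable item Blueprint for consumables that reports itself as always consumable and extends its parent's look-at and interact events.
; Each event branches by casting to the TFP or VR player, though only interaction adds behavior.
; TFP interaction destroys the item and logs a timestamped event with actor and user IDs through DBManager.
; VR interaction logs a different event type and leaves the item in place.
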(event EventBeginPlay
  (|CallParentFunction))

(event EventInteractwith
  (params (Player :type BP%20Player%20Object%20Reference))
  ;[1 1 1] Interact
  (|CallParentFunction Player)
  (Utilities|FlowControl|Sequence
    (:then_0
      (Utilities|Casting|CastToBP_Player_TFP Player)
      (Actor|DestroyActor)
      (bind _dbmanager (Variables|Default|GetDBManager)
        (:then
          (Default|SendInteractEventtoDB _dbmanager (Utilities|Struct|MakeF_InteractEventsTableItem 0 (Variables|Default|GetActorId) (Variables|/Game/Game/Blueprints/Characters/Players/BP_Player.BP_Player_C|GetUserId Player) "NewEnumerator0" "NewEnumerator9" (Math|DateTime|Now))))
        (:else)))
    (:then_1
      (Utilities|Casting|CastToBP_Player_VR Player)
      (bind _dbmanager_2 (Variables|Default|GetDBManager)
        (:then
          (Default|SendInteractEventtoDB _dbmanager_2 (Utilities|Struct|MakeF_InteractEventsTableItem 0 (Variables|Default|GetActorId) (Variables|/Game/Game/Blueprints/Characters/Players/BP_Player.BP_Player_C|GetUserId Player) "NewEnumerator0" "NewEnumerator6" (Math|DateTime|Now))))
        (:else)))))

(event EventStartLookat
  (params (Player :type BP%20Player%20Object%20Reference))
  ;[1 1 1] Look At
  (|CallParentFunction Player)
  (Utilities|FlowControl|Sequence
    (:then_0
      (Utilities|Casting|CastToBP_Player_TFP Player))
    (:then_1
      (Utilities|Casting|CastToBP_Player_VR Player))))

(event EventCancelInteract
  (params (Player :type BP%20Player%20Object%20Reference))
  ;[1 1 1] Interact
  (|CallParentFunction Player)
  (Utilities|FlowControl|Sequence
    (:then_0
      (Utilities|Casting|CastToBP_Player_TFP Player))
    (:then_1
      (Utilities|Casting|CastToBP_Player_VR Player))))

(event EventStopLookat
  (params (Player :type BP%20Player%20Object%20Reference))
  ;[1 1 1] Look At
  (|CallParentFunction Player)
  (Utilities|FlowControl|Sequence
    (:then_0
      (Utilities|Casting|CastToBP_Player_TFP Player))
    (:then_1
      (Utilities|Casting|CastToBP_Player_VR Player))))

(fn ConstructionScript
  (|CallParentFunction))

(fn CanConsume
  (return true))