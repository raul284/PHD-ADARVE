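; BP_Clamps is a usable clamps item that grabs nearby pickable items.
; Each Tick runs a small sphere trace for PhysicsBody objects at the mesh's PointToGrab socket, with persistent debug drawing left on.
; A hit BP_PickableItem flagged PickableByClamps is attached to the clamps actor, specifying PointToGrab as the socket, and HasItem is set to false.
; HasItem is never checked, and no release logic exists here.
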(event EventBeginPlay
  (|CallParentFunction) ; This node is disabled and will not be called.\nDrag off pins to build functionality.
)

(event Collision|EventActorBeginOverlap
  (params (OtherActor :type Actor%20Object%20Reference)))

(event EventTick
  (params (DeltaSeconds :type Float%20%28single-precision%29))
  (bind _staticmesh (Variables|Default|GetStaticMesh))
  (bind _returnvalue (Transformation|GetSocketLocation _staticmesh "PointToGrab"))
  (|CallParentFunction DeltaSeconds)
  (bind (_outhit _returnvalue_2) (Collision|SphereTraceForObjects _returnvalue _returnvalue 1e+01 (Utilities|Array|MakeArray "ObjectTypeQuery4") false 0 "Persistent" true "(R=0.000000,G=1.000000,B=1.000000,A=1.000000)" "(R=0.000000,G=1.000000,B=0.000000,A=1.000000)" 1.0))
  (if _returnvalue_2
    (bind _asbp_pickable_item (Utilities|Casting|CastToBP_PickableItem (.HitActor (Collision|BreakHitResult _outhit))))
    (if (Variables|/Game/Game/Blueprints/Actors/Items/BP_PickableItem.BP_PickableItem_C|GetPickableByClamps _asbp_pickable_item)
      (Transformation|AttachActorToActor _asbp_pickable_item self "PointToGrab" "SnapToTarget" "SnapToTarget" "KeepWorld" true)
      (Variables|Default|SetHasItem false))))

(fn ConstructionScript
  (|CallParentFunction))